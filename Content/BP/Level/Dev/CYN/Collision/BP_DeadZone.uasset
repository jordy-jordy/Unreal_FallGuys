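; BP_DeadZone is a level trigger volume that sends player characters back to their respawn position.
; When a BP_PlayCharacter overlaps its Box, the authority checks the status on the character's BP_PlayPlayerState.
; Unless that status is one specific excluded value, it moves the character to the RespawnPos stored on the character and calls PlayRespawnSound to play a sound there.
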(event OnComponentBeginOverlap(Box)
  (params (OverlappedComponent :type Primitive%20Component%20Object%20Reference) (OtherActor :type Actor%20Object%20Reference) (OtherComp :type Primitive%20Component%20Object%20Reference) (OtherBodyIndex :type Integer) (bFromSweep :type Boolean) (SweepResult :type Hit%20Result%20Structure%20%28by%20ref%29))
  (bind _asbp_play_character (Utilities|Casting|CastToBP_PlayCharacter OtherActor))
  (Networking|SwitchHasAuthority
    (:Authority
      (bind _asbp_play_player_state (Utilities|Casting|CastToBP_PlayPlayerState (Variables|/Script/Engine.Pawn|GetPlayerState _asbp_play_character)))
      (bind _returnvalue (Class|PlayPlayerState|GetPlayerStateStatus _asbp_play_player_state))
      (if (!= _returnvalue 3)
        (Transformation|SetActorLocation _asbp_play_character (Variables|/Game/BP/Mode/01_Play/BP_PlayCharacter.BP_PlayCharacter_C|GetRespawnPos _asbp_play_character) false false)
        (CallFunction|PlayRespawnSound)))))

(event Custom|Play%20Respawn%20Sound
  (Audio|PlaySoundatLocation "/Game/Resources/Level/Race/Sound/SFX/Player_Respawn__Fall_Guys_Sound__-_Sound_Effect_for_editing__mp3cut_net_.Player_Respawn__Fall_Guys_Sound__-_Sound_Effect_for_editing__mp3cut_net_" (Variables|/Game/BP/Mode/01_Play/BP_PlayCharacter.BP_PlayCharacter_C|GetRespawnPos (stale OnComponentBeginOverlap(Box) _asbp_play_character)) "0, 0, 0" 5.0 1.0 0.0 0 0 0 0))

(event EventBeginPlay)

(event Collision|EventActorBeginOverlap
  (params (OtherActor :type Actor%20Object%20Reference)))

(event EventTick
  (params (DeltaSeconds :type Float%20%28single-precision%29)))

(fn ConstructionScript)