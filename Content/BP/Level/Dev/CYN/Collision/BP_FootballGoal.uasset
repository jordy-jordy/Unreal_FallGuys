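; BP_FootballGoal is a team soccer goal that awards a point when a BP_Soccerball enters its Box trigger.
; On overlap it plays a goal sound, credits the team opposing the goal's side via the IsBlue flag, and destroys the ball.
; RedScore and BlueSocre increment that team's score on BP_TeamPlayGameState and print the new value on screen in the team's color.
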(event OnComponentBeginOverlap(Box)
  (params (OverlappedComponent :type Primitive%20Component%20Object%20Reference) (OtherActor :type Actor%20Object%20Reference) (OtherComp :type Primitive%20Component%20Object%20Reference) (OtherBodyIndex :type Integer) (bFromSweep :type Boolean) (SweepResult :type Hit%20Result%20Structure%20%28by%20ref%29))
  (bind _asbp_soccerball (Utilities|Casting|CastToBP_Soccerball OtherActor))
  (Audio|PlaySound2D "/Game/Resources/Level/Race/Sound/SFX/Fall_Ball_Goal__Fall_Guys_Sound__-_Sound_Effect_for_editing.Fall_Ball_Goal__Fall_Guys_Sound__-_Sound_Effect_for_editing" 1.0 1.0 0.0 0 0)
  (if (Variables|Default|GetIsBlue)
    (CallFunction|RedScore)
    (Actor|DestroyActor _asbp_soccerball)
    (else
      (CallFunction|BlueSocre)
      (Actor|DestroyActor _asbp_soccerball))))

(event EventBeginPlay)

(event Collision|EventActorBeginOverlap
  (params (OtherActor :type Actor%20Object%20Reference)))

(event EventTick
  (params (DeltaSeconds :type Float%20%28single-precision%29)))

(fn ConstructionScript)

(fn BlueSocre
  (bind _asbp_team_play_game_state (Utilities|Casting|CastToBP_TeamPlayGameState (Game|GetGameState)))
  (bind _returnvalue (Class|TeamPlayGameState|GetGameStateBLUETeamScore _asbp_team_play_game_state))
  (Class|TeamPlayGameState|SetBLUETeamScore _asbp_team_play_game_state (+ _returnvalue 1))
  (Development|PrintString (Utilities|String|ToString(Integer) (+ _returnvalue 1)) true true "(R=0.000000,G=0.000000,B=1.000000,A=1.000000)" 1e+01))

(fn RedScore
  (bind _asbp_team_play_game_state (Utilities|Casting|CastToBP_TeamPlayGameState (Game|GetGameState)))
  (bind _returnvalue (Class|TeamPlayGameState|GetGameStateREDTeamScore _asbp_team_play_game_state))
  (Class|TeamPlayGameState|SetREDTeamScore _asbp_team_play_game_state (+ _returnvalue 1))
  (Development|PrintString (Utilities|String|ToString(Integer) (+ _returnvalue 1)) true true "(R=1.000000,G=0.000000,B=0.000000,A=1.000000)" 1e+01))