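; BP_SlidePipe is a level actor that carries the player character along a spline, apparently as a slide through a pipe.
; Overlapping its box stores the BP_PlayCharacter and sets a Start flag, which Tick checks to play the SplineTime timeline.
; Timeline updates map alpha to spline distance and set the character's root location without sweeping, and finishing clears Start.
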(event OnComponentBeginOverlap(Box)
  (params (OverlappedComponent :type Primitive%20Component%20Object%20Reference) (OtherActor :type Actor%20Object%20Reference) (OtherComp :type Primitive%20Component%20Object%20Reference) (OtherBodyIndex :type Integer) (bFromSweep :type Boolean) (SweepResult :type Hit%20Result%20Structure%20%28by%20ref%29))
  (bind _asbp_play_character (Utilities|Casting|CastToBP_PlayCharacter OtherActor))
  (Variables|Default|SetStart true))

(event EventTick
  (params (DeltaSeconds :type Float%20%28single-precision%29))
  (bind _spline (Variables|Default|GetSpline))
  (if (Variables|Default|GetStart)
    (bind _spline_2 (Timeline|SplineTime Play)
      (:Update
        (Transformation|SetWorldLocation (Variables|/Script/Engine.Actor|GetRootComponent (stale OnComponentBeginOverlap(Box) _asbp_play_character)) (Spline|GetLocationatDistanceAlongSpline _spline (Math|Float|Lerp 0.0 (Spline|GetSplineLength _spline) _spline_2) "World") false false))
      (:Finished
        (Variables|Default|SetStart false)))))

(fn ConstructionScript)