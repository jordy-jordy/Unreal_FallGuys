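; Rotating weapon obstacle for race levels that reacts when it hits a player character.
; On Tick, the authority alone drives ObstacleMoveComp's SpinCycle on the Axis component about X, using the configured speed and angle limit.
; A capsule hit on BP_PlayCharacter plays one of three random hit sounds at the player and copies PhyTime onto them.
; The hit handler's authority switch is empty and gates neither action.
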(event OnComponentHit(CapsuleCollision)
  (params (HitComponent :type Primitive%20Component%20Object%20Reference) (OtherActor :type Actor%20Object%20Reference) (OtherComp :type Primitive%20Component%20Object%20Reference) (NormalImpulse :type Vector :default "0, 0, 0") (Hit :type Hit%20Result%20Structure%20%28by%20ref%29))
  (bind _asbp_play_character (Utilities|Casting|CastToBP_PlayCharacter OtherActor))
  (bind _output_get (Variables|Default|SetHit%20Sound%20Index (Math|Random|RandomIntegerinRange 0 2)))
  (Utilities|FlowControl|Sequence
    (:then_0
      (Networking|SwitchHasAuthority
        (:Authority
          _)
        (:Remote
          _))
      (switch int _output_get
        (:0
          (Audio|PlaySoundatLocation "/Game/Resources/Level/Race/Sound/SFX/Generic_Player_Hit__Nr__4___Fall_Guys_Sound__-_Sound_Effect_for_editing__mp3cut_net_.Generic_Player_Hit__Nr__4___Fall_Guys_Sound__-_Sound_Effect_for_editing__mp3cut_net_" (Transformation|GetActorLocation _asbp_play_character) "0, 0, 0" 1.0 1.0 0.0 0 0 0 0))
        (:1
          (Audio|PlaySoundatLocation "/Game/Resources/Level/Race/Sound/SFX/Generic_Player_Hit__Nr__6___Fall_Guys_Sound__-_Sound_Effect_for_editing__mp3cut_net_.Generic_Player_Hit__Nr__6___Fall_Guys_Sound__-_Sound_Effect_for_editing__mp3cut_net_" (Transformation|GetActorLocation _asbp_play_character) "0, 0, 0" 1.0 1.0 0.0 0 0 0 0))
        (:2
          (Audio|PlaySoundatLocation "/Game/Resources/Level/Race/Sound/SFX/Generic_Player_Hit__Nr__7___Fall_Guys_Sound__-_Sound_Effect_for_editing__mp3cut_net_.Generic_Player_Hit__Nr__7___Fall_Guys_Sound__-_Sound_Effect_for_editing__mp3cut_net_" (Transformation|GetActorLocation _asbp_play_character) "0, 0, 0" 1.0 1.0 0.0 0 0 0 0))))
    (:then_1
      (Variables|/Game/BP/Mode/01_Play/BP_PlayCharacter.BP_PlayCharacter_C|SetPhyTime _asbp_play_character (Variables|Default|GetPhyTime)))))

(event EventBeginPlay)

(event Collision|EventActorBeginOverlap
  (params (OtherActor :type Actor%20Object%20Reference)))

(event EventTick
  (params (DeltaSeconds :type Float%20%28single-precision%29))
  (Networking|SwitchHasAuthority
    (:Authority
      (Class|ObsMovementActorComponent|SpinCycle (Variables|Default|GetObstacleMoveComp) (Variables|Default|GetAxis) (Variables|Default|GetRotateSpeed) (Variables|Default|GetLimitAngle) "X" DeltaSeconds))))

(fn ConstructionScript)