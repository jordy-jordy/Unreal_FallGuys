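; Race obstacle that repeatedly fires a punch along its local Y axis and hits player characters in its path.
; Tick runs a DELAY, FIRE, RECOVER state machine, with only the authority timing the exit from DELAY.
; ObstacleMoveComp moves the punch until CheckLimitPos reports a travel limit.
; Overlaps during FIRE play a random player-hit sound plus an impact sound and set the character's PhyTime.
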(event OnComponentBeginOverlap(PunchCollision)
  (params (OverlappedComponent :type Primitive%20Component%20Object%20Reference) (OtherActor :type Actor%20Object%20Reference) (OtherComp :type Primitive%20Component%20Object%20Reference) (OtherBodyIndex :type Integer) (bFromSweep :type Boolean) (SweepResult :type Hit%20Result%20Structure%20%28by%20ref%29))
  (bind _asbp_play_character (Utilities|Casting|CastToBP_PlayCharacter OtherActor))
  (if (Utilities|Enum|Equal(Enum) (Variables|Default|GetCurPunchState) "FIRE")
    (bind _output_get (Variables|Default|SetHit%20Sound%20Index (Math|Random|RandomIntegerinRange 0 2)))
    (Utilities|FlowControl|Sequence
      (:then_0
        (Networking|SwitchHasAuthority
          (:Authority
            _)
          (:Remote
            _))
        (switch int _output_get
          (:0
            (Audio|PlaySoundatLocation "/Game/Resources/Level/Race/Sound/SFX/Generic_Player_Hit__Nr__4___Fall_Guys_Sound__-_Sound_Effect_for_editing__mp3cut_net_.Generic_Player_Hit__Nr__4___Fall_Guys_Sound__-_Sound_Effect_for_editing__mp3cut_net_" (Transformation|GetActorLocation _asbp_play_character) "0, 0, 0" 1.0 1.0 0.0 0 0 0 0))
          (:1
            (Audio|PlaySoundatLocation "/Game/Resources/Level/Race/Sound/SFX/Generic_Player_Hit__Nr__6___Fall_Guys_Sound__-_Sound_Effect_for_editing__mp3cut_net_.Generic_Player_Hit__Nr__6___Fall_Guys_Sound__-_Sound_Effect_for_editing__mp3cut_net_" (Transformation|GetActorLocation _asbp_play_character) "0, 0, 0" 1.0 1.0 0.0 0 0 0 0))
          (:2
            (Audio|PlaySoundatLocation "/Game/Resources/Level/Race/Sound/SFX/Generic_Player_Hit__Nr__7___Fall_Guys_Sound__-_Sound_Effect_for_editing__mp3cut_net_.Generic_Player_Hit__Nr__7___Fall_Guys_Sound__-_Sound_Effect_for_editing__mp3cut_net_" (Transformation|GetActorLocation _asbp_play_character) "0, 0, 0" 1.0 1.0 0.0 0 0 0 0))))
      (:then_1
        (Networking|SwitchHasAuthority
          (:Authority
            _)
          (:Remote
            _))
        (Audio|PlaySoundatLocation "/Game/Resources/Level/Race/Sound/SFX/Fall_Ball_Hit__Nr__3___Fall_Guys_Sound__-_Sound_Effect_for_editing__mp3cut_net_.Fall_Ball_Hit__Nr__3___Fall_Guys_Sound__-_Sound_Effect_for_editing__mp3cut_net_" (Transformation|GetActorLocation _asbp_play_character) "0, 0, 0" 1.0 1.0 0.0 0 0 0 0))
      (:then_2
        (Variables|/Game/BP/Mode/01_Play/BP_PlayCharacter.BP_PlayCharacter_C|SetPhyTime _asbp_play_character (Variables|Default|GetPhyTime))))))

(event EventBeginPlay)

(event Collision|EventActorBeginOverlap
  (params (OtherActor :type Actor%20Object%20Reference)))

(event EventTick
  (params (DeltaSeconds :type Float%20%28single-precision%29))
  (switch Utilities|FlowControl|Switch|SwitchonEPunchState (Variables|Default|GetCurPunchState)
    (:DELAY
      (Networking|SwitchHasAuthority
        (:Authority
          (Utilities|FlowControl|Delay (Variables|Default|GetDelayTime))
          (Variables|Default|SetCurPunchState "FIRE"))))
    (:FIRE
      (bind _islimit (CallFunction|CheckLimitPos (Variables|Default|GetCurPunchState)))
      (if _islimit
        (Class|ObsMovementActorComponent|MoveOnce (Variables|Default|GetObstacleMoveComp) (Variables|Default|GetPunch) (Variables|Default|GetFireSpeed) (Variables|Default|GetLimitPos) DeltaSeconds)
        (else
          (Variables|Default|SetCurPunchState "RECOVER"))))
    (:RECOVER
      (bind _islimit_2 (CallFunction|CheckLimitPos (Variables|Default|GetCurPunchState)))
      (if _islimit_2
        (Class|ObsMovementActorComponent|MoveOnce (Variables|Default|GetObstacleMoveComp) (Variables|Default|GetPunch) (Variables|Default|GetRecoverSpeed) "0.000000,340.000000,0.000000" DeltaSeconds)
        (else
          (Variables|Default|SetCurPunchState "DELAY"))))))

(fn ConstructionScript)

(fn CheckLimitPos
  (params (CurPunchState :type EPunchState%20Enum :default "DELAY"))
  (switch Utilities|FlowControl|Switch|SwitchonEPunchState CurPunchState
    (:FIRE
      (return (<= (.y (Variables|/Script/Engine.SceneComponent|GetRelativeLocation (Variables|Default|GetPunch))) (.y (Variables|Default|GetLimitPos)))))
    (:RECOVER
      (return (>= (.y (Variables|/Script/Engine.SceneComponent|GetRelativeLocation (Variables|Default|GetPunch))) 3.4e+02)))))

(fn SetSound
  (Audio|CreateSound2D "/Game/Resources/Level/Race/Sound/SFX/Generic_Player_Hit__Nr__4___Fall_Guys_Sound__-_Sound_Effect_for_editing__mp3cut_net_.Generic_Player_Hit__Nr__4___Fall_Guys_Sound__-_Sound_Effect_for_editing__mp3cut_net_" 1.0 1.0 0.0 0 false false))