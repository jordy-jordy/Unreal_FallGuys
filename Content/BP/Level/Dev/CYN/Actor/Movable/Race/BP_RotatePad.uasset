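; BP_RotatePad is a movable race-level obstacle that repeatedly tilts around its Axis component and returns to rest.
; Tick runs a three-state cycle: wait DelayTime, spin at RotateSpeed, then spin back at RecoverSpeed.
; ObstacleMoveComp.SpinOnce performs the rotation, while CheckLimit compares the Axis roll against LimitAngle or zero to switch states.
; An older version using AddRelativeRotation directly remains disconnected.
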(event EventBeginPlay)

(event Collision|EventActorBeginOverlap
  (params (OtherActor :type Actor%20Object%20Reference)))

(event EventTick
  (params (DeltaSeconds :type Float%20%28single-precision%29))
  (switch Utilities|FlowControl|Switch|SwitchonERotateState (Variables|Default|GetRotateState)
    (:DELAY
      (Utilities|FlowControl|Delay (Variables|Default|GetDelayTime))
      (Variables|Default|SetRotateState "MOVEUP"))
    (:MOVEUP
      (bind _islimit (CallFunction|CheckLimit (Variables|Default|GetRotateState)))
      (if _islimit
        (Class|ObsMovementActorComponent|SpinOnce (Variables|Default|GetObstacleMoveComp) (Variables|Default|GetAxis) (Variables|Default|GetRotateSpeed) (Variables|Default|GetLimitAngle) DeltaSeconds)
        (else
          (Variables|Default|SetRotateState "MOVEDOWN"))))
    (:MOVEDOWN
      (bind _islimit_2 (CallFunction|CheckLimit (Variables|Default|GetRotateState)))
      (if _islimit_2
        (Class|ObsMovementActorComponent|SpinOnce (Variables|Default|GetObstacleMoveComp) (Variables|Default|GetAxis) (Variables|Default|GetRecoverSpeed) (Variables|Default|GetLimitAngle) DeltaSeconds)
        (else
          (Variables|Default|SetRotateState "DELAY"))))))

(fn ConstructionScript)

(fn CheckLimit
  (params (CurRotateState :type ERotateState%20Enum :default "DELAY"))
  (switch Utilities|FlowControl|Switch|SwitchonERotateState CurRotateState
    (:MOVEUP
      (return (>= (.roll (Variables|/Script/Engine.SceneComponent|GetRelativeRotation (Variables|Default|GetAxis))) (.roll (Variables|Default|GetLimitAngle)))))
    (:MOVEDOWN
      (return (<= (.roll (Variables|/Script/Engine.SceneComponent|GetRelativeRotation (Variables|Default|GetAxis))) 0.0)))))