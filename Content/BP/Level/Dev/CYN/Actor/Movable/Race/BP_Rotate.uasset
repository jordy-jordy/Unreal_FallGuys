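; BP_Rotate is a movable level actor, filed under Race, that repeatedly swings its Axis component up and back on roll.
; Tick runs a RotateState machine that waits DelayTime, then rolls negatively at RotateSpeed until CheckMoveUp fails.
; It then rolls back at ReCoverSpeed until CheckMoveDown fails, and returns to the delay state.
; Both rotations scale by DeltaSeconds, and the wait is a latent Delay called from Tick.
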(event EventBeginPlay)

(event Collision|EventActorBeginOverlap
  (params (OtherActor :type Actor%20Object%20Reference)))

(event EventTick
  (params (DeltaSeconds :type Float%20%28single-precision%29))
  (switch Utilities|FlowControl|Switch|SwitchonERotateState (Variables|Default|GetRotateState)
    (:DELAY
      (Utilities|FlowControl|Delay (Variables|Default|GetDelayTime))
      (Variables|Default|SetRotateState "MOVEUP"))
    (:MOVEUP
      (bind _returnvalue (Class|RotatePad|CheckMoveUp))
      (if _returnvalue
        (Transformation|AddRelativeRotation (Variables|Default|GetAxis) (Math|Rotator|MakeRotator (* (* (Variables|Default|GetRotateSpeed) -1.0) DeltaSeconds) 0.0 0.0) false false)
        (else
          (Variables|Default|SetRotateState "MOVEDOWN"))))
    (:MOVEDOWN
      (bind _returnvalue_2 (Class|RotatePad|CheckMoveDown))
      (if _returnvalue_2
        (Transformation|AddRelativeRotation (Variables|Default|GetAxis) (Math|Rotator|MakeRotator (* (Variables|Default|GetReCoverSpeed) DeltaSeconds) 0.0 0.0) false false)
        (else
          (Variables|Default|SetRotateState "DELAY"))))))

(fn ConstructionScript)