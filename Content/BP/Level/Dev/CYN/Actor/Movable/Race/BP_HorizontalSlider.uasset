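; BP_HorizontalSlider is a moving race obstacle whose Slider component travels back and forth horizontally.
; On BeginPlay, the IsLeft flag on ObstacleMoveComp places the Slider at one of two mirrored X offsets to set its starting side.
; Each Tick delegates movement to ObstacleMoveComp's MoveCycle, cycling the Slider along the X axis using the MoveSpeed and LimitPos variables.
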(event EventBeginPlay
  (if (Variables|/Script/Unreal_FallGuys.ObsMovementActorComponent|GetIsLeft (Variables|Default|GetObstacleMoveComp))
    (Transformation|SetRelativeLocation (Variables|Default|GetSlider) "280.000000,0.000000,70.000000" false false)
    (else
      (Transformation|SetRelativeLocation (Variables|Default|GetSlider) "-280.000000,0.000000,70.000000" false false))))

(event Collision|EventActorBeginOverlap
  (params (OtherActor :type Actor%20Object%20Reference)))

(event EventTick
  (params (DeltaSeconds :type Float%20%28single-precision%29))
  (Class|ObsMovementActorComponent|MoveCycle (Variables|Default|GetObstacleMoveComp) (Variables|Default|GetSlider) (Variables|Default|GetMoveSpeed) (Variables|Default|GetLimitPos) "X" DeltaSeconds))

(fn ConstructionScript)