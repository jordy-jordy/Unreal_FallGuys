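; Spinning stick obstacle for the Jump ShowDown level, with a big stick and a small stick that rotate after the countdown.
; Once the countdown is over and IsRoateSpeedUp is false, Tick waits one second, then rotates both sticks at their yaw speeds scaled by DeltaSeconds.
; AddSpeed, which raises both speeds in opposite directions up to clamps, and the rotate helper functions are called only from disconnected nodes.
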(event EventBeginPlay)

(event Collision|EventActorBeginOverlap
  (params (OtherActor :type Actor%20Object%20Reference)))

(event EventTick
  (params (DeltaSeconds :type Float%20%28single-precision%29))
  (bind _returnvalue (Class|FallGlobal|GetIsCountDownOver))
  (if (and _returnvalue (not (Variables|Default|GetIsRoateSpeedUp)))
    (if (Variables|Default|GetIsStart)
      (Utilities|FlowControl|Sequence
        (:then_0
          (Transformation|AddRelativeRotation (Variables|Default|GetBigStick) (* (Variables|Default|GetStartSpeed_Big) DeltaSeconds) false false))
        (:then_1
          (Transformation|AddRelativeRotation (Variables|Default|GetSmallStick) (* (Variables|Default|GetStartSpeed_Small) DeltaSeconds) false false)))
      (else
        (Utilities|FlowControl|Delay 1.0)
        (Variables|Default|SetIsStart true)))))

(fn ConstructionScript)

(fn AddSpeed
  (Utilities|FlowControl|Sequence
    (:then_0
      (if (>= (+ (.yaw (Variables|Default|GetStartSpeed_Big)) (.yaw (Variables|Default|GetAccSpeed))) 9e+01)
        (Variables|Default|SetStartSpeed_Big "0.000000,90.000000,0.000000")
        (else
          (Variables|Default|SetStartSpeed_Big (Math|Rotator|MakeRotator 0.0 0.0 (+ (.yaw (Variables|Default|GetStartSpeed_Big)) (.yaw (Variables|Default|GetAccSpeed))))))))
    (:then_1
      (if (<= (+ (.yaw (Variables|Default|GetStartSpeed_Small)) (* (.yaw (Variables|Default|GetAccSpeed)) -1.0)) -1e+02)
        (Variables|Default|SetStartSpeed_Small "0.000000,-100.000000,0.000000")
        (else
          (Variables|Default|SetStartSpeed_Small (Math|Rotator|MakeRotator 0.0 0.0 (+ (.yaw (Variables|Default|GetStartSpeed_Small)) (* (.yaw (Variables|Default|GetAccSpeed)) -1.0)))))))))

(fn RotateBigStick
  (params (B :type Float%20%28single-precision%29))
  (Transformation|AddRelativeRotation (Variables|Default|GetBigStick) (* (Variables|Default|GetStartSpeed_Big) B) false false))

(fn RotateSmallSitck
  (params (B :type Float%20%28single-precision%29))
  (Transformation|AddRelativeRotation (Variables|Default|GetSmallStick) (* (Variables|Default|GetStartSpeed_Small) B) false false))