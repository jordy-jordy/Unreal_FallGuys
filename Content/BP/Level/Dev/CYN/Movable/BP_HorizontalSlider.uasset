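; BP_HorizontalSlider is a movable level piece whose Slider component shuttles back and forth along its local X axis.
; BeginPlay places the Slider at the left or right limit according to IsStartLeft.
; Tick moves it a fixed step per frame without delta-time scaling or sweep, flipping IsLeft past either limit, so speed depends on frame rate.
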(event EventBeginPlay
  (if (Variables|Default|GetIsStartLeft)
    (Transformation|SetRelativeLocation (Variables|Default|GetSlider) "-280.000000,0.000000,70.000000" false false)
    (else
      (Transformation|SetRelativeLocation (Variables|Default|GetSlider) "280.000000,0.000000,70.000000" false false))))

(event Collision|EventActorBeginOverlap
  (params (OtherActor :type Actor%20Object%20Reference)))

(event EventTick
  (params (DeltaSeconds :type Float%20%28single-precision%29))
  (bind _slider (Variables|Default|GetSlider))
  (bind _slider_2 (Variables|Default|GetSlider))
  (if (Variables|Default|GetIsLeft)
    (if (>= (.x (Variables|/Script/Engine.SceneComponent|GetRelativeLocation _slider_2)) -2.8e+02)
      (Transformation|AddRelativeLocation _slider_2 "-7.000000,0.000000,0.000000" false false)
      (else
        (Variables|Default|SetIsLeft false)))
    (elif (<= (.x (Variables|/Script/Engine.SceneComponent|GetRelativeLocation _slider)) 2.8e+02)
      (Transformation|AddRelativeLocation _slider "7.000000,0.000000,0.000000" false false)
      (else
        (Variables|Default|SetIsLeft true)))))

(fn ConstructionScript)