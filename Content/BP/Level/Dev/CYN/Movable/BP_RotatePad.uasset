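; BP_RotatePad is a level pad actor that periodically rotates up to about -85 degrees of pitch and back to level.
; BeginPlay picks the pause length between cycles from one of three CaseType presets.
; Tick drives the cycle with IsMove and IsUp flags, applying separate up and down rotation speeds scaled by delta time.
; While idle, Tick relies on a latent Delay to start the next swing.
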(event EventBeginPlay
  (switch int (Variables|Default|GetCaseType)
    (:0
      (Variables|Default|SetDelayTime 4.0))
    (:1
      (Variables|Default|SetDelayTime 6.0))
    (:2
      (Variables|Default|SetDelayTime 8.0))))

(event Collision|EventActorBeginOverlap
  (params (OtherActor :type Actor%20Object%20Reference)))

(event EventTick
  (params (DeltaSeconds :type Float%20%28single-precision%29))
  (if (Variables|Default|GetIsMove)
    (if (Variables|Default|GetIsUp)
      (if (>= (.pitch (Transformation|GetActorRotation)) -85.0)
        (Transformation|AddActorLocalRotation (* (Variables|Default|GetUpSpeed) DeltaSeconds) false false)
        (else
          (Variables|Default|SetIsUp false)))
      (elif (<= (.pitch (Transformation|GetActorRotation)) 0.0)
        (Transformation|AddActorLocalRotation (* (Variables|Default|GetDownSpeed) DeltaSeconds) false false)
        (else
          (Variables|Default|SetIsUp true)
          (Variables|Default|SetIsMove false))))
    (else
      (Utilities|FlowControl|Delay (Variables|Default|GetDelayTime))
      (Variables|Default|SetIsMove true)
      (Variables|Default|SetIsUp true))))

(fn ConstructionScript)