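; BP_RotateRoller is a movable level actor with a roller that spins while its axis swings back and forth.
; Each Tick, RotateAxis steps between roll limits in both directions, flipping IsLeft at each end, while RotateRoller spins in the matching direction.
; Rotation uses fixed per-frame increments without delta time, so speed depends on frame rate.
; The Box hit event casts to BP_PlayCharacter but does nothing further.
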(event OnComponentHit(Box)
  (params (HitComponent :type Primitive%20Component%20Object%20Reference) (OtherActor :type Actor%20Object%20Reference) (OtherComp :type Primitive%20Component%20Object%20Reference) (NormalImpulse :type Vector :default "0, 0, 0") (Hit :type Hit%20Result%20Structure%20%28by%20ref%29))
  (Utilities|Casting|CastToBP_PlayCharacter OtherActor))

(event EventBeginPlay)

(event Collision|EventActorBeginOverlap
  (params (OtherActor :type Actor%20Object%20Reference)))

(event EventTick
  (params (DeltaSeconds :type Float%20%28single-precision%29))
  (if (Variables|Default|GetIsLeft)
    (Utilities|FlowControl|Sequence
      (:then_0
        (if (>= (.roll (Variables|/Script/Engine.SceneComponent|GetRelativeRotation (Variables|Default|GetRotateAxis))) 7e+01)
          (Variables|Default|SetIsLeft false)
          (else
            (Transformation|AddRelativeRotation (Variables|Default|GetRotateAxis) "0.000000,0.000000,0.700000" false false))))
      (:then_1
        (Transformation|AddRelativeRotation (Variables|Default|GetRotateRoller) "0.000000,0.000000,1.000000" false false)))
    (else
      (Utilities|FlowControl|Sequence
        (:then_0
          (Transformation|AddRelativeRotation (Variables|Default|GetRotateRoller) "0.000000,0.000000,-1.000000" false false))
        (:then_1
          (if (<= (.roll (Variables|/Script/Engine.SceneComponent|GetRelativeRotation (Variables|Default|GetRotateAxis))) -7e+01)
            (Variables|Default|SetIsLeft true)
            (else
              (Transformation|AddRelativeRotation (Variables|Default|GetRotateAxis) "0.000000,0.000000,-0.700000" false false))))))))

(fn ConstructionScript)