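; Swinging pink hammer obstacle that rocks back and forth and affects player characters it hits.
; Tick flips MoveLeft when roll passes 60 degrees either side and adds fixed rotation steps through both Sequence pins, so the swing is frame-rate dependent.
; A Box hit sets PhyTime on BP_PlayCharacter to 1.
; Directional LaunchCharacter knockback logic exists but is disconnected and never runs.
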(event OnComponentHit(Box)
  (params (HitComponent :type Primitive%20Component%20Object%20Reference) (OtherActor :type Actor%20Object%20Reference) (OtherComp :type Primitive%20Component%20Object%20Reference) (NormalImpulse :type Vector :default "0, 0, 0") (Hit :type Hit%20Result%20Structure%20%28by%20ref%29))
  (bind _asbp_play_character (Utilities|Casting|CastToBP_PlayCharacter OtherActor))
  (Variables|/Game/BP/Mode/01_Play/BP_PlayCharacter.BP_PlayCharacter_C|SetPhyTime _asbp_play_character 1.0))

(event EventBeginPlay)

(event EventTick
  (params (DeltaSeconds :type Float%20%28single-precision%29))
  (Utilities|FlowControl|Sequence
    (:then_0
      (if (>= (.roll (Variables|/Script/Engine.SceneComponent|GetRelativeRotation (Variables|Default|GetPinkHammer))) -6e+01)
        _
        (else
          (Variables|Default|SetMoveLeft false))))
    (:then_1
      (if (<= (.roll (Variables|/Script/Engine.SceneComponent|GetRelativeRotation (Variables|Default|GetPinkHammer))) 6e+01)
        _
        (else
          (Variables|Default|SetMoveLeft true)))))
  (if (Variables|Default|GetMoveLeft)
    (Transformation|AddRelativeRotation (Variables|Default|GetPinkHammer) "0.000000,0.000000,-0.500000" false false)
    (else
      (Transformation|AddRelativeRotation (Variables|Default|GetPinkHammer) "0.000000,0.000000,0.500000" false false))))

(fn ConstructionScript)