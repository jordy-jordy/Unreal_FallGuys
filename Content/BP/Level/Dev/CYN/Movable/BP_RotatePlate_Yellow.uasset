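; BP_RotatePlate_Yellow is a movable level actor: a plate that spins continuously around its yaw axis.
; Every Tick it adds relative yaw to the RotationPlate component, scaled by RotateSpeed and delta time for frame-rate-independent motion.
; The IsDirLeft flag picks the spin direction by keeping or negating the speed, while BeginPlay, overlap and construction logic are empty.
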(event EventBeginPlay)

(event Collision|EventActorBeginOverlap
  (params (OtherActor :type Actor%20Object%20Reference)))

(event EventTick
  (params (DeltaSeconds :type Float%20%28single-precision%29))
  (if (Variables|Default|GetIsDirLeft)
    (Transformation|AddRelativeRotation (Variables|Default|GetRotation%20Plate) (Math|Rotator|MakeRotator 0.0 0.0 (* (Variables|Default|GetRotateSpeed) DeltaSeconds)) false false)
    (else
      (Transformation|AddRelativeRotation (Variables|Default|GetRotation%20Plate) (Math|Rotator|MakeRotator 0.0 0.0 (* (* (Variables|Default|GetRotateSpeed) -1.0) DeltaSeconds)) false false))))

(fn ConstructionScript)