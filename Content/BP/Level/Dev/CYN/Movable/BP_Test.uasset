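; BP_Test is a rotating obstacle actor that pushes the player character away on contact.
; Tick yaws the root component at RotateSpeed, scaled by delta time, with IsLeft choosing the spin direction.
; When the static mesh hits a BP_PlayCharacter, it launches that character horizontally along the direction from the actor to the player with a small fixed strength.
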(event OnComponentHit(StaticMesh)
  (params (HitComponent :type Primitive%20Component%20Object%20Reference) (OtherActor :type Actor%20Object%20Reference) (OtherComp :type Primitive%20Component%20Object%20Reference) (NormalImpulse :type Vector :default "0, 0, 0") (Hit :type Hit%20Result%20Structure%20%28by%20ref%29))
  (bind _asbp_play_character (Utilities|Casting|CastToBP_PlayCharacter OtherActor))
  (Character|LaunchCharacter _asbp_play_character (Math|Vector|MakeVector (.x (* (Math|Vector|GetUnitDirection(Vector) (Transformation|GetActorLocation) (Transformation|GetActorLocation _asbp_play_character)) 8e+01)) (.y (* (Math|Vector|GetUnitDirection(Vector) (Transformation|GetActorLocation) (Transformation|GetActorLocation _asbp_play_character)) 8e+01)) 0.0) false false))

(event EventBeginPlay)

(event Collision|EventActorBeginOverlap
  (params (OtherActor :type Actor%20Object%20Reference)))

(event EventTick
  (params (DeltaSeconds :type Float%20%28single-precision%29))
  (if (Variables|Default|GetIsLeft)
    (Transformation|AddRelativeRotation (Variables|Default|GetDefaultSceneRoot) (Math|Rotator|MakeRotator 0.0 0.0 (* (Variables|Default|GetRotateSpeed) DeltaSeconds)) false false)
    (else
      (Transformation|AddRelativeRotation (Variables|Default|GetDefaultSceneRoot) (Math|Rotator|MakeRotator 0.0 0.0 (* (* (Variables|Default|GetRotateSpeed) -1.0) DeltaSeconds)) false false))))

(fn ConstructionScript)