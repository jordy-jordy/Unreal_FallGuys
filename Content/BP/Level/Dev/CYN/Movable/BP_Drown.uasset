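; BP_Drown is a level actor for an indicator drone ("Drown") that comes in blue, red and mint variants.
; On BeginPlay, SetDrownMesh switches on DrownType and assigns the matching static meshes to the body, both propellers, light and light arrow.
; The swap runs only at runtime, as the construction script is empty, and the file contains no movement or overlap logic.
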(event EventBeginPlay
  (CallFunction|SetDrownMesh))

(event Collision|EventActorBeginOverlap
  (params (OtherActor :type Actor%20Object%20Reference)))

(event EventTick
  (params (DeltaSeconds :type Float%20%28single-precision%29)))

(fn ConstructionScript)

(fn SetDrownMesh
  ;[0.15 0.15 0.15 0.5] SetDrownMesh
  (switch Utilities|FlowControl|Switch|SwitchonEDrownType (Variables|Default|GetDrownType)
    (:BLUE
      ;;[0.01829 0.05861 0.15 0.5] SetBlueDrown
      (Utilities|FlowControl|Sequence
        (:then_0
          (Components|StaticMesh|SetStaticMesh (Variables|Default|GetDrownBody) "/Game/Platformer_2/Meshes/SM_indicator_001.SM_indicator_001"))
        (:then_1
          (Components|StaticMesh|SetStaticMesh (Variables|Default|GetDrownPropeller_Left) "/Game/Platformer_2/Meshes/SM_indicator_propeller_2_001.SM_indicator_propeller_2_001"))
        (:then_2
          (Components|StaticMesh|SetStaticMesh (Variables|Default|GetDrownPropeller_Right) "/Game/Platformer_2/Meshes/SM_indicator_propeller_1_001.SM_indicator_propeller_1_001"))
        (:then_3
          (Components|StaticMesh|SetStaticMesh (Variables|Default|GetDrownLight) "/Game/Platformer_2/Meshes/SM_indicator_light_001.SM_indicator_light_001"))
        (:then_4
          (Components|StaticMesh|SetStaticMesh (Variables|Default|GetDrownLightArrow) "/Game/Platformer_2/Meshes/SM_indicator_arrow_001.SM_indicator_arrow_001"))))
    (:RED
      ;;[0.15 0.00895 0.0194 0.5] SetRedDrown
      (Utilities|FlowControl|Sequence
        (:then_0
          (Components|StaticMesh|SetStaticMesh (Variables|Default|GetDrownBody) "/Game/Platformer_2/Meshes/SM_indicator_002.SM_indicator_002"))
        (:then_1
          (Components|StaticMesh|SetStaticMesh (Variables|Default|GetDrownPropeller_Left) "/Game/Platformer_2/Meshes/SM_indicator_propeller_2_002.SM_indicator_propeller_2_002"))
        (:then_2
          (Components|StaticMesh|SetStaticMesh (Variables|Default|GetDrownPropeller_Right) "/Game/Platformer_2/Meshes/SM_indicator_propeller_1_002.SM_indicator_propeller_1_002"))
        (:then_3
          (Components|StaticMesh|SetStaticMesh (Variables|Default|GetDrownLight) "/Game/Platformer_2/Meshes/SM_indicator_light_002.SM_indicator_light_002"))
        (:then_4
          (Components|StaticMesh|SetStaticMesh (Variables|Default|GetDrownLightArrow) "/Game/Platformer_2/Meshes/SM_indicator_arrow_002.SM_indicator_arrow_002"))))
    (:MINT
      ;;[0.02099 0.126 0.15 0.5] SetMintDrown
      (Utilities|FlowControl|Sequence
        (:then_0
          (Components|StaticMesh|SetStaticMesh (Variables|Default|GetDrownBody) "/Game/Platformer_2/Meshes/SM_indicator_003.SM_indicator_003"))
        (:then_1
          (Components|StaticMesh|SetStaticMesh (Variables|Default|GetDrownPropeller_Left) "/Game/Platformer_2/Meshes/SM_indicator_propeller_2_003.SM_indicator_propeller_2_003"))
        (:then_2
          (Components|StaticMesh|SetStaticMesh (Variables|Default|GetDrownPropeller_Right) "/Game/Platformer_2/Meshes/SM_indicator_propeller_1_003.SM_indicator_propeller_1_003"))
        (:then_3
          (Components|StaticMesh|SetStaticMesh (Variables|Default|GetDrownLight) "/Game/Platformer_2/Meshes/SM_indicator_light_003.SM_indicator_light_003"))
        (:then_4
          (Components|StaticMesh|SetStaticMesh (Variables|Default|GetDrownLightArrow) "/Game/Platformer_2/Meshes/SM_indicator_arrow_003.SM_indicator_arrow_003"))))))