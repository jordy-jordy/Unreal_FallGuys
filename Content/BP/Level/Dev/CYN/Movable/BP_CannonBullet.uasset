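; BP_CannonBullet is a cannon projectile actor that knocks the player character away on contact and has a limited lifetime.
; When the CannonBullet component begins overlapping a BP_PlayCharacter, it launches that character along the bullet-to-player direction scaled by LaunchForce, with vertical velocity set to JumpForce.
; Tick drives a Delay of ActiveTime that ends in DestroyActor, so the bullet is not destroyed on hit.
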(event OnComponentBeginOverlap(CannonBullet)
  (params (OverlappedComponent :type Primitive%20Component%20Object%20Reference) (OtherActor :type Actor%20Object%20Reference) (OtherComp :type Primitive%20Component%20Object%20Reference) (OtherBodyIndex :type Integer) (bFromSweep :type Boolean) (SweepResult :type Hit%20Result%20Structure%20%28by%20ref%29))
  (bind _asbp_play_character (Utilities|Casting|CastToBP_PlayCharacter OtherActor))
  (Character|LaunchCharacter _asbp_play_character (Math|Vector|MakeVector (.x (* (Math|Vector|GetUnitDirection(Vector) (Transformation|GetActorLocation) (Transformation|GetActorLocation _asbp_play_character)) (Variables|Default|GetLaunch%20Force))) (.y (* (Math|Vector|GetUnitDirection(Vector) (Transformation|GetActorLocation) (Transformation|GetActorLocation _asbp_play_character)) (Variables|Default|GetLaunch%20Force))) (Variables|Default|GetJump%20Force)) false false))

(event EventBeginPlay)

(event Collision|EventActorBeginOverlap
  (params (OtherActor :type Actor%20Object%20Reference)))

(event EventTick
  (params (DeltaSeconds :type Float%20%28single-precision%29))
  (Utilities|FlowControl|Delay (Variables|Default|GetActiveTime))
  (Actor|DestroyActor))

(fn ConstructionScript)