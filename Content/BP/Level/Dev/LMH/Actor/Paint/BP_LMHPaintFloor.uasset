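; A paintable floor actor that turns blue when a player character touches it.
; On BeginPlay the authority assigns the first player controller as the actor's owner.
; When a BP_PlayCharacter begins overlapping the Box, the Cube gets a new dynamic instance of the paintable ground material with its Color parameter set to blue.
; The color change runs locally in the overlap event, with no RPC or replication step in the graph.
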(event OnComponentBeginOverlap(Box)
  (params (OverlappedComponent :type Primitive%20Component%20Object%20Reference) (OtherActor :type Actor%20Object%20Reference) (OtherComp :type Primitive%20Component%20Object%20Reference) (OtherBodyIndex :type Integer) (bFromSweep :type Boolean) (SweepResult :type Hit%20Result%20Structure%20%28by%20ref%29))
  (Utilities|Casting|CastToBP_PlayCharacter OtherActor)
  (bind _returnvalue (Rendering|Material|CreateDynamicMaterialInstance (Variables|Default|GetCube) 0 "/Game/Resources/Level/Paint/Materials/MI_LMHPaintableGround.MI_LMHPaintableGround" "None" :!class /Script/Engine.PrimitiveComponent))
  (Variables|Default|SetCubeColor _returnvalue)
  (Rendering|Material|SetVectorParameterValue (Variables|Default|GetCubeColor) "Color" (Variables|Default|GetBlue) :!class /Script/Engine.MaterialInstanceDynamic))

(event EventBeginPlay
  (Networking|SwitchHasAuthority
    (:Authority
      (Actor|SetOwner (Game|GetPlayerController 0)))))

(fn ConstructionScript)