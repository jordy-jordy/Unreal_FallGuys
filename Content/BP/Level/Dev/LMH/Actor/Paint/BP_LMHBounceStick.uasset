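; BP_LMHBounceStick is a level obstacle: a stick that slides back and forth and knocks players away on contact.
; On authority, Tick moves it along relative X, reversing whenever the speed-scaled timer exceeds TotalTime.
; Hits on BP_PlayCharacter launch it along the inverted impact normal with fixed lift, authority only, and play a random hit sound.
; The construction script tints two material slots through dynamic instances.
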(event OnComponentHit(BounceStick)
  (params (HitComponent :type Primitive%20Component%20Object%20Reference) (OtherActor :type Actor%20Object%20Reference) (OtherComp :type Primitive%20Component%20Object%20Reference) (NormalImpulse :type Vector :default "0, 0, 0") (Hit :type Hit%20Result%20Structure%20%28by%20ref%29))
  (bind _power (Variables|Default|GetPower))
  (bind _returnvalue (* (.impactnormal Hit) _power))
  (bind _returnvalue_2 (* _returnvalue -1.0))
  (Utilities|FlowControl|Sequence
    (:then_0
      (bind _asbp_play_character (Utilities|Casting|CastToBP_PlayCharacter OtherActor))
      (if (Ability|HasAuthority _asbp_play_character)
        (Character|LaunchCharacter _asbp_play_character (Math|Vector|MakeVector (.x _returnvalue_2) (.y _returnvalue_2) 2e+02) false false)))
    (:then_1
      (bind _asbp_play_character_2 (Utilities|Casting|CastToBP_PlayCharacter OtherActor))
      (bind _output_get (Variables|Default|SetHit%20Sound%20Index (Math|Random|RandomIntegerinRange 0 2)))
      (Networking|SwitchHasAuthority
        (:Authority
          _)
        (:Remote
          _))
      (switch int _output_get
        (:0
          (Audio|PlaySoundatLocation "/Game/Resources/Level/Race/Sound/SFX/Generic_Player_Hit__Nr__4___Fall_Guys_Sound__-_Sound_Effect_for_editing__mp3cut_net_.Generic_Player_Hit__Nr__4___Fall_Guys_Sound__-_Sound_Effect_for_editing__mp3cut_net_" (Transformation|GetActorLocation _asbp_play_character_2) "0, 0, 0" 1.0 1.0 0.0 0 0 0 0))
        (:1
          (Audio|PlaySoundatLocation "/Game/Resources/Level/Race/Sound/SFX/Generic_Player_Hit__Nr__6___Fall_Guys_Sound__-_Sound_Effect_for_editing__mp3cut_net_.Generic_Player_Hit__Nr__6___Fall_Guys_Sound__-_Sound_Effect_for_editing__mp3cut_net_" (Transformation|GetActorLocation _asbp_play_character_2) "0, 0, 0" 1.0 1.0 0.0 0 0 0 0))
        (:2
          (Audio|PlaySoundatLocation "/Game/Resources/Level/Race/Sound/SFX/Generic_Player_Hit__Nr__7___Fall_Guys_Sound__-_Sound_Effect_for_editing__mp3cut_net_.Generic_Player_Hit__Nr__7___Fall_Guys_Sound__-_Sound_Effect_for_editing__mp3cut_net_" (Transformation|GetActorLocation _asbp_play_character_2) "0, 0, 0" 1.0 1.0 0.0 0 0 0 0))))))

(event EventTick
  (params (DeltaSeconds :type Float%20%28single-precision%29))
  (bind _bouncestick (Variables|Default|GetBounceStick))
  (bind _speed (Variables|MainSettings|GetSpeed))
  (bind _returnvalue (* DeltaSeconds _speed))
  (Networking|SwitchHasAuthority
    (:Authority
      (Variables|Default|SetCurTime (+ (Variables|Default|GetCurTime) _returnvalue))
      (if (> (Variables|Default|GetCurTime) (Variables|Default|GetTotalTime))
        (Variables|Default|SetIsLeft (not (Variables|Default|GetIsLeft)))
        (Variables|Default|SetCurTime 0.0))
      (if (Variables|Default|GetIsLeft)
        (Transformation|AddRelativeLocation _bouncestick (Math|Vector|MakeVector (* _returnvalue -1.0) 0.0 0.0) false false)
        (else
          (Transformation|AddRelativeLocation _bouncestick (Math|Vector|MakeVector _returnvalue 0.0 0.0) false false))))))

(event EventBeginPlay
  (Networking|SwitchHasAuthority
    (:Authority
      (Actor|SetOwner (Game|GetPlayerController 0)))))

(fn ConstructionScript
  (bind _returnvalue (Rendering|Material|CreateDynamicMaterialInstance (Variables|Default|GetBounceStick) 0 0 "None" :!class /Script/Engine.PrimitiveComponent))
  (Rendering|Material|SetVectorParameterValue _returnvalue "Color" (Variables|Appearance|GetColor) :!class /Script/Engine.MaterialInstanceDynamic)
  (bind _returnvalue_2 (Rendering|Material|CreateDynamicMaterialInstance (Variables|Default|GetBounceStick) 1 0 "None" :!class /Script/Engine.PrimitiveComponent))
  (Rendering|Material|SetVectorParameterValue _returnvalue_2 "Color" (Variables|Appearance|GetColor%202) :!class /Script/Engine.MaterialInstanceDynamic))