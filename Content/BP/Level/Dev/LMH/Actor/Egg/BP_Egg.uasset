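; BP_Egg is an egg actor that tracks which team's goal it is sitting in.
; Every Tick on the authority, it gathers all BP_LMHEggGoal actors and checks overlap with each, setting Team to the goal's first tag as an integer, or -1 if not overlapping.
; The loop never breaks, so the last goal checked decides Team, and each result is printed for debugging.
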(event EventTick
  (params (DeltaSeconds :type Float%20%28single-precision%29))
  (Networking|SwitchHasAuthority
    (:Authority
      (bind _outactors (Actor|GetAllActorsOfClass "/Game/BP/Level/Dev/LMH/Actor/Collision/BP_LMHEggGoal.BP_LMHEggGoal_C"))
      (for _array_element _outactors
        (Utilities|FlowControl|Sequence
          (:then_0
            (if (Collision|IsOverlappingActor self _array_element :!class /Script/Engine.Actor)
              (Variables|Default|SetTeam (Math|Conversions|ToInteger(Byte) (Utilities|String|ToString(Name) (Utilities|Array|Get(acopy) (Variables|/Script/Engine.Actor|GetTags _array_element)))))
              (Development|PrintString (Utilities|String|ToString(Integer) (Math|Conversions|ToInteger(Byte) (Utilities|String|ToString(Name) (Utilities|Array|Get(acopy) (Variables|/Script/Engine.Actor|GetTags _array_element))))))
              (else
                (bind _output_get (Variables|Default|SetTeam -1))
                (Development|PrintString (Utilities|String|ToString(Integer) _output_get))))))))))

(fn ConstructionScript)