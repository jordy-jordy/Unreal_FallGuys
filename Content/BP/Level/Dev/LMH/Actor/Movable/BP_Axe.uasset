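; BP_Axe is a movable level actor that swings back and forth in pitch like a pendulum.
; Each Tick calls AddRotation, which flips IsLeft beyond 50 degrees either side and applies a fixed one-degree local pitch step in that direction.
; The swing is frame-rate dependent because delta time is unused, and AddTime is an empty stub.
; BeginPlay sets the first player controller as the actor's owner.
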(event EventTick
  (params (DeltaSeconds :type Float%20%28single-precision%29))
  (CallFunction|AddRotation DeltaSeconds))

(event EventBeginPlay
  (Actor|SetOwner (Game|GetPlayerController 0)))

(fn ConstructionScript)

(fn AddTime
  (params (Delta%20Seconds :type Float%20%28double-precision%29)))

(fn AddRotation
  (params (Delta :type Float%20%28double-precision%29))
  (bind _returnvalue (Transformation|GetActorRotation))
  (Utilities|FlowControl|Sequence
    (:then_0
      (if (> (.pitch _returnvalue) 5e+01)
        (Variables|Default|SetIsLeft false)
        (elif (< (.pitch _returnvalue) -5e+01)
          (Variables|Default|SetIsLeft true))))
    (:then_1
      (if (Variables|Default|GetIsLeft)
        (Transformation|AddActorLocalRotation (Math|Rotator|MakeRotator 0.0 1.0 0.0) false false)
        (else
          (Transformation|AddActorLocalRotation (Math|Rotator|MakeRotator 0.0 -1.0 0.0) false false))))))