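; BP_Cannon is a movable cannon actor that rotates continuously around its local yaw axis.
; Each Tick adds a yaw rotation of Speed scaled by delta time, with the TurnRight flag choosing the direction.
; On BeginPlay it sets player controller 0 as its owner; the graph contains no firing or aiming logic.
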(event EventBeginPlay
  (Actor|SetOwner (Game|GetPlayerController 0)))

(event Collision|EventActorBeginOverlap
  (params (OtherActor :type Actor%20Object%20Reference)))

(event EventTick
  (params (DeltaSeconds :type Float%20%28single-precision%29))
  (bind _speed (Variables|Default|GetSpeed))
  (if (Variables|Default|GetTurnRight)
    (Transformation|AddActorLocalRotation (Math|Rotator|MakeRotator 0.0 0.0 (* DeltaSeconds _speed)) false false)
    (else
      (Transformation|AddActorLocalRotation (Math|Rotator|MakeRotator 0.0 0.0 (* (* DeltaSeconds _speed) -1.0)) false false))))

(fn ConstructionScript)