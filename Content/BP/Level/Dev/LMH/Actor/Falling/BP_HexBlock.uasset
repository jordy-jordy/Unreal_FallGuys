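; BP_HexBlock is a falling-floor hexagon tile that disappears shortly after a player character steps on it.
; BeginPlay sets the first player controller as owner and, after a short delay, applies the tile's material.
; The first BP_PlayCharacter overlap nudges the mesh down, switches it to an active material, then destroys the actor after brief delays.
; Tick polls the end-game state, which blocks new triggers once set.
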(event EventBeginPlay
  (Actor|SetOwner (Game|GetPlayerController 0))
  (Utilities|FlowControl|Delay 0.5)
  (Rendering|Material|SetMaterial (Variables|Default|GetStaticMesh) 0 (Variables|Default|GetMaterial)))

(event Collision|EventActorBeginOverlap
  (params (OtherActor :type Actor%20Object%20Reference))
  (if (not (Variables|Default|GetIsEndGame))
    (Utilities|Casting|CastToBP_PlayCharacter OtherActor)
    (Utilities|FlowControl|DoOnce false
      (:Completed
        (Transformation|AddLocalOffset (Variables|Default|GetStaticMesh) "0.000000,0.000000,-5.000000" false false)
        (Utilities|FlowControl|Delay 0.2)
        (Rendering|Material|SetMaterial (Variables|Default|GetStaticMesh) 0 "/Game/Resources/Level/Falling/Materials/M_ENV_FloorFall_Hexagons_Active.M_ENV_FloorFall_Hexagons_Active")
        (Utilities|FlowControl|Delay 0.5)
        (Actor|DestroyActor)))))

(event EventTick
  (params (DeltaSeconds :type Float%20%28single-precision%29))
  (bind _returnvalue (Class|FallGlobal|GetIsEndGame))
  (Variables|Default|SetIsEndGame _returnvalue))

(fn ConstructionScript)