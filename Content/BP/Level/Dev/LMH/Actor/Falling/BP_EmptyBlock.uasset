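; BP_EmptyBlock is a block actor in the Falling level set that removes itself once a countdown is over.
; On BeginPlay, the authority sets the first player controller as its owner and applies the Material variable to its static mesh.
; Each Tick, only the authority polls GetIsCountDownOver and destroys the actor when it returns true.
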(event EventBeginPlay
  (Networking|SwitchHasAuthority
    (:Authority
      (Actor|SetOwner (Game|GetPlayerController 0))
      (Rendering|Material|SetMaterial (Variables|Default|GetStaticMesh) 0 (Variables|Default|GetMaterial)))))

(event EventTick
  (params (DeltaSeconds :type Float%20%28single-precision%29))
  (Networking|SwitchHasAuthority
    (:Authority
      (bind _returnvalue (Class|FallGlobal|GetIsCountDownOver))
      (if _returnvalue
        (Actor|DestroyActor)))))

(fn ConstructionScript)