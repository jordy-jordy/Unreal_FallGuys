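; BP_GoallColl_After is a finish-line trigger that handles player characters overlapping its box.
; It reports the finisher to BP_PlayGameMode, hides the capsule and its children, and sets movement mode to None.
; Only a locally controlled character calls SpectatorOn.
; BeginPlay sets player controller 0 as owner, and collision and physics nodes are left unconnected.
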(event OnComponentBeginOverlap(Box)
  (params (OverlappedComponent :type Primitive%20Component%20Object%20Reference) (OtherActor :type Actor%20Object%20Reference) (OtherComp :type Primitive%20Component%20Object%20Reference) (OtherBodyIndex :type Integer) (bFromSweep :type Boolean) (SweepResult :type Hit%20Result%20Structure%20%28by%20ref%29))
  (bind _asbp_play_character (Utilities|Casting|CastToBP_PlayCharacter OtherActor))
  (Utilities|FlowControl|Sequence
    (:then_1
      ;[0.1422 0.15 0.1374 0.5] 결승선에 닿은 플레이어 처리
      (bind _asbp_play_game_mode (Utilities|Casting|CastToBP_PlayGameMode (Game|GetGameMode)))
      (Class|PlayGameMode|OnPlayerFinished _asbp_play_game_mode _asbp_play_character))
    (:then_2
      (Rendering|SetVisibility (Variables|/Script/Engine.Character|GetCapsuleComponent _asbp_play_character) false true)
      (Pawn|Components|CharacterMovement|SetMovementMode (Variables|/Script/Engine.Character|GetCharacterMovement _asbp_play_character) "MOVE_None" 0))
    (:then_3
      (if (Pawn|IsLocallyControlled _asbp_play_character)
        (Class|PlayCharacter|Spectatoron _asbp_play_character)))))

(event EventBeginPlay
  (Actor|SetOwner (Game|GetPlayerController 0))
  (Utilities|FlowControl|Delay 0.7))

(fn ConstructionScript)