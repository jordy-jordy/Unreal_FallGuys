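; BP_KillZone is a box trigger that puts overlapping BP_PlayCharacter pawns out of play by hiding their mesh and disabling capsule collision.
; For a locally controlled character it sets IsDie on the game instance.
; The authority branch only casts to BP_PlayGameMode, as the OnPlayerFinished call is disconnected.
; BeginPlay sets the first player controller as owner, then runs a delay with nothing after it.
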(event OnComponentBeginOverlap(Box)
  (params (OverlappedComponent :type Primitive%20Component%20Object%20Reference) (OtherActor :type Actor%20Object%20Reference) (OtherComp :type Primitive%20Component%20Object%20Reference) (OtherBodyIndex :type Integer) (bFromSweep :type Boolean) (SweepResult :type Hit%20Result%20Structure%20%28by%20ref%29))
  (bind _asbp_play_character (Utilities|Casting|CastToBP_PlayCharacter OtherActor))
  (Rendering|SetVisibility (Variables|/Script/Engine.Character|GetMesh _asbp_play_character) false false)
  (Collision|SetCollisionEnabled (Variables|/Script/Engine.Character|GetCapsuleComponent _asbp_play_character) "NoCollision")
  ;[0.15 0.15 0.15 0.5] 결승점 골인 Pawn 도착했음 설정
  (Utilities|FlowControl|Sequence
    (:then_0
      (if (Pawn|IsLocallyControlled _asbp_play_character)
        (bind _asbp_base_game_instance (Utilities|Casting|CastToBP_BaseGameInstance (Game|GetGameInstance)))
        (Variables|/Script/Unreal_FallGuys.BaseGameInstance|SetIsDie _asbp_base_game_instance true)))
    (:then_1
      (if (Ability|HasAuthority _asbp_play_character)
        ;[0.1422 0.15 0.1374 0.5] 생존 플레이어수 마이너스
        (bind _asbp_play_game_mode (Utilities|Casting|CastToBP_PlayGameMode (Game|GetGameMode)))))))

(event EventBeginPlay
  (Actor|SetOwner (Game|GetPlayerController 0))
  (Utilities|FlowControl|Delay 0.7))

(fn ConstructionScript)