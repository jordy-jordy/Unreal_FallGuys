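; BP_RespawnColl is a dead-zone collision actor that sends a player character back to its saved RespawnPos.
; On the server, the box overlap stores the BP_PlayCharacter and fires the S2M sound event.
; That event plays a respawn sound at RespawnPos, then moves the character there after a short delay.
; BeginPlay sets the first player controller as the actor's owner.
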(event OnComponentBeginOverlap(Box)
  (params (OverlappedComponent :type Primitive%20Component%20Object%20Reference) (OtherActor :type Actor%20Object%20Reference) (OtherComp :type Primitive%20Component%20Object%20Reference) (OtherBodyIndex :type Integer) (bFromSweep :type Boolean) (SweepResult :type Hit%20Result%20Structure%20%28by%20ref%29))
  ;[0.15 0.15 0.15 0.5] 캐릭터 DeadZone
  (Networking|SwitchHasAuthority
    (:Authority
      (bind _asbp_play_character (Utilities|Casting|CastToBP_PlayCharacter OtherActor))
      (CallFunction|S2MSoundMulti))))

(event Custom|S2M_SoundMulti
  ;[0.15 0.15 0.15 0.5] 캐릭터 DeadZone
  (Audio|PlaySoundatLocation "/Game/Resources/Level/Race/Sound/SFX/Player_Respawn__Fall_Guys_Sound__-_Sound_Effect_for_editing__mp3cut_net_.Player_Respawn__Fall_Guys_Sound__-_Sound_Effect_for_editing__mp3cut_net_" (Variables|/Game/BP/Mode/01_Play/BP_PlayCharacter.BP_PlayCharacter_C|GetRespawnPos (stale OnComponentBeginOverlap(Box) _asbp_play_character)) "0, 0, 0" 5.0 1.0 0.0 0 0 0 0)
  (Utilities|FlowControl|Delay 0.5)
  (Transformation|SetActorLocation (stale OnComponentBeginOverlap(Box) _asbp_play_character) (Variables|/Game/BP/Mode/01_Play/BP_PlayCharacter.BP_PlayCharacter_C|GetRespawnPos (stale OnComponentBeginOverlap(Box) _asbp_play_character)) false false))

(event EventBeginPlay
  (Networking|SwitchHasAuthority
    (:Authority
      _)
    (:Remote
      _))
  (Actor|SetOwner (Game|GetPlayerController 0)))

(fn ConstructionScript)