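; BP_GoallColl is a goal trigger volume that registers player characters reaching it.
; Box overlap hides the character's mesh and, for the locally controlled player, sets IsDie to false on the game instance.
; The game mode's OnPlayerFinished arrival count runs only when that character is both locally controlled and has authority.
; On BeginPlay the server makes player controller 0 its owner, followed by an unused delay.
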(event OnComponentBeginOverlap(Box)
  (params (OverlappedComponent :type Primitive%20Component%20Object%20Reference) (OtherActor :type Actor%20Object%20Reference) (OtherComp :type Primitive%20Component%20Object%20Reference) (OtherBodyIndex :type Integer) (bFromSweep :type Boolean) (SweepResult :type Hit%20Result%20Structure%20%28by%20ref%29))
  (bind _asbp_play_character (Utilities|Casting|CastToBP_PlayCharacter OtherActor))
  (Rendering|SetVisibility (Variables|/Script/Engine.Character|GetMesh _asbp_play_character) false false)
  (if (Pawn|IsLocallyControlled _asbp_play_character)
    (bind _asbp_base_game_instance (Utilities|Casting|CastToBP_BaseGameInstance (Game|GetGameInstance)))
    (Variables|/Script/Unreal_FallGuys.BaseGameInstance|SetIsDie _asbp_base_game_instance false)
    (if (Ability|HasAuthority _asbp_play_character)
      ;[0.1422 0.15 0.1374 0.5] 도착 플레이어수 카운트
      (bind _asbp_play_game_mode (Utilities|Casting|CastToBP_PlayGameMode (Game|GetGameMode)))
      (Class|PlayGameMode|OnPlayerFinished _asbp_play_game_mode))))

(event EventBeginPlay
  (Networking|SwitchHasAuthority
    (:Authority
      (Actor|SetOwner (Game|GetPlayerController 0))
      (Utilities|FlowControl|Delay 0.7))))

(fn ConstructionScript)