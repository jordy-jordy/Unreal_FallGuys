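; BP_Propeller is a short-lived actor in the Rhino dev folder that flies straight up while its propeller spins.
; On BeginPlay it makes the first player controller its owner.
; Tick accumulates elapsed time, yaws the Propeller component and lifts the actor along world Z at constant, frame-rate-independent speeds.
; Once the elapsed time exceeds FullTime, the actor destroys itself.
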(event Collision|EventActorBeginOverlap
  (params (OtherActor :type Actor%20Object%20Reference)))

(event EventTick
  (params (DeltaSeconds :type Float%20%28single-precision%29))
  (Variables|Default|SetCurTime (+ (Variables|Default|GetCurTime) DeltaSeconds))
  (Transformation|AddRelativeRotation (Variables|Default|GetPropeller) (Math|Rotator|MakeRotator 0.0 0.0 (* DeltaSeconds 5e+02)) false false)
  (if (> (Variables|Default|GetCurTime) (Variables|Default|GetFullTime))
    (Actor|DestroyActor)
    (else
      (Transformation|AddActorWorldOffset (Math|Vector|MakeVector 0.0 0.0 (* DeltaSeconds 2e+02))))))

(event EventBeginPlay
  (Actor|SetOwner (Game|GetPlayerController 0)))

(fn ConstructionScript)