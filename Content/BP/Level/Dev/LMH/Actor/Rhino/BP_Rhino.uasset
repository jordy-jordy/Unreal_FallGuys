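; Rhino character that targets the nearest player and charges at them after a wind-up pause.
; Tick runs a charge cooldown that triggers a timed stop, after which the charge flag turns on and is never cleared here.
; Outside the stop, it scans all BP_PlayCharacter actors each frame, yaws toward the closest and, when charging, drives forward movement input.
; CurAnimation tracks the stop, idle and charge states.
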(event EventBeginPlay)

(event Collision|EventActorBeginOverlap
  (params (OtherActor :type Actor%20Object%20Reference)))

(event EventTick
  (params (DeltaSeconds :type Float%20%28single-precision%29))
  (Variables|Default|SetChargeCoolTime (- (Variables|Default|GetChargeCoolTime) DeltaSeconds))
  (if (< (Variables|Default|GetChargeCoolTime) 0.0)
    (Variables|Default|SetIsStop true)
    (Variables|Default|SetChargeCoolTime 1e+01)
    (elif (Variables|Default|GetIsStop)
      (Variables|Default|SetCurAnimation "Stop")
      (Variables|Default|SetStopTime (- (Variables|Default|GetStopTime) DeltaSeconds))
      (if (< (Variables|Default|GetStopTime) 0.0)
        (Variables|Default|SetIsStop false)
        (Variables|Default|SetIsCharge true)
        (Variables|Default|SetStopTime 2.0))
      (else
        (if (Variables|Default|GetIsCharge)
          _
          (else
            _))
        (bind _outactors (Actor|GetAllActorsOfClass "/Game/BP/Mode/01_Play/BP_PlayCharacter.BP_PlayCharacter_C"))
        (for _array_element _outactors
          (if (< (Math|Vector|Distance(Vector) (Transformation|GetActorLocation _array_element) (Transformation|GetActorLocation)) (Variables|Default|GetClosestDistance))
            (Variables|Default|SetClosestPlayer _array_element)
            (Variables|Default|SetClosestDistance (Math|Vector|Distance(Vector) (Transformation|GetActorLocation _array_element) (Transformation|GetActorLocation)))))
        (Variables|Default|SetClosestDistance 9999999.0)
        (Variables|Default|SetPlayerNumber (Utilities|Array|Length _outactors))
        (Transformation|SetActorRotation (Math|Rotator|MakeRotator 0.0 0.0 (.yaw (Math|Rotator|FindLookatRotation (Transformation|GetActorLocation) (Transformation|GetActorLocation (Variables|Default|GetClosestPlayer))))))
        (if (Variables|Default|GetIsCharge)
          (Variables|Default|SetSpeed 3.0)
          (Pawn|Input|AddMovementInput (Math|Vector|GetForwardVector (Variables|Default|GetCapsule)) (Variables|Default|GetSpeed) false)
          (if (Class|KismetMathLibrary|EqualExactlyVectorVector (Transformation|GetVelocity) "0, 0, 0")
            (Variables|Default|SetCurAnimation "Idle")
            (elif (Variables|Default|GetIsCharge)
              (Variables|Default|SetCurAnimation "Charge")
              (else
                (Variables|Default|SetCurAnimation "Run"))))
          (else
            (Variables|Default|SetSpeed 1.0)))))))

(fn ConstructionScript)