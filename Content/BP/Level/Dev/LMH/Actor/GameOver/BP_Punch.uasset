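; BP_Punch is a level obstacle that repeatedly punches out on a spring and affects the player character it hits.
; Tick moves the Spring along local Y, extending quickly and retracting slowly, then waits on a Delay before the next cycle.
; IsLeft sets the Box orientation at BeginPlay, and a Box hit sets PhyTime on BP_PlayCharacter.
; The character launch logic is disconnected and never runs.
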(event OnComponentHit(Box)
  (params (HitComponent :type Primitive%20Component%20Object%20Reference) (OtherActor :type Actor%20Object%20Reference) (OtherComp :type Primitive%20Component%20Object%20Reference) (NormalImpulse :type Vector :default "0, 0, 0") (Hit :type Hit%20Result%20Structure%20%28by%20ref%29))
  (bind _asbp_play_character (Utilities|Casting|CastToBP_PlayCharacter OtherActor))
  (Variables|/Game/BP/Mode/01_Play/BP_PlayCharacter.BP_PlayCharacter_C|SetPhyTime _asbp_play_character 1.0))

(event EventBeginPlay
  (if (Variables|Default|GetIsLeft)
    (Transformation|SetRelativeRotation (Variables|Default|GetBox) "0.000000,180.000000,0.000000" false false)
    (else
      (Transformation|SetRelativeRotation (Variables|Default|GetBox) "0, 0, 0" false false))))

(event Collision|EventActorBeginOverlap
  (params (OtherActor :type Actor%20Object%20Reference)))

(event EventTick
  (params (DeltaSeconds :type Float%20%28single-precision%29))
  (bind _spring (Variables|Default|GetSpring))
  (bind _spring_2 (Variables|Default|GetSpring))
  (if (Variables|Default|GetIsMove)
    (if (Variables|Default|GetIsPush)
      (if (<= (.y (Variables|/Script/Engine.SceneComponent|GetRelativeLocation _spring_2)) 5.2e+02)
        (Transformation|AddRelativeLocation _spring_2 "0.000000,30.000000,0.000000" false false)
        (else
          (Variables|Default|SetIsPush false)))
      (elif (>= (.y (Variables|/Script/Engine.SceneComponent|GetRelativeLocation _spring)) 2.2e+02)
        (Transformation|AddRelativeLocation _spring "0.000000,-5.000000,0.000000" false false)
        (else
          (Variables|Default|SetIsPush true)
          (Variables|Default|SetIsMove false))))
    (else
      (Utilities|FlowControl|Delay 3.0)
      (Variables|Default|SetIsMove true)
      (Variables|Default|SetIsPush true))))

(fn ConstructionScript)