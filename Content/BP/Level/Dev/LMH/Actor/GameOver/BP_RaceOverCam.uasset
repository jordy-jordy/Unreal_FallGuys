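; BP_RaceOverCam is a game-over camera actor that takes over the player's view when the race ends.
; On BeginPlay it sets player controller 0 as its owner, waits briefly, then calls S2M_SetViewTarget.
; That event blends player controller 0's view to this actor with an ease-out function.
; C2S_SetViewTarget forwards to the same event, with the prefixes suggesting a client-to-server, server-to-multicast RPC pair.
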(event Custom|C2S_SetViewTarget
  (CallFunction|S2MSetViewTarget))

(event Custom|S2M_SetViewTarget
  (Game|Player|SetViewTargetwithBlend (Game|GetPlayerController 0) self 0.0 "VTBlend_EaseOut" 0.0 false))

(event EventBeginPlay
  (Utilities|FlowControl|Sequence
    (:then_0
      (Actor|SetOwner (Game|GetPlayerController 0))
      (Utilities|FlowControl|Delay 2.0)
      (CallFunction|S2MSetViewTarget))))

(fn ConstructionScript)