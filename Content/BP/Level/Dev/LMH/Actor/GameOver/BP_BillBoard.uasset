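; BP_BillBoard is a level actor whose WBP_BillBoard widget receives the number of surviving players.
; On BeginPlay the authority assigns player controller 0 as owner of the actor and widget, then seeds PlayerCount with the connected player count.
; Every Tick, without an authority check, it counts BP_LMHRaceOverPlayerState entries in BP_PlayGameState's PlayerArray that are not IsDie and writes the total to the widget.
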(event EventBeginPlay
  (bind _returnvalue (Game|GetPlayerController 0))
  (Networking|SwitchHasAuthority
    (:Authority
      (Actor|SetOwner _returnvalue)
      (Class|UserWidget|SetOwningPlayer (UserInterface|GetWidget (Variables|Default|GetWidget)) _returnvalue)
      (bind _aswbp_bill_board (Utilities|Casting|CastToWBP_BillBoard (UserInterface|GetWidget (Variables|Default|GetWidget))))
      (bind _returnvalue_2 (Class|FallGlobal|GetConnectedPlayers))
      (Variables|/Game/BP/Level/Dev/LMH/UI/WBP_BillBoard.WBP_BillBoard_C|SetPlayerCount _aswbp_bill_board _returnvalue_2))))

(event EventTick
  (params (DeltaSeconds :type Float%20%28single-precision%29))
  (Utilities|FlowControl|Sequence
    (:then_0
      (bind _asbp_play_game_state (Utilities|Casting|CastToBP_PlayGameState (Game|GetGameState)))
      (for _array_element (Variables|/Script/Engine.GameStateBase|GetPlayerArray _asbp_play_game_state)
        (bind _asbp_lmhrace_over_player_state (Utilities|Casting|CastToBP_LMHRaceOverPlayerState _array_element))
        (if (not (Variables|/Game/BP/Mode/Test/Dev/LMH/BP_LMHRaceOverPlayerState.BP_LMHRaceOverPlayerState_C|GetIsDie _asbp_lmhrace_over_player_state))
          (Math|Integer|IncrementInt (Variables|Default|GetSurvivorsCount))))
      (Variables|Default|SetTotalPlayers (Variables|Default|GetSurvivorsCount))
      (Variables|Default|SetSurvivorsCount 0))
    (:then_1
      (bind _aswbp_bill_board (Utilities|Casting|CastToWBP_BillBoard (UserInterface|GetWidget (Variables|Default|GetWidget))))
      (Variables|/Game/BP/Level/Dev/LMH/UI/WBP_BillBoard.WBP_BillBoard_C|SetPlayerCount _aswbp_bill_board (Variables|Default|GetTotalPlayers)))))

(fn ConstructionScript)