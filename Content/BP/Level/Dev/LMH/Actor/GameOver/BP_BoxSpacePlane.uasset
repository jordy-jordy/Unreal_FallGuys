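; BP_BoxSpacePlane is an actor with a plane that, if IsPunch is set, makes one punch-and-retract motion on BeginPlay.
; A timeline sweeps the plane from Back to Forward and sets PhyTime on any BP_LMHCustomCharacter that blocks it; a second returns it without sweeping.
; It also sets player controller 0 as owner; the capsule impulse logic is unconnected.
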(event EventBeginPlay
  (Utilities|FlowControl|Sequence
    (:then_0
      (Actor|SetOwner (Game|GetPlayerController 0)))
    (:then_1
      (if (Variables|Default|GetIsPunch)
        (bind _새_트랙_0 (Timeline|타임라인_0 PlayFromStart)
          (:Update
            (bind _sweephitresult (Transformation|SetWorldLocation (Variables|Default|GetPlane) (Math|Vector|Lerp(Vector) (Transformation|GetWorldLocation (Variables|Default|GetBack)) (Transformation|GetWorldLocation (Variables|Default|GetForward)) _새_트랙_0) true false))
            (if (.bblockinghit _sweephitresult)
              (bind _asbp_lmhcustom_character (Utilities|Casting|CastToBP_LMHCustomCharacter (.hitactor _sweephitresult)))
              (Variables|/Game/BP/Mode/Test/Dev/LMH/BP_LMHCustomCharacter.BP_LMHCustomCharacter_C|SetPhyTime _asbp_lmhcustom_character 5.0)))
          (:Finished
            (bind _새_트랙_0_2 (Timeline|타임라인 PlayFromStart)
              (:Update
                (Transformation|SetWorldLocation (Variables|Default|GetPlane) (Math|Vector|Lerp(Vector) (Transformation|GetWorldLocation (Variables|Default|GetForward)) (Transformation|GetWorldLocation (Variables|Default|GetBack)) _새_트랙_0_2) false false)))))))))

(event Collision|EventActorBeginOverlap
  (params (OtherActor :type Actor%20Object%20Reference)))

(fn ConstructionScript)