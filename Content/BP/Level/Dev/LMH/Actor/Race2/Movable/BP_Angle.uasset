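; BP_Angle is a movable race-level actor that continuously rocks back and forth around its roll axis.
; Each Tick calls AddActorRotation, which flips IsLeft when roll passes roughly 20 degrees either way and applies a constant-speed, delta-time-scaled local rotation.
; On BeginPlay, the authority sets player pawn 0 as owner, while the rotation itself runs without an authority check.
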(event EventBeginPlay
  (Networking|SwitchHasAuthority
    (:Authority
      (Actor|SetOwner (Game|Player|GetPlayerPawn 0)))))

(event Collision|EventActorBeginOverlap
  (params (OtherActor :type Actor%20Object%20Reference)))

(event EventTick
  (params (DeltaSeconds :type Float%20%28single-precision%29))
  (CallFunction|AddActorRotation DeltaSeconds))

(fn ConstructionScript)

(fn AddActorRotation
  (params (detla :type Float%20%28double-precision%29))
  (bind _returnvalue (Transformation|GetActorRotation))
  (bind _returnvalue_2 (* detla 8e+01))
  (Utilities|FlowControl|Sequence
    (:then_0
      (if (> (.roll _returnvalue) 2e+01)
        (Variables|Default|SetIsLeft false)
        (elif (< (.roll _returnvalue) -2e+01)
          (Variables|Default|SetIsLeft true))))
    (:then_1
      (if (Variables|Default|GetIsLeft)
        (Transformation|AddActorLocalRotation (Math|Rotator|MakeRotator _returnvalue_2 0.0 0.0) false false)
        (else
          (Transformation|AddActorLocalRotation (Math|Rotator|MakeRotator (* _returnvalue_2 -1.0) 0.0 0.0) false false))))))