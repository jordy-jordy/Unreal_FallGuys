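; BP_Punch is a Race2 level obstacle that knocks player characters away when its Box component registers a hit.
; The hit's inverted impact normal, scaled by JumpVector, goes to C2S_AddImpulse, named as a client-to-server event.
; That event copies PhyTime to the BP_PlayCharacter and adds the impulse only if its capsule is already simulating physics.
; BeginPlay sets player controller 0 as owner.
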(event OnComponentHit(Box)
  (params (HitComponent :type Primitive%20Component%20Object%20Reference) (OtherActor :type Actor%20Object%20Reference) (OtherComp :type Primitive%20Component%20Object%20Reference) (NormalImpulse :type Vector :default "0, 0, 0") (Hit :type Hit%20Result%20Structure%20%28by%20ref%29))
  (CallFunction|C2SAddImpulse OtherActor (* (* (.impactnormal Hit) -1.0) (Variables|Default|GetJump%20Vector))))

(event Custom|C2S_AddImpulse
  (params (Actor :type Actor%20Object%20Reference) (Impact :type Vector))
  (bind _asbp_play_character (Utilities|Casting|CastToBP_PlayCharacter Actor))
  (Variables|/Game/BP/Mode/01_Play/BP_PlayCharacter.BP_PlayCharacter_C|SetPhyTime _asbp_play_character (Variables|Default|GetPhyTime))
  (if (Physics|IsSimulatingPhysics (Variables|/Script/Engine.Character|GetCapsuleComponent _asbp_play_character) "None")
    (Physics|AddImpulse (Variables|/Script/Engine.Character|GetCapsuleComponent _asbp_play_character) Impact "None" false)))

(event EventBeginPlay
  (Actor|SetOwner (Game|GetPlayerController 0)))

(event Collision|EventActorBeginOverlap
  (params (OtherActor :type Actor%20Object%20Reference)))

(event EventTick
  (params (DeltaSeconds :type Float%20%28single-precision%29)))

(fn ConstructionScript)