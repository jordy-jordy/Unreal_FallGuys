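; BP_Angle is a movable level actor whose AddActorRotation function tilts it in pitch by a fixed step per call.
; The function toggles IsLeft against a single positive pitch threshold to choose direction, so the actor settles around that angle rather than sweeping a symmetric range.
; BeginPlay only calls SetOwner on the player pawn without a new owner; Tick is empty and nothing here calls the rotation function.
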(event EventBeginPlay
  (Actor|SetOwner (Game|Player|GetPlayerPawn 0) 0))

(event Collision|EventActorBeginOverlap
  (params (OtherActor :type Actor%20Object%20Reference)))

(event EventTick
  (params (DeltaSeconds :type Float%20%28single-precision%29)))

(fn ConstructionScript)

(fn AddActorRotation
  (bind _returnvalue (Transformation|GetActorRotation))
  (Utilities|FlowControl|Sequence
    (:then_0
      (if (> (.pitch _returnvalue) 1e+01)
        (Variables|Default|SetIsLeft false)
        (elif (< (.pitch _returnvalue) 1e+01)
          (Variables|Default|SetIsLeft true))))
    (:then_1
      (if (Variables|Default|GetIsLeft)
        (Transformation|AddActorLocalRotation (Math|Rotator|MakeRotator 0.0 1.0 0.0) false false)
        (else
          (Transformation|AddActorLocalRotation (Math|Rotator|MakeRotator 0.0 -1.0 0.0) false false))))))