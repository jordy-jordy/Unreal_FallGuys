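; Title-screen pawn that shows the FallGuy character with a plinth and background, switching between home and customization views.
; Two switch events swap the background material and play timelines that blend camera FOV, camera X/Z position and plinth yaw, lerping from current values.
; BeginPlay sets the home camera and background and snaps upper and lower costume components to the character's CustomSocket.
; The IA_PawnRotate input passes its value to PawnRotation on the plinth.
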(event Custom|SwitchHomeWidgetStart
  (bind _camera (Variables|Default|GetCamera))
  (bind _camerastartpos (Variables|Default|GetCameraStartPos))
  (bind _plinth (Variables|Default|GetPlinth))
  (bind _camera_2 (Variables|Default|GetCamera))
  (bind _relativelocation (Variables|/Script/Engine.SceneComponent|GetRelativeLocation _camera))
  (Rendering|Material|SetMaterial (Variables|Default|GetBG) 0 "/Game/Resources/UI/00_Title/Materials/M_TitleBG_Inst.M_TitleBG_Inst")
  (bind _새_트랙_0 (Timeline|타임라인 PlayFromStart)
    (:Update
      (Camera|SetFieldOfView _camera_2 (Math|Float|Lerp (Variables|/Script/Engine.CameraComponent|GetFieldOfView _camera_2) (Variables|Default|GetHomeFov) _새_트랙_0))
      (Transformation|SetRelativeRotation _plinth (Math|Rotator|MakeRotator 0.0 0.0 (Math|Float|Lerp (.yaw (Variables|/Script/Engine.SceneComponent|GetRelativeRotation _plinth)) 0.0 _새_트랙_0)) false false)
      (Transformation|SetRelativeLocation (Variables|Default|GetCamera) (Math|Vector|MakeVector (Math|Float|Lerp (.x _relativelocation) (.x _camerastartpos) _새_트랙_0) (.y _relativelocation) (Math|Float|Lerp (.z _relativelocation) (.z _camerastartpos) _새_트랙_0)) false false))))

(event Custom|SwitchCustomWidgetStart
  (bind _plinth (Variables|Default|GetPlinth))
  (bind _camera (Variables|Default|GetCamera))
  (bind _camera_2 (Variables|Default|GetCamera))
  (bind _relativelocation (Variables|/Script/Engine.SceneComponent|GetRelativeLocation _camera))
  (Rendering|Material|SetMaterial (Variables|Default|GetBG) 0 "/Game/Resources/UI/Custom/Character/Material/M_BGCharacterRing.M_BGCharacterRing")
  (bind _새_트랙_0 (Timeline|timeLine PlayFromStart)
    (:Update
      (Camera|SetFieldOfView _camera_2 (Math|Float|Lerp (Variables|/Script/Engine.CameraComponent|GetFieldOfView _camera_2) (Variables|Default|GetCustomFOV) _새_트랙_0))
      (Transformation|SetRelativeRotation _plinth (Math|Rotator|MakeRotator 0.0 0.0 (Math|Float|Lerp (.yaw (Variables|/Script/Engine.SceneComponent|GetRelativeRotation _plinth)) (Variables|Default|GetMeshRotationHomeToCustom) _새_트랙_0)) false false)
      (Transformation|SetRelativeLocation (Variables|Default|GetCamera) (Math|Vector|MakeVector (Math|Float|Lerp (.x _relativelocation) (Variables|Default|GetCameraLocHomeToCustom) _새_트랙_0) (.y _relativelocation) (Math|Float|Lerp (.z _relativelocation) (Variables|Default|GetCameraLocHomeToCustomY) _새_트랙_0)) false false))))

(event Input|EnhancedActionEvents|EnhancedInputActionIA_PawnRotate
  (params (ActionValue :type Vector%202D%20Structure) (ElapsedSeconds :type Float%20%28double-precision%29) (TriggeredSeconds :type Float%20%28double-precision%29) (InputAction :type Input%20Action%20Object%20Reference :default "/Game/BP/Mode/00_Title/Input/IA_PawnRotate.IA_PawnRotate"))
  (Class|TitlePawn|PawnRotation (Variables|Default|GetPlinth) ActionValue))

(event EventBeginPlay
  (Transformation|SetRelativeLocationAndRotation (Variables|Default|GetCamera) (Variables|Default|GetCameraStartPos) "0.000000,-90.000000,0.000000" false false)
  (Camera|SetFieldOfView (Variables|Default|GetCamera) (Variables|Default|GetHomeFov))
  (Rendering|Material|SetMaterial (Variables|Default|GetBG) 0 "/Game/Resources/UI/00_Title/Materials/M_TitleBG.M_TitleBG")
  ;[0.15 0.15 0.15 0.5] Static Mesh 부착
  (Transformation|AttachComponentToComponent (Variables|Default|GetUpComp) (Variables|Default|GetFallGuy) "CustomSocket" "SnapToTarget" "SnapToTarget" "SnapToTarget" true)
  (Transformation|AttachComponentToComponent (Variables|Default|GetLowComp) (Variables|Default|GetFallGuy) "CustomSocket" "SnapToTarget" "SnapToTarget" "SnapToTarget" true))

(fn ConstructionScript)