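; BP_PlayCharacter is the player character for play mode, with keyboard movement, repeated jumping and animation state selection.
; Enhanced Input actions call Jump and four per-direction move functions defined outside these graphs, while BeginPlay raises the jump count and hold time.
; Tick selects idle or run from velocity on the ground, and jump start, mid-air or fall from accumulated air time while falling.
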(event Input|EnhancedActionEvents|EnhancedInputActionIA_Jump
  (params (ActionValue :type Vector :default "0, 0, 0") (ElapsedSeconds :type Float%20%28double-precision%29) (TriggeredSeconds :type Float%20%28double-precision%29) (InputAction :type Input%20Action%20Object%20Reference :default "/Game/BP/Mode/01_Play/Input/IA_Jump.IA_Jump"))
  (Character|Jump))

(event Input|EnhancedActionEvents|EnhancedInputActionIA_WMove
  (params (ActionValue :type Vector%202D%20Structure) (ElapsedSeconds :type Float%20%28double-precision%29) (TriggeredSeconds :type Float%20%28double-precision%29) (InputAction :type Input%20Action%20Object%20Reference :default "/Game/BP/Mode/01_Play/Input/IA_WMove.IA_WMove"))
  (Class|PlayCharacter|PlayerWMove))

(event Input|EnhancedActionEvents|EnhancedInputActionIA_AMove
  (params (ActionValue :type Vector%202D%20Structure) (ElapsedSeconds :type Float%20%28double-precision%29) (TriggeredSeconds :type Float%20%28double-precision%29) (InputAction :type Input%20Action%20Object%20Reference :default "/Game/BP/Mode/01_Play/Input/IA_AMove.IA_AMove"))
  (Class|PlayCharacter|PlayerAMove))

(event Input|EnhancedActionEvents|EnhancedInputActionIA_SMove
  (params (ActionValue :type Vector%202D%20Structure) (ElapsedSeconds :type Float%20%28double-precision%29) (TriggeredSeconds :type Float%20%28double-precision%29) (InputAction :type Input%20Action%20Object%20Reference :default "/Game/BP/Mode/01_Play/Input/IA_SMove.IA_SMove"))
  (Class|PlayCharacter|PlayerSMove))

(event Input|EnhancedActionEvents|EnhancedInputActionIA_DMove
  (params (ActionValue :type Vector%202D%20Structure) (ElapsedSeconds :type Float%20%28double-precision%29) (TriggeredSeconds :type Float%20%28double-precision%29) (InputAction :type Input%20Action%20Object%20Reference :default "/Game/BP/Mode/01_Play/Input/IA_DMove.IA_DMove"))
  (Class|PlayCharacter|PlayerDMove))

(event EventBeginPlay
  (Variables|Default|SetJumpMaxCount 10)
  (Variables|Default|SetJumpMaxHoldTime 0.3))

(event Collision|EventActorBeginOverlap
  (params (OtherActor :type Actor%20Object%20Reference)))

(event EventTick
  (params (DeltaSeconds :type Float%20%28single-precision%29))
  (bind _airtime (Variables|Default|GetAirTime))
  (if (AI|Components|NavMovement|IsFalling (Variables|Character|GetCharacterMovement))
    (Class|PlayCharacter|AddAirTime DeltaSeconds)
    (Math|Float|CompareFloat _airtime 0.15
      (:>
        (Math|Float|CompareFloat _airtime 2.0
          (:>
            (Class|PlayCharacter|SetCurAnimnation "Fall"))
          (:<
            (Class|PlayCharacter|SetCurAnimnation "JumpMidAir"))))
      (:<
        (Class|PlayCharacter|SetCurAnimnation "JumpStart")))
    (else
      (Class|PlayCharacter|ResetAirTime)
      (if (Class|KismetMathLibrary|EqualExactlyVectorVector (Transformation|GetVelocity) "0, 0, 0")
        (Class|PlayCharacter|SetCurAnimnation "Idle")
        (else
          (Class|PlayCharacter|SetCurAnimnation "Run"))))))

(fn ConstructionScript)