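; Test play-mode player character with movement, jump-to-dive, egg grab/carry, name-tag toggling and spectating.
; Tick selects animation states from vertical velocity, timers and grab/carry flags, drives timed capsule physics, and enables spectating on FAIL or SUCCESS player status.
; An authority-checked overlap attaches eggs while grabbing; Q/E cycle the view through DEFAULT-status characters.
; Debug keys check death status and teleport to a marker through C2S/S2M events.
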(event OnComponentBeginOverlap(GrabCol)
  (params (OverlappedComponent :type Primitive%20Component%20Object%20Reference) (OtherActor :type Actor%20Object%20Reference) (OtherComp :type Primitive%20Component%20Object%20Reference) (OtherBodyIndex :type Integer) (bFromSweep :type Boolean) (SweepResult :type Hit%20Result%20Structure%20%28by%20ref%29))
  (if (Ability|HasAuthority)
    (if (Variables|Default|GetIsGrab)
      (bind _asbp_egg (Utilities|Casting|CastToBP_Egg OtherActor))
      (Physics|SetSimulatePhysics (Variables|/Game/BP/Level/Dev/LMH/Actor/Egg/BP_Egg.BP_Egg_C|GetStaticMesh _asbp_egg) false)
      (Collision|SetCollisionEnabled (Variables|/Game/BP/Level/Dev/LMH/Actor/Egg/BP_Egg.BP_Egg_C|GetStaticMesh _asbp_egg) "NoCollision")
      (Transformation|AttachComponentToComponent OtherActor (Variables|Default|GetTestScene) "None" "SnapToTarget" "SnapToTarget" "KeepWorld" true)
      (Variables|Default|SetIsCarry true)
      (Variables|Default|SetIsGrab false)
      (Variables|Default|SetCarrying%20Egg _asbp_egg))))

(event Custom|C2S_SetActorLocation
  (params (Loc :type Vector))
  ;[0.15 0.15 0.15 0.5] 개발용 : 결승선 앞에 순간이동
  (CallFunction|S2MSetActorLocation Loc))

(event Custom|GrabOff
  (bind _carrying_egg (Variables|Default|GetCarrying%20Egg))
  (bind _staticmesh (Variables|/Game/BP/Level/Dev/LMH/Actor/Egg/BP_Egg.BP_Egg_C|GetStaticMesh _carrying_egg))
  (Variables|Default|SetIsGrab false)
  (if (Variables|Default|GetIsCarry)
    (Transformation|DetachFromActor _carrying_egg "KeepWorld" "KeepWorld" "KeepWorld")
    (Physics|SetSimulatePhysics _staticmesh true)
    (Collision|SetCollisionEnabled _staticmesh "QueryAndPhysics")
    (Variables|Default|SetIsCarry false)))

(event Custom|GrabOn
  (if (not (Variables|Default|GetIsCarry))
    (Variables|Default|SetIsGrab true)))

(event Custom|S2M_SetActorLocation
  (params (NewParam :type Vector))
  ;[0.15 0.15 0.15 0.5] 개발용 : 결승선 앞에 순간이동
  (Transformation|SetActorLocation NewParam false false))

(event Input|EnhancedActionEvents|EnhancedInputActionIA_Jump
  (params (ActionValue :type Vector :default "0, 0, 0") (ElapsedSeconds :type Float%20%28double-precision%29) (TriggeredSeconds :type Float%20%28double-precision%29) (InputAction :type Input%20Action%20Object%20Reference :default "/Game/BP/Mode/01_Play/Input/IA_Jump.IA_Jump"))
  (:Started
    (if (Math|Float|NearlyEqual(Float) (.Z (Math|Vector|BreakVector (Transformation|GetVelocity))) 0.0 1e+01)
      (Character|Jump)
      (elif (not (Variables|Default|GetIsDive))
        (Class|PlayCharacter|SetCurAnimnation "DiveStart")
        (Class|PlayCharacter|DiveSwitch)
        (Variables|/Script/Engine.CharacterMovementComponent|SetbOrientRotationToMovement (Variables|Character|GetCharacterMovement) false)
        (Transformation|AddActorLocalRotation "-45.000000,0.000000,0.000000" false false)))))

(event Input|EnhancedActionEvents|EnhancedInputActionIA_Grab
  (params (ActionValue :type Boolean) (ElapsedSeconds :type Float%20%28double-precision%29) (TriggeredSeconds :type Float%20%28double-precision%29) (InputAction :type Input%20Action%20Object%20Reference :default "/Game/BP/Mode/01_Play/Input/IA_Grab.IA_Grab"))
  (:Triggered
    (CallFunction|Grabon))
  (:Completed
    (CallFunction|GrabOff)))

(event Input|EnhancedActionEvents|EnhancedInputActionIA_Spectator_E
  (params (ActionValue :type Boolean) (ElapsedSeconds :type Float%20%28double-precision%29) (TriggeredSeconds :type Float%20%28double-precision%29) (InputAction :type Input%20Action%20Object%20Reference :default "/Game/BP/Mode/01_Play/Input/IA_Spectator_E.IA_Spectator_E"))
  (:Started
    (if (Variables|Default|GetIsSpectator)
      (bind _outactors (Actor|GetAllActorsOfClass "/Game/BP/Mode/01_Play/BP_PlayCharacter.BP_PlayCharacter_C"))
      (for _array_element _outactors
        (bind _asplay_player_state (Utilities|Casting|CastToPlayPlayerState (Variables|/Script/Engine.Pawn|GetPlayerState _array_element)))
        (bind _returnvalue (Class|PlayPlayerState|GetPlayerStateStatus _asplay_player_state))
        (switch Utilities|FlowControl|Switch|SwitchonEPlayerStatus _returnvalue
          (:DEFAULT
            (Utilities|Array|Add (Variables|Default|GetAlive%20Players) _array_element))))
      (Variables|Default|SetSpectatorValue (+ (Variables|Default|GetSpectatorValue) 1))
      (if (>= (Variables|Default|GetSpectatorValue) (Utilities|Array|Length (Variables|Default|GetAlive%20Players)))
        (Variables|Default|SetSpectatorValue 0))
      (bind _newparam (CallFunction|SetInteger (Variables|Default|GetSpectatorValue)))
      (bind _output_get (Variables|Default|SetSpectatorValue _newparam))
      (Game|Player|SetViewTargetwithBlend (Game|GetPlayerController 0) (Utilities|Array|Get(acopy) (Variables|Default|GetAlive%20Players) _output_get) 0.0 "VTBlend_Linear" 0.0 false)
      (Utilities|Array|Clear (Variables|Default|GetAlive%20Players)))))

(event Input|EnhancedActionEvents|EnhancedInputActionIA_NameVisible
  (params (ActionValue :type Boolean) (ElapsedSeconds :type Float%20%28double-precision%29) (TriggeredSeconds :type Float%20%28double-precision%29) (InputAction :type Input%20Action%20Object%20Reference :default "/Game/BP/Mode/01_Play/Input/IA_NameVisible.IA_NameVisible"))
  ;[0.15 0.15 0.15 0.5] 닉네임 표시 On / Off
  (:Completed
    (if (Variables|Default|GetIsNameVisible)
      (Utilities|FlowControl|Sequence
        (:then_0
          (Variables|Default|SetIsNameVisible false))
        (:then_1
          (bind _outactors (Actor|GetAllActorsOfClass "/Game/BP/Mode/01_Play/BP_PlayCharacter.BP_PlayCharacter_C"))
          (for _array_element _outactors
            (Rendering|SetActorHiddenInGame (Variables|/Script/Engine.ChildActorComponent|GetChildActor (Variables|/Game/BP/Mode/01_Play/BP_PlayCharacter.BP_PlayCharacter_C|GetPlayerName _array_element)) true))))
      (else
        (Utilities|FlowControl|Sequence
          (:then_0
            (Variables|Default|SetIsNameVisible true))
          (:then_1
            (bind _outactors_2 (Actor|GetAllActorsOfClass "/Game/BP/Mode/01_Play/BP_PlayCharacter.BP_PlayCharacter_C"))
            (for _array_element_2 _outactors_2
              (Rendering|SetActorHiddenInGame (Variables|/Script/Engine.ChildActorComponent|GetChildActor (Variables|/Game/BP/Mode/01_Play/BP_PlayCharacter.BP_PlayCharacter_C|GetPlayerName _array_element_2)) false))))))))

(event Input|EnhancedActionEvents|EnhancedInputActionIA_WMove
  (params (ActionValue :type Vector%202D%20Structure) (ElapsedSeconds :type Float%20%28double-precision%29) (TriggeredSeconds :type Float%20%28double-precision%29) (InputAction :type Input%20Action%20Object%20Reference :default "/Game/BP/Mode/01_Play/Input/IA_WMove.IA_WMove"))
  (Class|PlayCharacter|PlayerWMove))

(event Input|EnhancedActionEvents|EnhancedInputActionIA_AMove
  (params (ActionValue :type Vector%202D%20Structure) (ElapsedSeconds :type Float%20%28double-precision%29) (TriggeredSeconds :type Float%20%28double-precision%29) (InputAction :type Input%20Action%20Object%20Reference :default "/Game/BP/Mode/01_Play/Input/IA_AMove.IA_AMove"))
  (Class|PlayCharacter|PlayerAMove))

(event Input|EnhancedActionEvents|EnhancedInputActionIA_SMove
  (params (ActionValue :type Vector%202D%20Structure) (ElapsedSeconds :type Float%20%28double-precision%29) (TriggeredSeconds :type Float%20%28double-precision%29) (InputAction :type Input%20Action%20Object%20Reference :default "/Game/BP/Mode/01_Play/Input/IA_SMove.IA_SMove"))
  (Class|PlayCharacter|PlayerSMove))

(event Input|EnhancedActionEvents|EnhancedInputActionIA_DMove
  (params (ActionValue :type Vector%202D%20Structure) (ElapsedSeconds :type Float%20%28double-precision%29) (TriggeredSeconds :type Float%20%28double-precision%29) (InputAction :type Input%20Action%20Object%20Reference :default "/Game/BP/Mode/01_Play/Input/IA_DMove.IA_DMove"))
  (Class|PlayCharacter|PlayerDMove))

(event Input|EnhancedActionEvents|EnhancedInputActionIA_Spectator_Q
  (params (ActionValue :type Boolean) (ElapsedSeconds :type Float%20%28double-precision%29) (TriggeredSeconds :type Float%20%28double-precision%29) (InputAction :type Input%20Action%20Object%20Reference :default "/Game/BP/Mode/01_Play/Input/IA_Spectator_Q.IA_Spectator_Q"))
  (:Started
    (if (Variables|Default|GetIsSpectator)
      (bind _outactors (Actor|GetAllActorsOfClass "/Game/BP/Mode/01_Play/BP_PlayCharacter.BP_PlayCharacter_C"))
      (for _array_element _outactors
        (bind _asplay_player_state (Utilities|Casting|CastToPlayPlayerState (Variables|/Script/Engine.Pawn|GetPlayerState _array_element)))
        (bind _returnvalue (Class|PlayPlayerState|GetPlayerStateStatus _asplay_player_state))
        (switch Utilities|FlowControl|Switch|SwitchonEPlayerStatus _returnvalue
          (:DEFAULT
            (Utilities|Array|Add (Variables|Default|GetAlive%20Players) _array_element))))
      (Variables|Default|SetSpectatorValue (- (Variables|Default|GetSpectatorValue) 1))
      (if (< (Variables|Default|GetSpectatorValue) 0)
        (Variables|Default|SetSpectatorValue (- (Utilities|Array|Length (Variables|Default|GetAlive%20Players)) 1)))
      (bind _newparam (CallFunction|SetInteger (Variables|Default|GetSpectatorValue)))
      (bind _output_get (Variables|Default|SetSpectatorValue _newparam))
      (Game|Player|SetViewTargetwithBlend (Game|GetPlayerController 0) (Utilities|Array|Get(acopy) (Variables|Default|GetAlive%20Players) _output_get) 0.0 "VTBlend_Linear" 0.0 false)
      (Utilities|Array|Clear (Variables|Default|GetAlive%20Players)))))

(event EventBeginPlay
  ;[0.15 0.15 0.15 0.5] 비긴 플레이
  (Utilities|FlowControl|Sequence
    (:then_0
      (Variables|Default|SetJumpMaxCount 1)
      (Variables|Default|SetJumpMaxHoldTime 0.3))
    (:then_1
      (bind _asbp_player_name (Utilities|Casting|CastToBP_PlayerName (Variables|/Script/Engine.ChildActorComponent|GetChildActor (Variables|Default|GetPlayerName))))
      (Variables|/Game/BP/Mode/01_Play/BP_PlayerName.BP_PlayerName_C|SetPlayerCharacter _asbp_player_name self))))

(event EventTick
  (params (DeltaSeconds :type Float%20%28single-precision%29))
  (bind _returnvalue (Transformation|GetVelocity))
  (bind _getuptime (Variables|Default|GetGetUpTime))
  (bind _airtime (Variables|Default|GetAirTime))
  (bind _z (Math|Vector|BreakVector _returnvalue))
  (bind _returnvalue_2 (Math|Float|NearlyEqual(Float) _z 0.0 1e+01))
  (Utilities|FlowControl|Sequence
    (:then_0
      (if (Variables|Default|GetIsDive)
        (if _returnvalue_2
          (Class|PlayCharacter|AddGetUpTime DeltaSeconds)
          (Math|Float|CompareFloat _getuptime 0.17
            (:>
              (Math|Float|CompareFloat _getuptime 0.34
                (:>
                  (Class|PlayCharacter|DiveSwitch)
                  (Transformation|AddActorLocalRotation "45.000000,0.000000,0.000000" false false)
                  (Variables|/Script/Engine.CharacterMovementComponent|SetbOrientRotationToMovement (Variables|Character|GetCharacterMovement) true)
                  (Class|PlayCharacter|ResetDiveTime)
                  (Class|PlayCharacter|ResetGetUpTime 0.0))
                (:<
                  (Class|PlayCharacter|SetCurAnimnation "DiveGetUp"))))
            (:<
              (Class|PlayCharacter|SetCurAnimnation "DiveLand")))
          (else
            (Class|PlayCharacter|AddDiveTime DeltaSeconds)
            (Transformation|AddActorWorldOffset (* (Math|Vector|GetForwardVector (Variables|/Script/Engine.MovementComponent|GetUpdatedPrimitive (Variables|Character|GetCharacterMovement))) "2.000000,2.000000,0.000000"))
            (Math|Float|CompareFloat (Variables|Default|GetDiveTime) 0.5
              (:>
                (Class|PlayCharacter|SetCurAnimnation "DiveLoop")))))
        (elif _returnvalue_2
          (Class|PlayCharacter|ResetAirTime)
          (if (Class|KismetMathLibrary|EqualExactlyVectorVector (Transformation|GetVelocity) "0, 0, 0")
            (if (Variables|Default|GetIsGrab)
              (Class|PlayCharacter|SetCurAnimnation "GrabIdle")
              (elif (Variables|Default|GetIsCarry)
                (Class|PlayCharacter|SetCurAnimnation "CarryIdle")
                (else
                  (Class|PlayCharacter|SetCurAnimnation "Idle"))))
            (elif (Variables|Default|GetIsGrab)
              (Class|PlayCharacter|SetCurAnimnation "GrabRun")
              (elif (Variables|Default|GetIsCarry)
                (Class|PlayCharacter|SetCurAnimnation "CarryRun")
                (else
                  (Class|PlayCharacter|SetCurAnimnation "Run")))))
          (else
            (Class|PlayCharacter|AddAirTime DeltaSeconds)
            (Math|Float|CompareFloat _airtime 0.15
              (:>
                (Math|Float|CompareFloat _airtime 2.0
                  (:>
                    (Class|PlayCharacter|SetCurAnimnation "Fall"))
                  (:<
                    (Class|PlayCharacter|SetCurAnimnation "JumpMidAir"))))
              (:<
                (Class|PlayCharacter|SetCurAnimnation "JumpStart")))))))
    (:then_1
      (CallFunction|PhyTimeCheck DeltaSeconds))
    (:then_2
      (bind _asplay_player_state (Utilities|Casting|CastToPlayPlayerState (Variables|Default|GetPlayerState)))
      (bind _returnvalue_3 (Class|PlayPlayerState|GetPlayerStateStatus _asplay_player_state))
      (switch Utilities|FlowControl|Switch|SwitchonEPlayerStatus _returnvalue_3
        (:NONE
          (Variables|Default|SetIsSpectator false :!label _label))
        (:DEFAULT
          (goto _label))
        (:FAIL
          (Variables|Default|SetIsSpectator true :!label _label_2))
        (:SUCCESS
          (goto _label_2))))))

(event Input|KeyboardEvents|Slash
  (params (Key :type Key%20Structure :default "None"))
  ;[0.15 0.15 0.15 0.5] 개발용 : 캐릭터 죽었는지 확인
  (:Pressed
    (Class|PlayCharacter|DebugCheckDieStatus self)))

(event Input|KeyboardEvents|1
  (params (Key :type Key%20Structure :default "None"))
  ;[0.15 0.15 0.15 0.5] 개발용 : 결승선 앞에 순간이동
  (:Pressed
    (bind _outactors (Actor|GetAllActorsOfClass "/Game/BP/Level/Dev/LMH/DebugMode/BP_DebugPos1.BP_DebugPos1_C"))
    (CallFunction|C2SSetActorLocation (Transformation|GetActorLocation (Utilities|Array|Get(acopy) _outactors)))))

(fn ConstructionScript)

(fn PhyTimeCheck
  (params (Delta%20Time :type Float%20%28double-precision%29))
  (if (< (Variables|Default|GetPhyTime) 0.0)
    (Physics|SetSimulatePhysics (Variables|Default|GetCapsuleComponent) false)
    (else
      (Variables|Default|SetPhyTime (- (Variables|Default|GetPhyTime) Delta%20Time))
      (Physics|SetSimulatePhysics (Variables|Default|GetCapsuleComponent) true))))

(fn SetInteger
  (params (NewParam1 :type Integer))
  (return NewParam1))

(fn SpectatorModeFunction
  (bind _outactors (Actor|GetAllActorsOfClass "/Game/BP/Mode/01_Play/BP_PlayCharacter.BP_PlayCharacter_C"))
  (if (== (+ (Variables|Default|GetSpectatorValue) 1) (Utilities|Array|Length _outactors))
    (bind _newparam (CallFunction|SetInteger))
    (bind _output_get (Variables|Default|SetSpectatorValue _newparam))
    (bind _outactors_2 (Actor|GetAllActorsOfClass "/Game/BP/Mode/01_Play/BP_PlayCharacter.BP_PlayCharacter_C"))
    (Game|Player|SetViewTargetwithBlend (Game|GetPlayerController 0) (Utilities|Array|Get(acopy) _outactors_2 _output_get) 0.0 "VTBlend_Linear" 0.0 false)
    (else
      (bind _newparam_2 (CallFunction|SetInteger (+ (Variables|Default|GetSpectatorValue) 1)))
      (bind _output_get_2 (Variables|Default|SetSpectatorValue _newparam_2))
      (bind _outactors_3 (Actor|GetAllActorsOfClass "/Game/BP/Mode/01_Play/BP_PlayCharacter.BP_PlayCharacter_C"))
      (Game|Player|SetViewTargetwithBlend (Game|GetPlayerController 0) (Utilities|Array|Get(acopy) _outactors_3 _output_get_2) 0.0 "VTBlend_Linear" 0.0 false))))