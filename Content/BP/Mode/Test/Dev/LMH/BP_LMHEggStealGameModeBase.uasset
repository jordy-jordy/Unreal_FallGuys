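; BP_LMHEggStealGameModeBase is a developer test game mode for an egg-steal mode with Red and Blue team scores.
; Every Tick it casts the GameState to BP_EggPlayGameState and loops over its team egg counts.
; Index 0 feeds CountREDTeamScore and index 1 feeds CountBLUETeamScore, neither of which is defined in this graph.
; A failed cast prints the first player pawn's display name.
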(event EventTick
  (params (DeltaSeconds :type Float%20%28single-precision%29))
  (bind _asbp_egg_play_game_state (Utilities|Casting|CastToBP_EggPlayGameState (Game|GetGameState))
    (:then
      (for (_array_element _array_index) (Class|TeamPlayGameState|GetTeamEggCount _asbp_egg_play_game_state)
        (if (== _array_index 0)
          ;[0.15 0.15 0.15 0.5] Red Blue Team Egg 계산하기
          (Class|TeamPlayGameMode|CountREDTeamScore _array_element)
          (elif (== _array_index 1)
            (Class|TeamPlayGameMode|CountBLUETeamScore _array_element)))))
    (:CastFailed
      (Development|PrintString (Utilities|GetDisplayName (Game|Player|GetPlayerPawn 0))))))

(fn ConstructionScript)