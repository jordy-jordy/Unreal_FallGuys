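; Test game mode, named for travel testing, that holds spawning until two players have arrived.
; HandleStartingNewPlayer collects each BP_PlayPlayerController in an array, printing a debug string until the count is reached.
; It then loops the array, restarting players at the PlayerStart found by their index as name.
; The array is cleared inside the loop body, so only the first controller gets restarted.
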(event EventBeginPlay
  (Variables|Default|SetNumPlayer 2))

(event EventTick
  (params (DeltaSeconds :type Float%20%28single-precision%29)))

(event EventHandleStartingNewPlayer
  (params (NewPlayer :type Player%20Controller%20Object%20Reference))
  (bind _asbp_play_player_controller (Utilities|Casting|CastToBP_PlayPlayerController NewPlayer))
  (Utilities|Array|Add (Variables|Default|GetAs%20BP%20Play%20Player%20Controller) _asbp_play_player_controller)
  (if (== (Utilities|Array|Length (Variables|Default|GetAs%20BP%20Play%20Player%20Controller)) (Variables|Default|GetNumPlayer))
    (for (_array_element _array_index) (Variables|Default|GetAs%20BP%20Play%20Player%20Controller)
      (Class|GameModeBase|RestartPlayeratPlayerStart _array_element (Class|GameModeBase|FindPlayerStart _array_element (Utilities|String|ToString(Integer) _array_index)))
      (Utilities|Array|Clear (Variables|Default|GetAs%20BP%20Play%20Player%20Controller)))
    (else
      (Development|PrintString "Hello"))))

(fn ConstructionScript)