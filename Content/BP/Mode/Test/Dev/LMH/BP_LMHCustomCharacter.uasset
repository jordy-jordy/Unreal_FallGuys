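; BP_LMHCustomCharacter is a test character that assembles a baseball outfit from separate upper and lower static meshes.
; On BeginPlay, it assigns the baseball meshes to the UP and LW components and snaps each to RootSocket on the character Mesh.
; Each successful attachment prints a debug message, while Tick, overlap and the construction script are empty.
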(event EventBeginPlay
  (Utilities|FlowControl|Sequence
    (:then_0
      (Components|StaticMesh|SetStaticMesh (Variables|Default|GetUP) "/Game/Resources/Character/Dev/LMH/CH_Baseball_UP_LOD0.CH_Baseball_UP_LOD0")
      (bind _returnvalue (Transformation|AttachComponentToComponent (Variables|Default|GetUP) (Variables|Character|GetMesh) "RootSocket" "SnapToTarget" "SnapToTarget" "SnapToTarget" true))
      (if _returnvalue
        (Development|PrintString "Up Attached!!")))
    (:then_1
      (Components|StaticMesh|SetStaticMesh (Variables|Default|GetLW) "/Game/Resources/Character/Dev/LMH/CH_Baseball_LW_LOD0.CH_Baseball_LW_LOD0")
      (bind _returnvalue_2 (Transformation|AttachComponentToComponent (Variables|Default|GetLW) (Variables|Character|GetMesh) "RootSocket" "SnapToTarget" "SnapToTarget" "SnapToTarget" true))
      (if _returnvalue_2
        (Development|PrintString "Low Attached!!")))))

(event Collision|EventActorBeginOverlap
  (params (OtherActor :type Actor%20Object%20Reference)))

(event EventTick
  (params (DeltaSeconds :type Float%20%28single-precision%29)))

(fn ConstructionScript)