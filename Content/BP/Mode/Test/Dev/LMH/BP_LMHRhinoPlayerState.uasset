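; Test player state that can enlarge the player character.
; The S2M_SizeUp event casts player character 0 to BP_PlayCharacter, then multiplies its relative scale and spring arm length by five so the camera distance grows with it.
; An authority-gated call to the event is left unconnected and never runs, and BeginPlay and Tick are empty.
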(event Custom|S2M_SizeUp
  (bind _asbp_play_character (Utilities|Casting|CastToBP_PlayCharacter (Game|GetPlayerCharacter 0)))
  (Transformation|SetActorRelativeScale3D _asbp_play_character (* (Class|Actor|GetActorRelativeScale3D _asbp_play_character) 5.0))
  (Variables|/Script/Engine.SpringArmComponent|SetTargetArmLength (Variables|/Script/Unreal_FallGuys.PlayCharacter|GetSpringArmComponent _asbp_play_character) (* (Variables|/Script/Engine.SpringArmComponent|GetTargetArmLength (Variables|/Script/Unreal_FallGuys.PlayCharacter|GetSpringArmComponent _asbp_play_character)) 5.0)))

(event EventBeginPlay)

(event EventTick
  (params (DeltaSeconds :type Float%20%28single-precision%29)))

(fn ConstructionScript)