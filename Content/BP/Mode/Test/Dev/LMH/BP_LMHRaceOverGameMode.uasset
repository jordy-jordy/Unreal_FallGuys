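; Game mode for the race-over level, which stages players and signals when to move to the result level.
; BeginPlay moves player pawns onto PlayerStarts, then after a short delay sends characters flagged CanHiddenAtResult far below the map, hidden and without collision.
; Tick polls every player state's IsPlayEnd and, once all are done, waits before setting the game state's move-to-result flag.
; A spectator-flag branch for failed local players is disconnected.
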(event Custom|S2M_OutFailPlayer
  (params (Actor :type Actor%20Object%20Reference))
  (Transformation|SetActorLocation Actor "0.000000,0.000000,-1000000.000000" false false)
  (Rendering|SetActorHiddenInGame Actor true)
  (Collision|SetActorEnableCollision Actor false))

(event EventBeginPlay
  (bind _returnvalue (Game|GetGameState))
  (bind _playeridx (Variables|Default|GetplayerIdx))
  (bind _playerarray (Variables|/Script/Engine.GameStateBase|GetPlayerArray _returnvalue))
  (bind _output (Utilities|Array|Get(acopy) _playerarray _playeridx))
  (bind _returnvalue_2 (PlayerState|GetPawn _output))
  (Utilities|FlowControl|Sequence
    (:then_0
      (bind _outactors (Actor|GetAllActorsOfClass "/Script/Engine.PlayerStart"))
      (for _array_element _outactors
        (Utilities|IsValid _array_element
          (:Is%20Valid
            (Utilities|IsValid _output
              (:Is%20Valid
                (Utilities|IsValid _returnvalue_2
                  (:Is%20Valid
                    (Transformation|SetActorLocation _returnvalue_2 (Transformation|GetActorLocation _array_element) false false)
                    (Math|Integer|IncrementInt (Variables|Default|GetplayerIdx))))))))))
    (:then_1
      (Utilities|FlowControl|Delay 0.5)
      (bind _outactors_2 (Actor|GetAllActorsOfClass "/Game/BP/Level/Dev/LMH/Anim/BP_RaceOverCharacter.BP_RaceOverCharacter_C"))
      (for _array_element_2 _outactors_2
        (bind _asbp_lmhrace_over_player_state (Utilities|Casting|CastToBP_LMHRaceOverPlayerState (Variables|/Script/Engine.Pawn|GetPlayerState _array_element_2)))
        (bind _returnvalue_3 (Class|PlayPlayerState|GetCanHiddenatResult _asbp_lmhrace_over_player_state))
        (if _returnvalue_3
          (CallFunction|S2MOutFailPlayer _array_element_2))))))

(event EventTick
  (params (DeltaSeconds :type Float%20%28single-precision%29))
  (if (not (Variables|Default|GetIsLevelEnd))
    (Utilities|FlowControl|Sequence
      (:then_0
        (bind _asbp_play_game_state (Utilities|Casting|CastToBP_PlayGameState (Game|GetGameState)))
        (for _array_element (Variables|/Script/Engine.GameStateBase|GetPlayerArray _asbp_play_game_state)
          (bind _asbp_lmhrace_over_player_state (Utilities|Casting|CastToBP_LMHRaceOverPlayerState _array_element))
          (if (not (Variables|/Game/BP/Mode/Test/Dev/LMH/BP_LMHRaceOverPlayerState.BP_LMHRaceOverPlayerState_C|GetIsPlayEnd _asbp_lmhrace_over_player_state))
            (Variables|Default|SetIsPlayEnd false)))
        (if (Variables|Default|GetIsPlayEnd)
          ;[0.15 0.15 0.15 0.5] Level 이 끝남을 알림
          (Utilities|FlowControl|Delay 5.0)
          (bind _asbp_play_game_state_2 (Utilities|Casting|CastToBP_PlayGameState (Game|GetGameState)))
          (Class|PlayGameState|SetCanMoveResultLevelTrue _asbp_play_game_state_2)
          (Variables|Default|SetIsLevelEnd true)
          (else
            (Variables|Default|SetIsPlayEnd true)))))))

(fn ConstructionScript)