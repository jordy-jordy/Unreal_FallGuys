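; Test game mode for a team floor-painting game, scoring Red and Blue by painted floor count.
; BeginPlay caches all BP_LMHPaintFloor actors, and Tick copies per-team counts from GetTeamFloors into BP_TeamPlayGameState's scores.
; CalTeam is meant to tally floors by color, but it only clears TeamFloors and loops with a validity check, as the counting nodes are disconnected.
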(event EventTick
  (params (DeltaSeconds :type Float%20%28single-precision%29))
  ;[0.15 0 0 0.5] 호출시 Team이 가진 Floor갯수 반환
  (bind _returnvalue (Class|TeamPlayGameMode|GetTeamFloors))
  (if (Utilities|Map|IsNotEmpty _returnvalue)
    (bind _keys (Utilities|Map|Keys _returnvalue))
    (for _array_element _keys
      (switch Utilities|FlowControl|Switch|SwitchonETeamType _array_element
        (:RED
          (bind _asbp_team_play_game_state (Utilities|Casting|CastToBP_TeamPlayGameState (Game|GetGameState)))
          ;[0.15 0.15 0.15 0.5] Red, Blue팀 스코어 계산
          (Class|TeamPlayGameState|SetREDTeamScore _asbp_team_play_game_state (.Value (Utilities|Map|Find _returnvalue _array_element))))
        (:BLUE
          (Class|TeamPlayGameState|SetBLUETeamScore _asbp_team_play_game_state (.Value (Utilities|Map|Find _returnvalue _array_element))))))))

(event EventBeginPlay
  (bind _outactors (Actor|GetAllActorsOfClass "/Game/BP/Level/Dev/LMH/Actor/Paint/BP_LMHPaintFloor.BP_LMHPaintFloor_C"))
  (Variables|Team|SetPaintFloors _outactors))

(event EventCalTeam
  ;[0.15 0.15 0.15 0.5] Floor 이 가진 색으로 (Red, Blue) 팀마다 Floor 갯수 셈
  (Utilities|Map|Clear (Variables|Default|GetTeamFloors))
  (for _array_element (Variables|Team|GetPaintFloors)
    (Utilities|IsValid _array_element)))

(fn ConstructionScript)