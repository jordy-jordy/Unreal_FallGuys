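; BP_EggPlayGameState is a developer test GameState for an egg gameplay mode.
; On BeginPlay the server spawns the egg manager.
; On Tick, the server, when player controller 0 is local, reads per-team egg counts from the spawner and loops over them without acting, leaving a debug print unconnected.
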(event EventBeginPlay
  (Networking|SwitchHasAuthority
    (:Authority
      (Class|PlayGameState|SpawnEggManager))))

(event EventTick
  (params (DeltaSeconds :type Float%20%28single-precision%29))
  (Networking|SwitchHasAuthority
    (:Authority
      (if (Pawn|IsLocalPlayerController (Game|GetPlayerController 0))
        (bind _returnvalue (Class|EggSpawnManager|GetTeamEggCount (Variables|Default|GetSpawnner)))
        (for _array_element _returnvalue
          _)))))

(fn ConstructionScript)