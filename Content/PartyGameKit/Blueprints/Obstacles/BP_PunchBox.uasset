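; BP_PunchBox is an obstacle that extends and retracts a punch mesh and knocks third-person party game characters away.
; On BeginPlay the server plays a designer-tuned timeline that drives PunchMesh's relative Z location.
; Separately, a server-only Box overlap launches the character horizontally away from the actor's origin by LaunchPower, with JumpPower as the upward velocity.
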(event OnComponentBeginOverlap(Box)
  (params (OverlappedComponent :type Primitive%20Component%20Object%20Reference) (OtherActor :type Actor%20Object%20Reference) (OtherComp :type Primitive%20Component%20Object%20Reference) (OtherBodyIndex :type Integer) (bFromSweep :type Boolean) (SweepResult :type Hit%20Result%20Structure%20%28by%20ref%29))
  ;[0 0 0] The character is launched towards a target or jumps with added directional force. You can make any adjustments you want to the Launch Power or Jump Power values.
  (Networking|SwitchHasAuthority
    (:Authority
      (bind _asbp_pgkthird_person_character (Utilities|Casting|CastToBP_PGKThirdPersonCharacter OtherActor))
      (Character|LaunchCharacter _asbp_pgkthird_person_character (Math|Vector|MakeVector (.x (* (Math|Vector|GetUnitDirection(Vector) (Transformation|GetActorLocation) (Transformation|GetActorLocation _asbp_pgkthird_person_character)) (Variables|MainSettings|GetLaunch%20Power))) (.y (* (Math|Vector|GetUnitDirection(Vector) (Transformation|GetActorLocation) (Transformation|GetActorLocation _asbp_pgkthird_person_character)) (Variables|MainSettings|GetLaunch%20Power))) (Variables|MainSettings|GetJump%20Power)) false false))))

(event EventBeginPlay
  ;[0 0 0] BP_PunchBox moves the PunchMesh forward and backward based on the attached Punch Box Timeline. To make it function the way you want, you will need to adjust the Timeline accordingly.
  (Networking|SwitchHasAuthority
    (:Authority
      (bind _location (Timeline|Punch%20Box%20Timeline Play)
        (:Update
          (Transformation|SetRelativeLocation (Variables|Default|GetPunchMesh) (Math|Vector|MakeVector 0.0 0.0 _location) false false))))))

(fn ConstructionScript)