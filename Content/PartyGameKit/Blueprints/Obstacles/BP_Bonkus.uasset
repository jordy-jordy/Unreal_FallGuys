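; BP_Bonkus is a party-game obstacle that spins around its X axis and knocks away characters that hit it.
; On the server, a timeline played at Rotation Speed drives the mesh's roll, negated when Reverse is set.
; Server-side hits launch BP_PGKThirdPersonCharacter horizontally away from the actor using Launch Power, with Jump Power as lift.
; The construction script applies six editable colors through dynamic material instances.
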(event OnComponentHit(Bonkus)
  (params (HitComponent :type Primitive%20Component%20Object%20Reference) (OtherActor :type Actor%20Object%20Reference) (OtherComp :type Primitive%20Component%20Object%20Reference) (NormalImpulse :type Vector :default "0, 0, 0") (Hit :type Hit%20Result%20Structure%20%28by%20ref%29))
  ;[0 0 0] The character is launched towards a target or jumps with added directional force. You can make any adjustments you want to the Launch Power or Jump Power values.
  (Networking|SwitchHasAuthority
    (:Authority
      (bind _asbp_pgkthird_person_character (Utilities|Casting|CastToBP_PGKThirdPersonCharacter OtherActor))
      (Character|LaunchCharacter _asbp_pgkthird_person_character (Math|Vector|MakeVector (.x (* (Math|Vector|GetUnitDirection(Vector) (Transformation|GetActorLocation) (Transformation|GetActorLocation _asbp_pgkthird_person_character)) (Variables|MainSettings|GetLaunch%20Power))) (.y (* (Math|Vector|GetUnitDirection(Vector) (Transformation|GetActorLocation) (Transformation|GetActorLocation _asbp_pgkthird_person_character)) (Variables|MainSettings|GetLaunch%20Power))) (Variables|MainSettings|GetJump%20Power)) false false))))

(event EventBeginPlay
  (bind _bonkus (Variables|Default|GetBonkus))
  ;[0 0 0] BP_Bonkus rotates 360 degrees on the X-axis over 1 second using a Timeline. If the reverse option is selected, it will rotate backward. You can adjust its speed using the "Rotation Speed" value or by modifying the settings within the Timeline.
  (Networking|SwitchHasAuthority
    (:Authority
      (Components|Timeline|SetPlayRate (Variables|Default|GetBonkus%20Rotation%20Timeline) (Variables|MainSettings|GetRotation%20Speed))
      (bind _rotation_value (Timeline|Bonkus%20Rotation%20Timeline Play)
        (:Update
          (if (Variables|MainSettings|GetReverse?)
            (Transformation|SetRelativeRotation _bonkus (Math|Rotator|MakeRotator (* _rotation_value -1.0) 0.0 0.0) true false)
            (else
              (Transformation|SetRelativeRotation _bonkus (Math|Rotator|MakeRotator _rotation_value 0.0 0.0) true false))))))))

(fn ConstructionScript
  (bind _returnvalue (Rendering|Material|CreateDynamicMaterialInstance (Variables|Default|GetBonkus) 0 0 "None" :!class /Script/Engine.PrimitiveComponent))
  (Rendering|Material|SetVectorParameterValue _returnvalue "Color" (Variables|Appearance|GetColor) :!class /Script/Engine.MaterialInstanceDynamic)
  (bind _returnvalue_2 (Rendering|Material|CreateDynamicMaterialInstance (Variables|Default|GetBonkus) 1 0 "None" :!class /Script/Engine.PrimitiveComponent))
  (Rendering|Material|SetVectorParameterValue _returnvalue_2 "Color" (Variables|Appearance|GetColor%202) :!class /Script/Engine.MaterialInstanceDynamic)
  (bind _returnvalue_3 (Rendering|Material|CreateDynamicMaterialInstance (Variables|Default|GetBonkus) 2 0 "None" :!class /Script/Engine.PrimitiveComponent))
  (Rendering|Material|SetVectorParameterValue _returnvalue_3 "Color" (Variables|Appearance|GetColor%203) :!class /Script/Engine.MaterialInstanceDynamic)
  (bind _returnvalue_4 (Rendering|Material|CreateDynamicMaterialInstance (Variables|Default|GetBonkus) 3 0 "None" :!class /Script/Engine.PrimitiveComponent))
  (Rendering|Material|SetVectorParameterValue _returnvalue_4 "Color" (Variables|Appearance|GetColor%204) :!class /Script/Engine.MaterialInstanceDynamic)
  (bind _returnvalue_5 (Rendering|Material|CreateDynamicMaterialInstance (Variables|Default|GetBonkus) 4 0 "None" :!class /Script/Engine.PrimitiveComponent))
  (Rendering|Material|SetVectorParameterValue _returnvalue_5 "Color" (Variables|Appearance|GetColor%205) :!class /Script/Engine.MaterialInstanceDynamic)
  (bind _returnvalue_6 (Rendering|Material|CreateDynamicMaterialInstance (Variables|Default|GetBonkus) 5 0 "None" :!class /Script/Engine.PrimitiveComponent))
  (Rendering|Material|SetVectorParameterValue _returnvalue_6 "Color" (Variables|Appearance|GetColor%206) :!class /Script/Engine.MaterialInstanceDynamic))