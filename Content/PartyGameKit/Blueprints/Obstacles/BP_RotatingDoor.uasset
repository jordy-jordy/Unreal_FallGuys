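; BP_RotatingDoor is a party-game obstacle door that spins its static mesh around the Z-axis.
; On BeginPlay, only the network authority plays a Timeline, described as a 360-degree turn over 3 seconds, with play rate scaled by Speed.
; Each Timeline update writes the yaw to the mesh's relative rotation.
; The construction script creates dynamic material instances for three mesh slots, giving each its own configurable color.
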(event EventBeginPlay
  ;[0 0 0] Rotates 360 degrees on the Z-axis over 3 seconds using a Timeline. If you want to adjust its speed, you can modify the Speed value.
  (Networking|SwitchHasAuthority
    (:Authority
      (Components|Timeline|SetPlayRate (Variables|Default|GetRotating%20Door%20Timeline) (Variables|MainSettings|GetSpeed))
      (bind _rotation_value (Timeline|Rotating%20Door%20Timeline Play)
        (:Update
          (Transformation|SetRelativeRotation (Variables|Default|GetStaticMesh) (Math|Rotator|MakeRotator 0.0 0.0 _rotation_value) false false))))))

(fn ConstructionScript
  (bind _returnvalue (Rendering|Material|CreateDynamicMaterialInstance (Variables|Default|GetStaticMesh) 0 0 "None" :!class /Script/Engine.PrimitiveComponent))
  (Rendering|Material|SetVectorParameterValue _returnvalue "Color" (Variables|Appearance|GetColor) :!class /Script/Engine.MaterialInstanceDynamic)
  (bind _returnvalue_2 (Rendering|Material|CreateDynamicMaterialInstance (Variables|Default|GetStaticMesh) 1 0 "None" :!class /Script/Engine.PrimitiveComponent))
  (Rendering|Material|SetVectorParameterValue _returnvalue_2 "Color" (Variables|Appearance|GetColor%202) :!class /Script/Engine.MaterialInstanceDynamic)
  (bind _returnvalue_3 (Rendering|Material|CreateDynamicMaterialInstance (Variables|Default|GetStaticMesh) 2 0 "None" :!class /Script/Engine.PrimitiveComponent))
  (Rendering|Material|SetVectorParameterValue _returnvalue_3 "Color" (Variables|Appearance|GetColor%203) :!class /Script/Engine.MaterialInstanceDynamic))