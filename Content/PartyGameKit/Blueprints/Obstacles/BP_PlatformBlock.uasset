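; BP_PlatformBlock is a Party Game Kit obstacle platform that shrinks and vanishes after a player touches it, then reappears.
; An authority-only box overlap with the player character waits briefly, then a timeline shrinks the cube horizontally, leaving its height unchanged.
; When it finishes, Reset spawns a Niagara poof, hides the cube and disables its collision, then restores scale, visibility and collision after the adjustable AppearDelay.
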(event OnComponentBeginOverlap(Box)
  (params (OverlappedComponent :type Primitive%20Component%20Object%20Reference) (OtherActor :type Actor%20Object%20Reference) (OtherComp :type Primitive%20Component%20Object%20Reference) (OtherBodyIndex :type Integer) (bFromSweep :type Boolean) (SweepResult :type Hit%20Result%20Structure%20%28by%20ref%29))
  ;[0 0 0] BP_PlatformBlock is very similar to BP_Block. After a player makes contact with the block, it shrinks within half a second and then disappears. After a specified time, it reappears in its original position. You can adjust when it reappears by modifying the Appear Delay value.
  (Networking|SwitchHasAuthority
    (:Authority
      (Utilities|Casting|CastToBP_PGKThirdPersonCharacter OtherActor)
      (Utilities|FlowControl|Delay 0.2)
      (bind _newtrack_0 (Timeline|Timeline Play)
        (:Update
          (Transformation|SetWorldScale3D (Variables|Default|GetCube) (Math|Vector|Lerp(Vector) "1.000000,1.000000,1.000000" "0.500000,0.500000,1.000000" _newtrack_0)))
        (:Finished
          (CallFunction|Reset))))))

(event Custom|Reset
  (bind _cube (Variables|Default|GetCube))
  (bind _cube_2 (Variables|Default|GetCube))
  (bind _cube_3 (Variables|Default|GetCube))
  (bind _returnvalue (Transformation|GetWorldTransform _cube))
  ;[0 0 0] BP_PlatformBlock is very similar to BP_Block. After a player makes contact with the block, it shrinks within half a second and then disappears. After a specified time, it reappears in its original position. You can adjust when it reappears by modifying the Appear Delay value.
  (Components|Timeline|SetNewTime (Variables|Default|GetTimeline) 0.0)
  (Niagara|SpawnSystematLocation "/Game/PartyGameKit/VFX/Poof/NS_Poof.NS_Poof" (.location _returnvalue) (.rotation _returnvalue) (.scale _returnvalue))
  (Development|SetHiddeninGame _cube_3 true false)
  (Collision|SetCollisionEnabled _cube_3 "NoCollision")
  (Utilities|FlowControl|Delay (Variables|MainSettings|GetAppear%20Delay))
  (Transformation|SetWorldScale3D (Variables|Default|GetCube) "1.000000,1.000000,1.000000")
  (Development|SetHiddeninGame _cube_2 false false)
  (Collision|SetCollisionEnabled _cube_2 "QueryAndPhysics"))

(fn ConstructionScript)