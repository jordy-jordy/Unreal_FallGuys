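; BP_SwingingAxe is a party game obstacle that swings an axe and launches player characters it hits.
; On the server, a timeline with play rate set by RotationSpeed drives the Sphere component's relative yaw, negated when Reverse is set.
; A hit on the Sphere, also handled only with authority, launches any BP_PGKThirdPersonCharacter using JumpPower converted to a vector, overriding its existing velocity.
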(event OnComponentHit(Sphere)
  (params (HitComponent :type Primitive%20Component%20Object%20Reference) (OtherActor :type Actor%20Object%20Reference) (OtherComp :type Primitive%20Component%20Object%20Reference) (NormalImpulse :type Vector :default "0, 0, 0") (Hit :type Hit%20Result%20Structure%20%28by%20ref%29))
  (Networking|SwitchHasAuthority
    (:Authority
      (bind _asbp_pgkthird_person_character (Utilities|Casting|CastToBP_PGKThirdPersonCharacter OtherActor))
      (Character|LaunchCharacter _asbp_pgkthird_person_character (Math|Conversions|ToVector(Float) (Variables|Default|GetJump%20Power)) true true))))

(event EventBeginPlay
  (bind _sphere (Variables|Default|GetSphere))
  (Networking|SwitchHasAuthority
    (:Authority
      (Components|Timeline|SetPlayRate (Variables|Default|GetSwinging%20Axe%20Timeline) (Variables|Default|GetRotation%20Speed))
      (bind _rotation_value (Timeline|Swinging%20Axe%20Timeline Play)
        (:Update
          (if (Variables|Default|GetReverse?)
            (Transformation|SetRelativeRotation _sphere (Math|Rotator|MakeRotator 0.0 0.0 (* _rotation_value -1.0)) false false)
            (else
              (Transformation|SetRelativeRotation _sphere (Math|Rotator|MakeRotator 0.0 0.0 _rotation_value) false false))))))))

(fn ConstructionScript)