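; BP_BounceStick is a party game obstacle that slides back and forth and knocks players away on contact.
; On the authority, a looping Timeline moves the stick along its relative X axis, with configurable speed and start delay.
; Hits launch BP_PGKThirdPersonCharacter horizontally away from the actor's origin using LaunchPower, with JumpPower setting upward velocity.
; The construction script tints two material slots through dynamic material instances.
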(event OnComponentHit(BounceStick)
  (params (HitComponent :type Primitive%20Component%20Object%20Reference) (OtherActor :type Actor%20Object%20Reference) (OtherComp :type Primitive%20Component%20Object%20Reference) (NormalImpulse :type Vector :default "0, 0, 0") (Hit :type Hit%20Result%20Structure%20%28by%20ref%29))
  ;[0 0 0] The character is launched towards a target or jumps with added directional force. You can make any adjustments you want to the Launch Power or Jump Power values.
  (Networking|SwitchHasAuthority
    (:Authority
      (bind _asbp_pgkthird_person_character (Utilities|Casting|CastToBP_PGKThirdPersonCharacter OtherActor))
      (Character|LaunchCharacter _asbp_pgkthird_person_character (Math|Vector|MakeVector (.x (* (Math|Vector|GetUnitDirection(Vector) (Transformation|GetActorLocation) (Transformation|GetActorLocation _asbp_pgkthird_person_character)) (Variables|MainSettings|GetLaunch%20Power))) (.y (* (Math|Vector|GetUnitDirection(Vector) (Transformation|GetActorLocation) (Transformation|GetActorLocation _asbp_pgkthird_person_character)) (Variables|MainSettings|GetLaunch%20Power))) (Variables|MainSettings|GetJump%20Power)) false false))))

(event EventBeginPlay
  ;[0 0 0] BP_BounceStick moves back and forth along the X-axis to predetermined points in a loop using a Timeline. To move it along a different axis or to different distances, adjustments are needed. To change its speed, you can modify the Speed value or make changes within the Timeline.
  (Networking|SwitchHasAuthority
    (:Authority
      (Components|Timeline|SetPlayRate (Variables|Default|GetBounce%20Stick%20Location%20Timeline) (Variables|MainSettings|GetSpeed))
      (Utilities|FlowControl|Delay (Variables|MainSettings|GetStarting%20Delay))
      (bind _newtrack_0 (Timeline|Bounce%20Stick%20Location%20Timeline Play)
        (:Update
          (Transformation|SetRelativeLocation (Variables|Default|GetBounceStick) (Math|Vector|MakeVector _newtrack_0 0.0 0.0) false false))))))

(fn ConstructionScript
  (bind _returnvalue (Rendering|Material|CreateDynamicMaterialInstance (Variables|Default|GetBounceStick) 0 0 "None" :!class /Script/Engine.PrimitiveComponent))
  (Rendering|Material|SetVectorParameterValue _returnvalue "Color" (Variables|Appearance|GetColor) :!class /Script/Engine.MaterialInstanceDynamic)
  (bind _returnvalue_2 (Rendering|Material|CreateDynamicMaterialInstance (Variables|Default|GetBounceStick) 1 0 "None" :!class /Script/Engine.PrimitiveComponent))
  (Rendering|Material|SetVectorParameterValue _returnvalue_2 "Color" (Variables|Appearance|GetColor%202) :!class /Script/Engine.MaterialInstanceDynamic))