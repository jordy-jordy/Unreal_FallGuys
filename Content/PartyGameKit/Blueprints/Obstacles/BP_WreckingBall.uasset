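; BP_WreckingBall is a party-game obstacle that rotates a sphere component on its pitch axis as a wrecking ball.
; On BeginPlay, only the authority plays the WreckingBallSpeed timeline, with its play rate set from Speed.
; Each timeline update sets the sphere's relative pitch from the rotation track, negated when Opposite is set to reverse the direction.
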(event EventBeginPlay
  (bind _sphere (Variables|Default|GetSphere))
  (Networking|SwitchHasAuthority
    (:Authority
      (Components|Timeline|SetPlayRate (Variables|Default|GetWreckingBall%20Speed) (Variables|Default|GetSpeed))
      (bind _rotation_value (Timeline|WreckingBall%20Speed Play)
        (:Update
          (if (Variables|Default|GetOpposite?)
            (Transformation|SetRelativeRotation _sphere (Math|Rotator|MakeRotator 0.0 (* _rotation_value -1.0) 0.0) false false)
            (else
              (Transformation|SetRelativeRotation _sphere (Math|Rotator|MakeRotator 0.0 _rotation_value 0.0) false false))))))))

(fn ConstructionScript)