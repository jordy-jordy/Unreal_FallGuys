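; BP_SpinningStick is a party game obstacle that spins its static mesh around the Z axis.
; On BeginPlay, only the authority plays a Timeline at a rate set by Speed, applying its 360-degree curve as relative yaw on each update.
; The Reverse flag negates the yaw to flip the spin direction.
; The construction script creates dynamic material instances for five mesh slots, each tinted by its own color variable.
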(event EventBeginPlay
  (bind _staticmesh (Variables|Default|GetStaticMesh))
  ;[0 0 0] It rotates 360 degrees on the Z-axis over 1 second using a Timeline. If you want to adjust its speed, you can modify the Speed value or edit the Timeline.
  (Networking|SwitchHasAuthority
    (:Authority
      (Components|Timeline|SetPlayRate (Variables|Default|GetSpinning%20Stick%20Rotation) (Variables|MainSettings|GetSpeed))
      (bind _rotation_value (Timeline|Spinning%20Stick%20Rotation Play)
        (:Update
          (if (not (Variables|MainSettings|GetReverse?))
            (Transformation|SetRelativeRotation _staticmesh (Math|Rotator|MakeRotator 0.0 0.0 _rotation_value) true false)
            (else
              (Transformation|SetRelativeRotation _staticmesh (Math|Rotator|MakeRotator 0.0 0.0 (* _rotation_value -1.0)) true false))))))))

(fn ConstructionScript
  (bind _returnvalue (Rendering|Material|CreateDynamicMaterialInstance (Variables|Default|GetStaticMesh) 0 0 "None" :!class /Script/Engine.PrimitiveComponent))
  (Rendering|Material|SetVectorParameterValue _returnvalue "Color" (Variables|Appearance|GetColor) :!class /Script/Engine.MaterialInstanceDynamic)
  (bind _returnvalue_2 (Rendering|Material|CreateDynamicMaterialInstance (Variables|Default|GetStaticMesh) 1 0 "None" :!class /Script/Engine.PrimitiveComponent))
  (Rendering|Material|SetVectorParameterValue _returnvalue_2 "Color" (Variables|Appearance|GetColor%202) :!class /Script/Engine.MaterialInstanceDynamic)
  (bind _returnvalue_3 (Rendering|Material|CreateDynamicMaterialInstance (Variables|Default|GetStaticMesh) 2 0 "None" :!class /Script/Engine.PrimitiveComponent))
  (Rendering|Material|SetVectorParameterValue _returnvalue_3 "Color" (Variables|Appearance|GetColor%203) :!class /Script/Engine.MaterialInstanceDynamic)
  (bind _returnvalue_4 (Rendering|Material|CreateDynamicMaterialInstance (Variables|Default|GetStaticMesh) 3 0 "None" :!class /Script/Engine.PrimitiveComponent))
  (Rendering|Material|SetVectorParameterValue _returnvalue_4 "Color" (Variables|Appearance|GetColor%204) :!class /Script/Engine.MaterialInstanceDynamic)
  (bind _returnvalue_5 (Rendering|Material|CreateDynamicMaterialInstance (Variables|Default|GetStaticMesh) 4 0 "None" :!class /Script/Engine.PrimitiveComponent))
  (Rendering|Material|SetVectorParameterValue _returnvalue_5 "Color" (Variables|Appearance|GetColor%205) :!class /Script/Engine.MaterialInstanceDynamic))