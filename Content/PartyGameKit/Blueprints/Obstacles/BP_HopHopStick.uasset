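; Party-game spinning stick obstacle that knocks characters away and eliminates them once it spins fast enough.
; On the server, a timeline drives mesh yaw while an endless delayed loop raises its play rate at lengthening intervals.
; Hits launch the character outward by JumpPower; above a speed threshold they also ragdoll, then become a spectator as the character is destroyed.
; The construction script tints four material slots from color variables.
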(event OnComponentHit(StaticMesh)
  (params (HitComponent :type Primitive%20Component%20Object%20Reference) (OtherActor :type Actor%20Object%20Reference) (OtherComp :type Primitive%20Component%20Object%20Reference) (NormalImpulse :type Vector :default "0, 0, 0") (Hit :type Hit%20Result%20Structure%20%28by%20ref%29))
  (Networking|SwitchHasAuthority
    (:Authority
      (bind _asbp_pgkthird_person_character (Utilities|Casting|CastToBP_PGKThirdPersonCharacter OtherActor))
      (Character|LaunchCharacter _asbp_pgkthird_person_character (* (Math|Vector|GetUnitDirection(Vector) (Transformation|GetActorLocation) (Transformation|GetActorLocation _asbp_pgkthird_person_character)) (Variables|MainSettings|GetJump%20Power)) false false)
      (if (>= (Variables|MainSettings|GetSpeed) 0.3)
        (Default|SVRRagdoll _asbp_pgkthird_person_character)
        (Utilities|FlowControl|Delay 2.0)
        (bind _returnvalue (Game|SpawnActorfromClass "/Script/Engine.SpectatorPawn" (Math|Transform|MakeTransform "0, 0, 0" "0, 0, 0" "1.000000,1.000000,1.000000") "Undefined" "MultiplyWithRoot" 0 0))
        (Pawn|Possess (Pawn|GetController _asbp_pgkthird_person_character) _returnvalue)
        (Actor|DestroyActor _asbp_pgkthird_person_character)))))

(event Custom|Start
  (Networking|SwitchHasAuthority
    (:Authority
      (Components|Timeline|SetPlayRate (Variables|Default|GetSpinning%20Stick%20Rotation) (Variables|MainSettings|GetSpeed))
      (Utilities|FlowControl|Sequence
        (:then_0
          (bind _rotation_value (Timeline|Spinning%20Stick%20Rotation Play)
            (:Update
              (Transformation|SetRelativeRotation (Variables|Default|GetStaticMesh) (Math|Rotator|MakeRotator 0.0 0.0 _rotation_value) true false))))
        (:then_1
          (bind _output_get (Variables|MainSettings|SetSpeed (* (Variables|MainSettings|GetSpeed) 1.5) :!label _label))
          (Components|Timeline|SetPlayRate (Variables|Default|GetSpinning%20Stick%20Rotation) _output_get)
          (Utilities|FlowControl|RetriggerableDelay (Variables|MainSettings|GetDelay))
          (Variables|MainSettings|SetDelay (+ (Variables|MainSettings|GetDelay) 5.0))
          (Variables|MainSettings|SetKnockback%20Settings (* (Variables|MainSettings|GetKnockback%20Settings) 2.0))
          (goto _label))))))

(fn ConstructionScript
  (bind _returnvalue (Rendering|Material|CreateDynamicMaterialInstance (Variables|Default|GetStaticMesh) 0 0 "None" :!class /Script/Engine.PrimitiveComponent))
  (Rendering|Material|SetVectorParameterValue _returnvalue "Color" (Variables|Appearance|GetColor) :!class /Script/Engine.MaterialInstanceDynamic)
  (bind _returnvalue_2 (Rendering|Material|CreateDynamicMaterialInstance (Variables|Default|GetStaticMesh) 1 0 "None" :!class /Script/Engine.PrimitiveComponent))
  (Rendering|Material|SetVectorParameterValue _returnvalue_2 "Color" (Variables|Appearance|GetColor%202) :!class /Script/Engine.MaterialInstanceDynamic)
  (bind _returnvalue_3 (Rendering|Material|CreateDynamicMaterialInstance (Variables|Default|GetStaticMesh) 2 0 "None" :!class /Script/Engine.PrimitiveComponent))
  (Rendering|Material|SetVectorParameterValue _returnvalue_3 "Color" (Variables|Appearance|GetColor%203) :!class /Script/Engine.MaterialInstanceDynamic)
  (bind _returnvalue_4 (Rendering|Material|CreateDynamicMaterialInstance (Variables|Default|GetStaticMesh) 3 0 "None" :!class /Script/Engine.PrimitiveComponent))
  (Rendering|Material|SetVectorParameterValue _returnvalue_4 "Color" (Variables|Appearance|GetColor%204) :!class /Script/Engine.MaterialInstanceDynamic))