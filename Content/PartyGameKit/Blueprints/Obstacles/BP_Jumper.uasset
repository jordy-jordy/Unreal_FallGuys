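; BP_Jumper is an obstacle actor that bounces player characters up and away when they collide with it.
; On a static mesh hit, only the authority calls LaunchCharacter on a BP_PGKThirdPersonCharacter.
; Horizontal velocity follows the direction from the jumper to the character scaled by LaunchPower, while JumpPower sets the vertical velocity.
; The construction script tints the mesh through a dynamic material instance using the Color variable.
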(event OnComponentHit(StaticMesh)
  (params (HitComponent :type Primitive%20Component%20Object%20Reference) (OtherActor :type Actor%20Object%20Reference) (OtherComp :type Primitive%20Component%20Object%20Reference) (NormalImpulse :type Vector :default "0, 0, 0") (Hit :type Hit%20Result%20Structure%20%28by%20ref%29))
  ;[0 0 0] The character is launched towards a target or jumps with added directional force. You can make any adjustments you want to the Launch Power or Jump Power values.
  (Networking|SwitchHasAuthority
    (:Authority
      (bind _asbp_pgkthird_person_character (Utilities|Casting|CastToBP_PGKThirdPersonCharacter OtherActor))
      (Character|LaunchCharacter _asbp_pgkthird_person_character (Math|Vector|MakeVector (.x (* (Math|Vector|GetUnitDirection(Vector) (Transformation|GetActorLocation) (Transformation|GetActorLocation _asbp_pgkthird_person_character)) (Variables|Default|GetLaunch%20Power))) (.y (* (Math|Vector|GetUnitDirection(Vector) (Transformation|GetActorLocation) (Transformation|GetActorLocation _asbp_pgkthird_person_character)) (Variables|Default|GetLaunch%20Power))) (Variables|Default|GetJump%20Power)) false false))))

(event EventBeginPlay)

(fn ConstructionScript
  (bind _returnvalue (Rendering|Material|CreateDynamicMaterialInstance (Variables|Default|GetStaticMesh) 0 0 "None" :!class /Script/Engine.PrimitiveComponent))
  (Rendering|Material|SetVectorParameterValue _returnvalue "Color" (Variables|Appearance|GetColor) :!class /Script/Engine.MaterialInstanceDynamic))