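; Spectator pawn for the party game (going by its name) that triggers the spectator UI and carries debug shortcuts for session and map control.
; The Spectator event casts the given controller to BP_PC_PartyGame and calls SpectatorWidget.
; NextMap advances the game instance's MapIndex and server-travels to that MapList entry, with no bounds check.
; Test-only numpad keys destroy the session and open the menu, or call NextMap.
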(event Custom|Spectator
  (params (PC :type Controller%20Object%20Reference))
  (bind _asbp_pc_party_game (Utilities|Casting|CastToBP_PC_PartyGame PC))
  (Default|SpectatorWidget _asbp_pc_party_game))

(event Custom|NextMap
  (bind _asgi_party_game (Utilities|Casting|CastToGI_PartyGame (Game|GetGameInstance)))
  (bind _result (Math|Integer|IncrementInt (Variables|/Game/PartyGameKit/Blueprints/GI_PartyGame.GI_PartyGame_C|GetMapIndex _asgi_party_game))
    (:%20%20
      (bind _output_get (Variables|/Game/PartyGameKit/Blueprints/GI_PartyGame.GI_PartyGame_C|SetMapIndex _asgi_party_game _result))
      (Development|ExecuteConsoleCommand (Utilities|String|Append "servertravel /game/PartyGameKit/Maps/" (Utilities|Array|Get(acopy) (Variables|/Game/PartyGameKit/Blueprints/GI_PartyGame.GI_PartyGame_C|GetMapList _asgi_party_game) _output_get)) (Game|GetPlayerController 0)))))

(event Input|KeyboardEvents|DebugKeyNumPadEight
  (params (Key :type Key%20Structure) (ActionValue :type Input%20Action%20Value%20Structure))
  ;[0 1 0.1575] For Testing - You can delete this.
  (:Pressed
    (CallFunction|NextMap)))

(event Input|KeyboardEvents|DebugKeyNumPadSeven
  (params (Key :type Key%20Structure) (ActionValue :type Input%20Action%20Value%20Structure))
  ;[0 1 0.1575] For Testing - You can delete this.
  (:Pressed
    (|DestroySession (Game|GetPlayerController 0)
      (:then
        _)
      (:OnSuccess
        _)
      (:OnFailure
        _))
    (Game|OpenLevel(byObjectReference) "/Game/PartyGameKit/Maps/Menu.Menu")))

(fn ConstructionScript)