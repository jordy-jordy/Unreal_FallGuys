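; Physics football actor, apparently for the party game lobby, that players knock around, swapping its material on NightFootball levels.
; Player hits record the last hitter's name and apply an impulse along the impact normal, or straight up if the player is dashing.
; Kick sounds and a timed Niagara smoke effect, triggered by the authority at high speed, are relayed through server-to-multicast event pairs.
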(event OnComponentHit(Ball)
  (params (HitComponent :type Primitive%20Component%20Object%20Reference) (OtherActor :type Actor%20Object%20Reference) (OtherComp :type Primitive%20Component%20Object%20Reference) (NormalImpulse :type Vector :default "0, 0, 0") (Hit :type Hit%20Result%20Structure%20%28by%20ref%29))
  (bind _asbp_third_person_character (Utilities|Casting|CastTo OtherActor))
  (bind _output_get (Variables|Default|SetLast%20Hit (Variables|Default|GetPlayerName _asbp_third_person_character)))
  (Development|PrintString _output_get)
  (if (not (Variables|Default|GetisDashing? _asbp_third_person_character))
    (Physics|AddImpulse (Variables|Default|GetBall) (* (.ImpactNormal (Collision|BreakHitResult Hit)) 1e+03) "None" true)
    (CallFunction|SRBallSFX)
    (else
      (Physics|AddImpulse (Variables|Default|GetBall) "0.000000,0.000000,500.000000" "None" true)
      (CallFunction|SRBallSFX))))

(event Custom|RPC_Smoke
  (bind _niagara (Variables|Default|GetNiagara))
  (Components|Activation|SetActive _niagara true false)
  (Utilities|FlowControl|Delay 3.0)
  (Components|Activation|SetActive _niagara false false))

(event Custom|SVR_Smoke
  (CallFunction|RPCSmoke))

(event Custom|MC_BallSFX
  (Audio|PlaySoundatLocation 0 (Transformation|GetActorLocation) "0, 0, 0" 1.0 1.0 0.0 0 0 0 0))

(event Custom|SR_BallSFX
  (CallFunction|MCBallSFX))

(event EventTick
  (params (DeltaSeconds :type Float%20%28single-precision%29))
  (Networking|SwitchHasAuthority
    (:Authority
      (if (>= (Math|Vector|VectorLength (Transformation|GetVelocity)) 2e+03)
        (CallFunction|SVRSmoke)))))

(event EventBeginPlay
  (bind _returnvalue (Game|GetCurrentLevelName true))
  (if (Utilities|String|Contains _returnvalue "NightFootball")
    (Rendering|Material|SetMaterial (Variables|Default|GetBall) 0 0)))

(fn ConstructionScript)