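; BP_Projectile is a party game projectile that knocks player characters away when they touch it.
; On Sphere1 overlap, the server launches an overlapped BP_PGKThirdPersonCharacter horizontally away from the projectile, scaled by LaunchPower, with JumpPower as vertical velocity, then destroys the projectile.
; The hit event does nothing, and a separate server-side destroy branch is never run.
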(event OnComponentBeginOverlap(Sphere1)
  (params (OverlappedComponent :type Primitive%20Component%20Object%20Reference) (OtherActor :type Actor%20Object%20Reference) (OtherComp :type Primitive%20Component%20Object%20Reference) (OtherBodyIndex :type Integer) (bFromSweep :type Boolean) (SweepResult :type Hit%20Result%20Structure%20%28by%20ref%29))
  (Networking|SwitchHasAuthority
    (:Authority
      (bind _asbp_pgkthird_person_character (Utilities|Casting|CastToBP_PGKThirdPersonCharacter OtherActor))
      (Character|LaunchCharacter _asbp_pgkthird_person_character (Math|Vector|MakeVector (.x (* (Math|Vector|GetUnitDirection(Vector) (Transformation|GetActorLocation) (Transformation|GetActorLocation _asbp_pgkthird_person_character)) (Variables|Default|GetLaunch%20Power))) (.y (* (Math|Vector|GetUnitDirection(Vector) (Transformation|GetActorLocation) (Transformation|GetActorLocation _asbp_pgkthird_person_character)) (Variables|Default|GetLaunch%20Power))) (Variables|Default|GetJump%20Power)) false false)
      (Actor|DestroyActor))))

(event OnComponentHit(Sphere1)
  (params (HitComponent :type Primitive%20Component%20Object%20Reference) (OtherActor :type Actor%20Object%20Reference) (OtherComp :type Primitive%20Component%20Object%20Reference) (NormalImpulse :type Vector :default "0, 0, 0") (Hit :type Hit%20Result%20Structure%20%28by%20ref%29)))

(fn ConstructionScript)