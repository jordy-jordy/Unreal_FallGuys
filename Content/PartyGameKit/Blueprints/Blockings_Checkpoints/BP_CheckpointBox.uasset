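; Respawn trigger box that teleports an overlapping BP_PGKThirdPersonCharacter back to its saved checkpoint.
; On overlap, it passes the character's CheckpointName to TeleportCheckpoint, which scans every BP_Checkpoint for a substring match.
; A match sends the character to one of that checkpoint's three arrows at random, with zeroed rotation.
; An empty checkpoint name sends it to a random PlayerStart instead.
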(event OnComponentBeginOverlap(Box)
  (params (OverlappedComponent :type Primitive%20Component%20Object%20Reference) (OtherActor :type Actor%20Object%20Reference) (OtherComp :type Primitive%20Component%20Object%20Reference) (OtherBodyIndex :type Integer) (bFromSweep :type Boolean) (SweepResult :type Hit%20Result%20Structure%20%28by%20ref%29))
  ;[0 0 0] It triggers the TeleportCheckpoint event on the overlapping character.
  (bind _asbp_pgkthird_person_character (Utilities|Casting|CastToBP_PGKThirdPersonCharacter OtherActor))
  (CallFunction|TeleportCheckpoint _asbp_pgkthird_person_character (Variables|/Game/PartyGameKit/Blueprints/Characters/BP_PGKThirdPersonCharacter.BP_PGKThirdPersonCharacter_C|GetCheckpointName _asbp_pgkthird_person_character)))

(event Custom|TeleportCheckpoint
  (params (Character :type BP%20PGK%20Third%20Person%20Character%20Object%20Reference) (Checkpoint :type String))
  ;[0 0 0] It checks all checkpoints on the map, matches the character’s saved checkpoint, and teleports the character to it.
  (bind _outactors (Actor|GetAllActorsOfClass "/Game/PartyGameKit/Blueprints/Blockings_Checkpoints/BP_Checkpoint.BP_Checkpoint_C"))
  (for _array_element _outactors
    (if (Utilities|String|Contains Checkpoint (Variables|/Game/PartyGameKit/Blueprints/Blockings_Checkpoints/BP_Checkpoint.BP_Checkpoint_C|GetCheckpoint%20Name _array_element))
      (Transformation|Teleport Character (Transformation|GetWorldLocation (.OutItem (Utilities|Array|Random (Utilities|Array|MakeArray (Variables|/Game/PartyGameKit/Blueprints/Blockings_Checkpoints/BP_Checkpoint.BP_Checkpoint_C|GetArrow _array_element) (Variables|/Game/PartyGameKit/Blueprints/Blockings_Checkpoints/BP_Checkpoint.BP_Checkpoint_C|GetArrow1 _array_element) (Variables|/Game/PartyGameKit/Blueprints/Blockings_Checkpoints/BP_Checkpoint.BP_Checkpoint_C|GetArrow2 _array_element))))) "0, 0, 0")))
  ;[0 0 0] If the checkpoint registered to the character cannot be found, the player teleports to the start.
  (if (== (Utilities|String|Len Checkpoint) 0)
    (bind _outactors_2 (Actor|GetAllActorsOfClass "/Script/Engine.PlayerStart"))
    (Transformation|Teleport Character (Transformation|GetWorldLocation (Variables|/Script/Engine.Actor|GetRootComponent (.OutItem (Utilities|Array|Random _outactors_2)))) "0, 0, 0")))

(fn ConstructionScript)