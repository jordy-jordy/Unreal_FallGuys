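; Game mode for the Paint Floor party minigame, running a timed Red versus Blue match from waiting phase to map change.
; After a countdown it alternates characters between teams; players joining after the start become spectators.
; When time expires it locks floor tiles and compares team totals parsed from each controller's counter widget text.
; It awards points to the winning team, then server-travels to the next map in the game instance's list.
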(event Custom|UpdateScore
  (for _array_element (Variables|Default|GetAll%20Players)
    (Default|UpdateScore (.AsBP%20PC%20Party%20Game (Utilities|Casting|CastToBP_PC_PartyGame _array_element)))))

(event Custom|Timer
  (bind _outactors (Actor|GetAllActorsOfClass "/Game/PartyGameKit/Blueprints/BP_PC_PartyGame.BP_PC_PartyGame_C"))
  (for _array_element _outactors
    (Default|Timer _array_element (Variables|Default|GetFinish%20Game%20Delay))))

(event Custom|RemoveWaitingWidget
  (bind _outactors (Actor|GetAllActorsOfClass "/Game/PartyGameKit/Blueprints/BP_PC_PartyGame.BP_PC_PartyGame_C"))
  (for _array_element _outactors
    (Default|RemoveWaiting _array_element)))

(event Custom|Winner
  (bind _outactors (Actor|GetAllActorsOfClass "/Game/PartyGameKit/Blueprints/BP_PC_PartyGame.BP_PC_PartyGame_C"))
  (for _array_element _outactors
    (bind _pf_countervar (Variables|/Game/PartyGameKit/Blueprints/BP_PC_PartyGame.BP_PC_PartyGame_C|GetPF_CounterVar _array_element)
      (:then
        (Variables|/Game/PartyGameKit/UI/InGame/WBP_PaintFloorScore.WBP_PaintFloorScore_C|SetisGameFinished? _pf_countervar true)
        (Variables|Default|SetRedFinalScore (Math|Conversions|ToFloat(Integer) (Utilities|String|ToString(Text) (Variables|/Script/UMG.TextBlock|GetText (Variables|/Game/PartyGameKit/UI/InGame/WBP_PaintFloorScore.WBP_PaintFloorScore_C|GetRed _pf_countervar)))))
        (Variables|Default|SetBlueFinalScore (Math|Conversions|ToFloat(Integer) (Utilities|String|ToString(Text) (Variables|/Script/UMG.TextBlock|GetText (Variables|/Game/PartyGameKit/UI/InGame/WBP_PaintFloorScore.WBP_PaintFloorScore_C|GetBlue _pf_countervar)))))
        (CallFunction|RemoveWaitingWidget)
        (if (> (Variables|Default|GetRedFinalScore) (Variables|Default|GetBlueFinalScore))
          (CallFunction|RedWinUI)
          (CallFunction|SetScore "Red")
          (Utilities|FlowControl|Delay 5.0 :!label _label)
          (CallFunction|NextMap)
          (elif (> (Variables|Default|GetBlueFinalScore) (Variables|Default|GetRedFinalScore))
            (CallFunction|BlueWinUI)
            (CallFunction|SetScore "Blue")
            (goto _label)
            (elif (== (Variables|Default|GetRedFinalScore) (Variables|Default|GetBlueFinalScore))
              (goto _label)))))
      (:else))))

(event Custom|SetTeam
  (bind _outactors (Actor|GetAllActorsOfClass "/Game/PartyGameKit/Blueprints/Characters/BP_PGKThirdPersonCharacter.BP_PGKThirdPersonCharacter_C"))
  (for (_array_element _array_index) _outactors
    (if (== (Math|Integer|%(Integer) _array_index 2) 0)
      (Variables|/Game/PartyGameKit/Blueprints/Characters/BP_PGKThirdPersonCharacter.BP_PGKThirdPersonCharacter_C|SetTeam _array_element "Red")
      (else
        (Variables|/Game/PartyGameKit/Blueprints/Characters/BP_PGKThirdPersonCharacter.BP_PGKThirdPersonCharacter_C|SetTeam _array_element "Blue")))))

(event Custom|Spectator
  (params (PC :type Player%20Controller%20Object%20Reference))
  (bind _asbp_pc_party_game (Utilities|Casting|CastToBP_PC_PartyGame PC))
  (Default|Spectator _asbp_pc_party_game))

(event Custom|NextMap
  (bind _asgi_party_game (Utilities|Casting|CastToGI_PartyGame (Game|GetGameInstance)))
  (bind _result (Math|Integer|IncrementInt (Variables|/Game/PartyGameKit/Blueprints/GI_PartyGame.GI_PartyGame_C|GetMapIndex _asgi_party_game))
    (:%20%20
      (bind _output_get (Variables|/Game/PartyGameKit/Blueprints/GI_PartyGame.GI_PartyGame_C|SetMapIndex _asgi_party_game _result))
      (Development|ExecuteConsoleCommand (Utilities|String|Append "servertravel /game/PartyGameKit/Maps/" (Utilities|Array|Get(acopy) (Variables|/Game/PartyGameKit/Blueprints/GI_PartyGame.GI_PartyGame_C|GetMapList _asgi_party_game) _output_get)) (Game|GetPlayerController 0)))))

(event Custom|FinishGame
  (Utilities|FlowControl|Delay (Variables|Default|GetFinish%20Game%20Delay))
  (CallFunction|CanChangeDisable)
  (CallFunction|TimeOver)
  (Utilities|FlowControl|Delay 4.0)
  (CallFunction|Winner))

(event Custom|BlueWinUI
  (bind _outactors (Actor|GetAllActorsOfClass "/Game/PartyGameKit/Blueprints/BP_PC_PartyGame.BP_PC_PartyGame_C"))
  (for _array_element _outactors
    (Default|BlueTeamWins _array_element)))

(event Custom|RedWinUI
  (bind _outactors (Actor|GetAllActorsOfClass "/Game/PartyGameKit/Blueprints/BP_PC_PartyGame.BP_PC_PartyGame_C"))
  (for _array_element _outactors
    (Default|RedTeamWins _array_element)))

(event Custom|FloorSettings
  (bind _outactors (Actor|GetAllActorsOfClass "/Game/PartyGameKit/Blueprints/Gamemode_Content/BP_Floor.BP_Floor_C"))
  (for _array_element _outactors
    (Default|DynamicMaterial _array_element)))

(event Custom|WaitingWidget
  (params (Controller :type Controller%20Object%20Reference))
  (bind _asbp_pc_party_game (Utilities|Casting|CastToBP_PC_PartyGame Controller))
  (Default|WaitingforPlayers _asbp_pc_party_game))

(event Custom|TimeOver
  (bind _outactors (Actor|GetAllActorsOfClass "/Game/PartyGameKit/Blueprints/BP_PC_PartyGame.BP_PC_PartyGame_C"))
  (for _array_element _outactors
    (Default|TimeOver _array_element)))

(event Custom|SetScore
  (params (Team :type String))
  (bind _outactors (Actor|GetAllActorsOfClass "/Game/PartyGameKit/Blueprints/Characters/BP_PGKThirdPersonCharacter.BP_PGKThirdPersonCharacter_C"))
  (for _array_element _outactors
    (if (Utilities|String|Contains (Variables|/Game/PartyGameKit/Blueprints/Characters/BP_PGKThirdPersonCharacter.BP_PGKThirdPersonCharacter_C|GetTeam _array_element) Team)
      (Default|SetScore _array_element (+ (Variables|/Game/PartyGameKit/Blueprints/Characters/BP_PGKThirdPersonCharacter.BP_PGKThirdPersonCharacter_C|GetCurrentScore _array_element) (Variables|Default|GetPF_Score)))))
  (CallFunction|UpdateScore))

(event Custom|CanChangeDisable
  (bind _outactors (Actor|GetAllActorsOfClass "/Game/PartyGameKit/Blueprints/Gamemode_Content/BP_Floor.BP_Floor_C"))
  (for _array_element _outactors
    (Variables|/Game/PartyGameKit/Blueprints/Gamemode_Content/BP_Floor.BP_Floor_C|SetCanChange? _array_element false)))

(event EventOnSwapPlayerControllers
  (params (OldPC :type Player%20Controller%20Object%20Reference) (NewPC :type Player%20Controller%20Object%20Reference))
  ;[0 0 0] Player Connect - Disconnect
  (Utilities|Array|Add (Variables|Default|GetAll%20Players) NewPC))

(event EventPostLogin
  (params (NewPlayer :type Player%20Controller%20Object%20Reference))
  ;[0 0 0] Player Connect - Disconnect
  (Utilities|Array|Add (Variables|Default|GetAll%20Players) NewPlayer)
  (if (Variables|Default|GetisGameStarted?)
    (CallFunction|Spectator NewPlayer)
    (else
      (CallFunction|WaitingWidget NewPlayer)))
  (CallFunction|UpdateScore))

(event EventBeginPlay
  (Utilities|FlowControl|Delay (Variables|Default|GetWaiting%20For%20Players))
  (Variables|Default|SetisGameStarted? true)
  (CallFunction|RemoveWaitingWidget)
  (CallFunction|FloorSettings)
  (bind _outactors (Actor|GetAllActorsOfClass "/Game/PartyGameKit/Blueprints/BP_PC_PartyGame.BP_PC_PartyGame_C"))
  (for _array_element _outactors
    (Default|Countdown _array_element)
    (Default|PFFloorCounter _array_element))
  (Utilities|FlowControl|Delay 3.0)
  (CallFunction|SetTeam)
  (CallFunction|Timer)
  (CallFunction|FinishGame))

(event EventOnLogout
  (params (ExitingController :type Controller%20Object%20Reference))
  ;[0 0 0] Player Connect - Disconnect
  (bind _asbp_pc_party_game (Utilities|Casting|CastToBP_PC_PartyGame ExitingController))
  (Utilities|Array|RemoveItem (Variables|Default|GetAll%20Players) _asbp_pc_party_game)
  (CallFunction|UpdateScore))

(fn ConstructionScript)