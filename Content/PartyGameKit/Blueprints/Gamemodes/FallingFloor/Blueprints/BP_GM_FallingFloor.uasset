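; Game mode for the Falling Floor party minigame, where the last remaining character wins.
; After a wait and countdown, it destroys spawn-tagged blocks, lets the rest dissolve and enables movement; players joining mid-game spectate.
; While running, Tick polls the character count to announce a winner or "NO ONE".
; A winner gets points, then the game instance's map list drives server travel to the next map.
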(event Custom|UpdateScore
  (for _array_element (Variables|DoNotEdit|GetAll%20Players)
    (Default|UpdateScore (.AsBP%20PC%20Party%20Game (Utilities|Casting|CastToBP_PC_PartyGame _array_element)))))

(event Custom|SVR_GameEnd
  ;[0 0 0] From the start of the game, it checks if any players remain in the game. When only one player is left, they are selected as the winner. The event also accounts for rare cases where the last players may fall simultaneously. The winning player is awarded a score, and the game proceeds to the next map.
  (bind _outactors (Actor|GetAllActorsOfClass "/Game/PartyGameKit/Blueprints/Characters/BP_PGKThirdPersonCharacter.BP_PGKThirdPersonCharacter_C"))
  (if (== (Utilities|Array|Length _outactors) 1)
    (Variables|DoNotEdit|SetisGameStarted? false)
    (bind _returnvalue (Actor|GetActorOfClass "/Game/PartyGameKit/Blueprints/Characters/BP_PGKThirdPersonCharacter.BP_PGKThirdPersonCharacter_C"))
    (Pawn|Components|CharacterMovement|DisableMovement (Variables|/Script/Engine.Character|GetCharacterMovement _returnvalue))
    (bind _outactors_2 (Actor|GetAllActorsOfClass "/Game/PartyGameKit/Blueprints/BP_PC_PartyGame.BP_PC_PartyGame_C"))
    (for _array_element _outactors_2
      (Default|WinnerText _array_element (Variables|/Game/PartyGameKit/Blueprints/Characters/BP_PGKThirdPersonCharacter.BP_PGKThirdPersonCharacter_C|GetPlayerName _returnvalue)))
    (Utilities|FlowControl|Delay 5.0)
    (CallFunction|SetScore _returnvalue)
    (CallFunction|UpdateScore)
    (CallFunction|NextMap)
    (elif (== (Utilities|Array|Length _outactors) 0)
      (Variables|DoNotEdit|SetisGameStarted? false)
      (bind _outactors_3 (Actor|GetAllActorsOfClass "/Game/PartyGameKit/Blueprints/BP_PC_PartyGame.BP_PC_PartyGame_C"))
      (for _array_element_2 _outactors_3
        (Default|WinnerText _array_element_2 "NO ONE"))
      (Utilities|FlowControl|Delay 5.0)
      (CallFunction|NextMap))))

(event Custom|Spectator
  (params (PC :type Player%20Controller%20Object%20Reference))
  (bind _asbp_pc_party_game (Utilities|Casting|CastToBP_PC_PartyGame PC))
  (Default|Spectator _asbp_pc_party_game))

(event Custom|StartGame
  (bind _outactors (Actor|GetAllActorsOfClasswithTag "/Game/PartyGameKit/Blueprints/Gamemode_Content/BP_Block.BP_Block_C" "Spawns"))
  (for _array_element _outactors
    (Actor|DestroyActor _array_element))
  (bind _outactors_2 (Actor|GetAllActorsOfClass "/Game/PartyGameKit/Blueprints/Gamemode_Content/BP_Block.BP_Block_C"))
  (for _array_element_2 _outactors_2
    (Variables|/Game/PartyGameKit/Blueprints/Gamemode_Content/BP_Block.BP_Block_C|SetCanDissolve _array_element_2 true))
  (Variables|DoNotEdit|SetisGameStarted? true))

(event Custom|DisableMovement
  (bind _outactors (Actor|GetAllActorsOfClass "/Game/PartyGameKit/Blueprints/Characters/BP_PGKThirdPersonCharacter.BP_PGKThirdPersonCharacter_C"))
  (for _array_element _outactors
    (Pawn|Components|CharacterMovement|SetMovementMode (Variables|/Script/Engine.Character|GetCharacterMovement _array_element) "MOVE_None" 0)))

(event Custom|ActivateMovement
  (bind _outactors (Actor|GetAllActorsOfClass "/Game/PartyGameKit/Blueprints/Characters/BP_PGKThirdPersonCharacter.BP_PGKThirdPersonCharacter_C"))
  (for _array_element _outactors
    (Pawn|Components|CharacterMovement|SetMovementMode (Variables|/Script/Engine.Character|GetCharacterMovement _array_element) "MOVE_Walking" 0)))

(event Custom|Countdown
  (bind _outactors (Actor|GetAllActorsOfClass "/Game/PartyGameKit/Blueprints/BP_PC_PartyGame.BP_PC_PartyGame_C"))
  (for _array_element _outactors
    (Default|Countdown _array_element)))

(event Custom|WaitingWidget
  (params (Controller :type Controller%20Object%20Reference))
  (bind _asbp_pc_party_game (Utilities|Casting|CastToBP_PC_PartyGame Controller))
  (Default|WaitingforPlayers _asbp_pc_party_game))

(event Custom|RemoveWaitingWidget
  (bind _outactors (Actor|GetAllActorsOfClass "/Game/PartyGameKit/Blueprints/BP_PC_PartyGame.BP_PC_PartyGame_C"))
  (for _array_element _outactors
    (Default|RemoveWaiting _array_element)))

(event Custom|NextMap
  (bind _asgi_party_game (Utilities|Casting|CastToGI_PartyGame (Game|GetGameInstance)))
  (bind _result (Math|Integer|IncrementInt (Variables|/Game/PartyGameKit/Blueprints/GI_PartyGame.GI_PartyGame_C|GetMapIndex _asgi_party_game))
    (:%20%20
      (bind _output_get (Variables|/Game/PartyGameKit/Blueprints/GI_PartyGame.GI_PartyGame_C|SetMapIndex _asgi_party_game _result))
      (Development|ExecuteConsoleCommand (Utilities|String|Append "servertravel /game/PartyGameKit/Maps/" (Utilities|Array|Get(acopy) (Variables|/Game/PartyGameKit/Blueprints/GI_PartyGame.GI_PartyGame_C|GetMapList _asgi_party_game) _output_get)) (Game|GetPlayerController 0)))))

(event Custom|SetScore
  (params (Target :type BP%20PGK%20Third%20Person%20Character%20Object%20Reference))
  (Default|SetScore Target (+ (Variables|/Game/PartyGameKit/Blueprints/Characters/BP_PGKThirdPersonCharacter.BP_PGKThirdPersonCharacter_C|GetCurrentScore Target) (Variables|MainSettings|GetFF_Score))))

(event EventBeginPlay
  (Utilities|FlowControl|Delay (Variables|MainSettings|GetWaitingForPlayersDelay))
  (CallFunction|RemoveWaitingWidget)
  (CallFunction|Countdown)
  (Utilities|FlowControl|Delay 3.0)
  (CallFunction|StartGame)
  (CallFunction|ActivateMovement))

(event EventOnSwapPlayerControllers
  (params (OldPC :type Player%20Controller%20Object%20Reference) (NewPC :type Player%20Controller%20Object%20Reference))
  ;[0 0 0] Player Connect - Disconnect
  (Utilities|Array|Add (Variables|DoNotEdit|GetAll%20Players) NewPC))

(event EventPostLogin
  (params (NewPlayer :type Player%20Controller%20Object%20Reference))
  ;[0 0 0] Player Connect - Disconnect
  (Utilities|Array|Add (Variables|DoNotEdit|GetAll%20Players) NewPlayer)
  (if (Variables|DoNotEdit|GetisGameStarted?)
    (CallFunction|Spectator NewPlayer)
    (else
      (CallFunction|WaitingWidget NewPlayer)))
  (CallFunction|UpdateScore)
  (CallFunction|DisableMovement))

(event EventTick
  (params (DeltaSeconds :type Float%20%28single-precision%29))
  (if (Variables|DoNotEdit|GetisGameStarted?)
    (CallFunction|SVRGameEnd)))

(event EventOnLogout
  (params (ExitingController :type Controller%20Object%20Reference))
  ;[0 0 0] Player Connect - Disconnect
  (bind _asbp_pc_party_game (Utilities|Casting|CastToBP_PC_PartyGame ExitingController))
  (Utilities|Array|RemoveItem (Variables|DoNotEdit|GetAll%20Players) _asbp_pc_party_game)
  (CallFunction|UpdateScore))

(fn ConstructionScript)