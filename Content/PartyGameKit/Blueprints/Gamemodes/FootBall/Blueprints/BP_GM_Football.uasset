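; Football party-game mode that runs a team match to five goals, then server-travels to the next map in the game instance's list.
; After a waiting delay it alternates characters into Blue and Red teams at tagged TargetPoints and spawns the ball; late joiners spectate.
; Tick polls goal actors (a separate class on NightFootball maps), awarding the opposing team points and win UI.
; A match-time event exists but is never called here.
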(event Custom|UpdateScoreboard
  (for _array_element (Variables|DoNotEdit|GetAll%20Players)
    (Default|UpdateScore (.AsBP%20PC%20Party%20Game (Utilities|Casting|CastToBP_PC_PartyGame _array_element)))))

(event Custom|SVR_SpawnBall
  (bind _outactors (Actor|GetAllActorsOfClasswithTag "/Script/Engine.TargetPoint" "BallSpawn"))
  (Game|SpawnActorfromClass "/Game/PartyGameKit/Blueprints/Gamemode_Content/BP_Ball.BP_Ball_C" (Transformation|GetActorTransform (Utilities|Array|Get(acopy) _outactors)) "Undefined" "MultiplyWithRoot" 0 0))

(event Custom|SetTeams
  (bind _outactors (Actor|GetAllActorsOfClass "/Game/PartyGameKit/Blueprints/Characters/BP_PGKThirdPersonCharacter.BP_PGKThirdPersonCharacter_C"))
  (for (_array_element _array_index) _outactors
    (Variables|/Game/PartyGameKit/Blueprints/Characters/BP_PGKThirdPersonCharacter.BP_PGKThirdPersonCharacter_C|SetGamemodeEnum _array_element "NewEnumerator0")
    (if (== (Math|Integer|%(Integer) _array_index 2) 0)
      (bind _outactors_2 (Actor|GetAllActorsOfClasswithTag "/Script/Engine.TargetPoint" "Blue"))
      (Transformation|Teleport _array_element (Transformation|GetActorLocation (.OutItem (Utilities|Array|Random _outactors_2))) "0, 0, 0")
      (Variables|/Game/PartyGameKit/Blueprints/Characters/BP_PGKThirdPersonCharacter.BP_PGKThirdPersonCharacter_C|SetTeam _array_element "Blue")
      (Default|SetTeamColor _array_element)
      (else
        (bind _outactors_3 (Actor|GetAllActorsOfClasswithTag "/Script/Engine.TargetPoint" "Red"))
        (Transformation|Teleport _array_element (Transformation|GetActorLocation (.OutItem (Utilities|Array|Random _outactors_3))) "0, 0, 0")
        (Variables|/Game/PartyGameKit/Blueprints/Characters/BP_PGKThirdPersonCharacter.BP_PGKThirdPersonCharacter_C|SetTeam _array_element "Red")
        (Default|SetTeamColor _array_element)))))

(event Custom|Spectator
  (params (PC :type Player%20Controller%20Object%20Reference))
  (bind _asbp_pc_party_game (Utilities|Casting|CastToBP_PC_PartyGame PC))
  (Default|Spectator _asbp_pc_party_game))

(event Custom|CheckTimeEnd
  (Utilities|FlowControl|Delay (Variables|MainSettings|GetMatchTime))
  (bind _returnvalue (Actor|GetActorOfClass "/Game/PartyGameKit/Blueprints/Gamemode_Content/BP_Ball.BP_Ball_C"))
  (Actor|DestroyActor _returnvalue))

(event Custom|BlueWinUI
  (bind _outactors (Actor|GetAllActorsOfClass "/Game/PartyGameKit/Blueprints/BP_PC_PartyGame.BP_PC_PartyGame_C"))
  (for _array_element _outactors
    (Default|BlueTeamWins _array_element)))

(event Custom|RedWinUI
  (bind _outactors (Actor|GetAllActorsOfClass "/Game/PartyGameKit/Blueprints/BP_PC_PartyGame.BP_PC_PartyGame_C"))
  (for _array_element _outactors
    (Default|RedTeamWins _array_element)))

(event Custom|NextMap
  (bind _asgi_party_game (Utilities|Casting|CastToGI_PartyGame (Game|GetGameInstance)))
  (bind _result (Math|Integer|IncrementInt (Variables|/Game/PartyGameKit/Blueprints/GI_PartyGame.GI_PartyGame_C|GetMapIndex _asgi_party_game))
    (:%20%20
      (bind _output_get (Variables|/Game/PartyGameKit/Blueprints/GI_PartyGame.GI_PartyGame_C|SetMapIndex _asgi_party_game _result))
      (Development|ExecuteConsoleCommand (Utilities|String|Append "servertravel /game/PartyGameKit/Maps/" (Utilities|Array|Get(acopy) (Variables|/Game/PartyGameKit/Blueprints/GI_PartyGame.GI_PartyGame_C|GetMapList _asgi_party_game) _output_get)) (Game|GetPlayerController 0)))))

(event Custom|WaitingWidget
  (params (Controller :type Controller%20Object%20Reference))
  (bind _asbp_pc_party_game (Utilities|Casting|CastToBP_PC_PartyGame Controller))
  (Default|WaitingforPlayers _asbp_pc_party_game))

(event Custom|RemoveWaitingWidget
  (bind _outactors (Actor|GetAllActorsOfClass "/Game/PartyGameKit/Blueprints/BP_PC_PartyGame.BP_PC_PartyGame_C"))
  (for _array_element _outactors
    (Default|RemoveWaiting _array_element)))

(event Custom|SetScore
  (params (Team :type String))
  (bind _outactors (Actor|GetAllActorsOfClass "/Game/PartyGameKit/Blueprints/Characters/BP_PGKThirdPersonCharacter.BP_PGKThirdPersonCharacter_C"))
  (for _array_element _outactors
    (if (Utilities|String|Contains (Variables|/Game/PartyGameKit/Blueprints/Characters/BP_PGKThirdPersonCharacter.BP_PGKThirdPersonCharacter_C|GetTeam _array_element) Team)
      (Default|SetScore _array_element (+ (Variables|/Game/PartyGameKit/Blueprints/Characters/BP_PGKThirdPersonCharacter.BP_PGKThirdPersonCharacter_C|GetCurrentScore _array_element) (Variables|MainSettings|GetF_Score))))))

(event EventTick
  (params (DeltaSeconds :type Float%20%28single-precision%29))
  (if (Variables|DoNotEdit|GetisGameStarted?)
    (if (not (Variables|DoNotEdit|GetNightMap))
      (bind _outactors (Actor|GetAllActorsOfClass "/Game/PartyGameKit/Blueprints/Gamemode_Content/BP_Goal.BP_Goal_C"))
      (for _array_element _outactors
        (if (== (Variables|/Game/PartyGameKit/Blueprints/Gamemode_Content/BP_Goal.BP_Goal_C|GetScore _array_element) 5.0)
          (if (Utilities|String|Contains (Variables|/Game/PartyGameKit/Blueprints/Gamemode_Content/BP_Goal.BP_Goal_C|GetTeam _array_element) "Red")
            (Utilities|FlowControl|DoOnce false
              (:Completed
                (CallFunction|SetScore "Blue")
                (CallFunction|BlueWinUI)))
            (else
              (Utilities|FlowControl|DoOnce false
                (:Completed
                  (CallFunction|SetScore "Red")
                  (CallFunction|RedWinUI)))))
          (Variables|DoNotEdit|SetisGameStarted? false)
          (CallFunction|UpdateScoreboard)
          (bind _returnvalue (Actor|GetActorOfClass "/Game/PartyGameKit/Blueprints/Gamemode_Content/BP_Ball.BP_Ball_C"))
          (Actor|DestroyActor _returnvalue)
          (Utilities|FlowControl|Delay 5.0)
          (CallFunction|NextMap)))
      (else
        (bind _outactors_2 (Actor|GetAllActorsOfClass "/Game/PartyGameKit/Blueprints/Gamemode_Content/BP_Goal1.BP_Goal1_C"))
        (for _array_element_2 _outactors_2
          (if (== (Variables|/Game/PartyGameKit/Blueprints/Gamemode_Content/BP_Goal1.BP_Goal1_C|GetScore _array_element_2) 5.0)
            (if (Utilities|String|Contains (Variables|/Game/PartyGameKit/Blueprints/Gamemode_Content/BP_Goal1.BP_Goal1_C|GetTeam _array_element_2) "Red")
              (Utilities|FlowControl|DoOnce false
                (:Completed
                  (CallFunction|SetScore "Blue")
                  (CallFunction|BlueWinUI)))
              (else
                (Utilities|FlowControl|DoOnce false
                  (:Completed
                    (CallFunction|SetScore "Red")
                    (CallFunction|RedWinUI)))))
            (Variables|DoNotEdit|SetisGameStarted? false)
            (CallFunction|UpdateScoreboard)
            (bind _returnvalue_2 (Actor|GetActorOfClass "/Game/PartyGameKit/Blueprints/Gamemode_Content/BP_Ball.BP_Ball_C"))
            (Actor|DestroyActor _returnvalue_2)
            (Utilities|FlowControl|Delay 5.0)
            (CallFunction|NextMap)))))))

(event EventOnSwapPlayerControllers
  (params (OldPC :type Player%20Controller%20Object%20Reference) (NewPC :type Player%20Controller%20Object%20Reference))
  ;[0 0 0] Player Connect - Disconnect
  (Utilities|Array|Add (Variables|DoNotEdit|GetAll%20Players) NewPC))

(event EventPostLogin
  (params (NewPlayer :type Player%20Controller%20Object%20Reference))
  ;[0 0 0] Player Connect - Disconnect
  (Utilities|Array|Add (Variables|DoNotEdit|GetAll%20Players) NewPlayer)
  (if (Variables|DoNotEdit|GetisGameStarted?)
    (CallFunction|Spectator NewPlayer)
    (else
      (CallFunction|WaitingWidget NewPlayer)))
  (CallFunction|UpdateScoreboard))

(event EventBeginPlay
  (Utilities|FlowControl|Delay (Variables|MainSettings|GetWaitingForPlayersDelay))
  (CallFunction|RemoveWaitingWidget)
  (bind _outactors (Actor|GetAllActorsOfClass "/Game/PartyGameKit/Blueprints/BP_PC_PartyGame.BP_PC_PartyGame_C"))
  (for _array_element _outactors
    (Default|Countdown _array_element)
    (Default|FFootballScore _array_element))
  (CallFunction|SetTeams)
  (Utilities|FlowControl|Delay 3.0)
  (CallFunction|SVRSpawnBall)
  (Audio|PlaySound2D 0 1.0 1.0 0.0 0 0)
  (Variables|DoNotEdit|SetisGameStarted? true)
  (bind _returnvalue (Game|GetCurrentLevelName true))
  (Variables|DoNotEdit|SetNightMap (Utilities|String|Contains _returnvalue "NightFootball")))

(event EventOnLogout
  (params (ExitingController :type Controller%20Object%20Reference))
  ;[0 0 0] Player Connect - Disconnect
  (bind _asbp_pc_party_game (Utilities|Casting|CastToBP_PC_PartyGame ExitingController))
  (Utilities|Array|RemoveItem (Variables|DoNotEdit|GetAll%20Players) _asbp_pc_party_game)
  (CallFunction|UpdateScoreboard))

(fn ConstructionScript)