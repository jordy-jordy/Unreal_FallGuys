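; Game mode for the Mountain Run party minigame, handling player joins, scoring, round flow and map rotation.
; After a waiting delay it runs a countdown, removes the tagged start wall and fires the cannons; late joiners spectate.
; TriggerTimer starts the finish timer and a Tick check that ends the round early when no characters remain.
; Finishing shows time-over, then server-travels to the next map in GI_PartyGame's list.
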(event Custom|UpdateScore
  (for _array_element (Variables|Default|GetAll%20Players)
    (Default|UpdateScore (.AsBP%20PC%20Party%20Game (Utilities|Casting|CastToBP_PC_PartyGame _array_element)))))

(event Custom|RemoveWall
  (bind _outactors (Actor|GetAllActorsOfClasswithTag "/Script/Engine.TriggerBox" "Remove"))
  (Actor|DestroyActor (Utilities|Array|Get(acopy) _outactors)))

(event Custom|TriggerTimer
  (bind _finish_game_delay (Variables|Default|GetFinish%20Game%20Delay))
  (bind _outactors (Actor|GetAllActorsOfClass "/Game/PartyGameKit/Blueprints/BP_PC_PartyGame.BP_PC_PartyGame_C"))
  (for _array_element _outactors
    (Default|Timer _array_element _finish_game_delay)
    (Variables|Default|SetCheckPlayer true)
    (Utilities|FlowControl|Delay _finish_game_delay)
    (CallFunction|FinishGame)))

(event Custom|NextMap
  (bind _asgi_party_game (Utilities|Casting|CastToGI_PartyGame (Game|GetGameInstance)))
  (bind _result (Math|Integer|IncrementInt (Variables|/Game/PartyGameKit/Blueprints/GI_PartyGame.GI_PartyGame_C|GetMapIndex _asgi_party_game))
    (:%20%20
      (bind _output_get (Variables|/Game/PartyGameKit/Blueprints/GI_PartyGame.GI_PartyGame_C|SetMapIndex _asgi_party_game _result))
      (Development|ExecuteConsoleCommand (Utilities|String|Append "servertravel /game/PartyGameKit/Maps/" (Utilities|Array|Get(acopy) (Variables|/Game/PartyGameKit/Blueprints/GI_PartyGame.GI_PartyGame_C|GetMapList _asgi_party_game) _output_get)) (Game|GetPlayerController 0)))))

(event Custom|CheckPlayers
  (bind _outactors (Actor|GetAllActorsOfClass "/Game/PartyGameKit/Blueprints/Characters/BP_PGKThirdPersonCharacter.BP_PGKThirdPersonCharacter_C"))
  (if (== (Utilities|Array|Length _outactors) 0)
    (Variables|Default|SetCheckPlayer false)
    (CallFunction|FinishGame)))

(event Custom|Spectator
  (params (PC :type Player%20Controller%20Object%20Reference))
  (bind _asbp_pc_party_game (Utilities|Casting|CastToBP_PC_PartyGame PC))
  (Default|Spectator _asbp_pc_party_game))

(event Custom|FinishGame
  (CallFunction|TimeOver)
  (Utilities|FlowControl|Delay 5.0)
  (CallFunction|NextMap))

(event Custom|TimeOver
  (bind _outactors (Actor|GetAllActorsOfClass "/Game/PartyGameKit/Blueprints/BP_PC_PartyGame.BP_PC_PartyGame_C"))
  (for _array_element _outactors
    (Default|TimeOver _array_element)))

(event Custom|Counter
  (bind _outactors (Actor|GetAllActorsOfClass "/Game/PartyGameKit/Blueprints/BP_PC_PartyGame.BP_PC_PartyGame_C"))
  (for _array_element _outactors
    (Default|Countdown _array_element)))

(event Custom|Cannon
  (bind _outactors (Actor|GetAllActorsOfClass "/Game/PartyGameKit/Blueprints/Obstacles/BP_Cannon.BP_Cannon_C"))
  (for _array_element _outactors
    ;[1 1 1] Comment
    (Default|ServerTriggerCannon _array_element)))

(event Custom|WaitingWidget
  (params (Controller :type Controller%20Object%20Reference))
  (bind _asbp_pc_party_game (Utilities|Casting|CastToBP_PC_PartyGame Controller))
  (Default|WaitingforPlayers _asbp_pc_party_game))

(event Custom|RemoveWidget
  (bind _outactors (Actor|GetAllActorsOfClass "/Game/PartyGameKit/Blueprints/BP_PC_PartyGame.BP_PC_PartyGame_C"))
  (for _array_element _outactors
    (Default|RemoveWaiting _array_element)))

(event Custom|SetScore
  (params (Target :type BP%20PGK%20Third%20Person%20Character%20Object%20Reference))
  (Default|SetScore Target (+ (Variables|/Game/PartyGameKit/Blueprints/Characters/BP_PGKThirdPersonCharacter.BP_PGKThirdPersonCharacter_C|GetCurrentScore Target) (Variables|Default|GetMR_Score)))
  (CallFunction|UpdateScore))

(event EventTick
  (params (DeltaSeconds :type Float%20%28single-precision%29))
  (if (Variables|Default|GetCheckPlayer)
    (CallFunction|CheckPlayers)))

(event EventOnSwapPlayerControllers
  (params (OldPC :type Player%20Controller%20Object%20Reference) (NewPC :type Player%20Controller%20Object%20Reference))
  ;[0 0 0] Player Connect - Disconnect
  (Utilities|Array|Add (Variables|Default|GetAll%20Players) NewPC))

(event EventPostLogin
  (params (NewPlayer :type Player%20Controller%20Object%20Reference))
  ;[0 0 0] Player Connect - Disconnect
  (Utilities|Array|Add (Variables|Default|GetAll%20Players) NewPlayer)
  (if (Variables|Default|GetisGameStarted?)
    (CallFunction|Spectator NewPlayer)
    (else
      (CallFunction|WaitingWidget NewPlayer)))
  (CallFunction|UpdateScore))

(event EventBeginPlay
  (Utilities|FlowControl|Delay (Variables|Default|GetWaitingForPlayersDelay))
  (Variables|Default|SetisGameStarted? true)
  (CallFunction|RemoveWidget)
  (CallFunction|Counter)
  (Utilities|FlowControl|Delay 3.0)
  (CallFunction|RemoveWall)
  (CallFunction|Cannon))

(event EventOnLogout
  (params (ExitingController :type Controller%20Object%20Reference))
  ;[0 0 0] Player Connect - Disconnect
  (bind _asbp_pc_party_game (Utilities|Casting|CastToBP_PC_PartyGame ExitingController))
  (Utilities|Array|RemoveItem (Variables|Default|GetAll%20Players) _asbp_pc_party_game)
  (CallFunction|UpdateScore))

(fn ConstructionScript)