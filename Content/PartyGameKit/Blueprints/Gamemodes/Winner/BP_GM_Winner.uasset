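; Party game winner-stage game mode that presents the final top three and can restart the match.
; Tracks joining and leaving controllers, showing waiting or spectator views.
; Ten seconds after BeginPlay it blends players to the winner camera, sorts character scores, teleports score matches to tagged podium points, then shows final lobby and scoreboard.
; StartingGame resets GameInstance map index and scores, then server-travels to the first map.
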(event Custom|UpdateScoreboard
  (for _array_element (Variables|Default|GetAll%20Players)
    (Default|UpdateScore (.AsBP%20PC%20Party%20Game (Utilities|Casting|CastToBP_PC_PartyGame _array_element)))))

(event Custom|GetWidget
  (bind _outactors (Actor|GetAllActorsOfClass "/Game/PartyGameKit/Blueprints/BP_PC_PartyGame.BP_PC_PartyGame_C"))
  (for _array_element _outactors
    (Default|FinalLobby _array_element)))

(event Custom|Starting%20Game
  ;[0 0 0] Start Again
  (Networking|SwitchHasAuthority
    (:Authority
      (bind _asgi_party_game (Utilities|Casting|CastToGI_PartyGame (Game|GetGameInstance)))
      (Variables|/Game/PartyGameKit/Blueprints/GI_PartyGame.GI_PartyGame_C|SetMapIndex _asgi_party_game 0)
      (Utilities|Map|Clear (Variables|/Game/PartyGameKit/Blueprints/GI_PartyGame.GI_PartyGame_C|GetPlayerScores _asgi_party_game))
      (bind _asgi_party_game_2 (Utilities|Casting|CastToGI_PartyGame (Game|GetGameInstance)))
      (Development|ExecuteConsoleCommand (Utilities|String|Append "servertravel /game/PartyGameKit/Maps/" (Utilities|Array|Get(acopy) (Variables|/Game/PartyGameKit/Blueprints/GI_PartyGame.GI_PartyGame_C|GetMapList _asgi_party_game_2) (Variables|/Game/PartyGameKit/Blueprints/GI_PartyGame.GI_PartyGame_C|GetMapIndex _asgi_party_game_2))) (Game|GetPlayerController 0)))))

(event Custom|WinnerCamera
  (bind _outactors (Actor|GetAllActorsOfClasswithTag "/Script/Engine.CameraActor" "WinnerCamera"))
  (bind _outactors_2 (Actor|GetAllActorsOfClass "/Game/PartyGameKit/Blueprints/BP_PC_PartyGame.BP_PC_PartyGame_C"))
  (for _array_element _outactors_2
    (Game|Player|SetViewTargetwithBlend _array_element (Utilities|Array|Get(acopy) _outactors) 3.0 "VTBlend_Linear" 0.0 false)))

(event Custom|Spectator
  (params (PC :type Player%20Controller%20Object%20Reference))
  (bind _asbp_pc_party_game (Utilities|Casting|CastToBP_PC_PartyGame PC))
  (Default|Spectator _asbp_pc_party_game))

(event Custom|MC_Effects
  (Niagara|SpawnSystematLocation "/Game/PartyGameKit/VFX/Confetti/NS_Confetti.NS_Confetti" (Transformation|GetActorLocation (Variables|Default|Get1stWinner))))

(event Custom|Find3rdPlayer
  ;[0 0 0] Determines the top three winners and teleports them according to their ranking.
  (bind _outactors (Actor|GetAllActorsOfClass "/Game/PartyGameKit/Blueprints/Characters/BP_PGKThirdPersonCharacter.BP_PGKThirdPersonCharacter_C"))
  (for _array_element _outactors
    (if (== (Variables|/Game/PartyGameKit/Blueprints/Characters/BP_PGKThirdPersonCharacter.BP_PGKThirdPersonCharacter_C|GetCurrentScore _array_element) (Utilities|Array|Get(acopy) (Variables|Default|GetAllScores) 2))
      (bind _output_get (Variables|Default|Set3stWinner _array_element))
      (bind _outactors_2 (Actor|GetAllActorsOfClasswithTag "/Script/Engine.TargetPoint" "3rd"))
      (Transformation|Teleport _output_get (Transformation|GetActorLocation (Utilities|Array|Get(acopy) _outactors_2)) (Transformation|GetActorRotation (Utilities|Array|Get(acopy) _outactors_2))))))

(event Custom|FindWinnerPlayer
  ;[0 0 0] Determines the top three winners and teleports them according to their ranking.
  (bind _outactors (Actor|GetAllActorsOfClass "/Game/PartyGameKit/Blueprints/Characters/BP_PGKThirdPersonCharacter.BP_PGKThirdPersonCharacter_C"))
  (for _array_element _outactors
    (if (== (Variables|/Game/PartyGameKit/Blueprints/Characters/BP_PGKThirdPersonCharacter.BP_PGKThirdPersonCharacter_C|GetCurrentScore _array_element) (Utilities|Array|Get(acopy) (Variables|Default|GetAllScores)))
      (bind _output_get (Variables|Default|Set1stWinner _array_element))
      (bind _outactors_2 (Actor|GetAllActorsOfClasswithTag "/Script/Engine.TargetPoint" "1st"))
      (Transformation|Teleport _output_get (Transformation|GetActorLocation (Utilities|Array|Get(acopy) _outactors_2)) (Transformation|GetActorRotation (Utilities|Array|Get(acopy) _outactors_2))))))

(event Custom|FinalScoreboard
  (bind _outactors (Actor|GetAllActorsOfClass "/Game/PartyGameKit/Blueprints/BP_PC_PartyGame.BP_PC_PartyGame_C"))
  (for _array_element _outactors
    (Default|UpdateScore _array_element)))

(event Custom|WaitingWidget
  (params (Controller :type Controller%20Object%20Reference))
  (bind _asbp_pc_party_game (Utilities|Casting|CastToBP_PC_PartyGame Controller))
  (Default|WaitingforPlayers _asbp_pc_party_game))

(event Custom|RemoveWaitingWidget
  (bind _outactors (Actor|GetAllActorsOfClass "/Game/PartyGameKit/Blueprints/BP_PC_PartyGame.BP_PC_PartyGame_C"))
  (for _array_element _outactors
    (Default|RemoveWaiting _array_element)))

(event Custom|GetAllScores
  ;[0 0 0] Get all scores and sort them from highest to lowest.
  (bind _outactors (Actor|GetAllActorsOfClass "/Game/PartyGameKit/Blueprints/Characters/BP_PGKThirdPersonCharacter.BP_PGKThirdPersonCharacter_C"))
  (for _array_element _outactors
    (Utilities|Array|Add (Variables|Default|GetAllScores) (Variables|/Game/PartyGameKit/Blueprints/Characters/BP_PGKThirdPersonCharacter.BP_PGKThirdPersonCharacter_C|GetCurrentScore _array_element)))
  (Class|KismetArrayLibrary|SortIntArray (Variables|Default|GetAllScores) false "Descending"))

(event Custom|Find2ndPlayer
  ;[0 0 0] Determines the top three winners and teleports them according to their ranking.
  (bind _outactors (Actor|GetAllActorsOfClass "/Game/PartyGameKit/Blueprints/Characters/BP_PGKThirdPersonCharacter.BP_PGKThirdPersonCharacter_C"))
  (for _array_element _outactors
    (if (== (Variables|/Game/PartyGameKit/Blueprints/Characters/BP_PGKThirdPersonCharacter.BP_PGKThirdPersonCharacter_C|GetCurrentScore _array_element) (Utilities|Array|Get(acopy) (Variables|Default|GetAllScores) 1))
      (bind _output_get (Variables|Default|Set2stWinner _array_element))
      (bind _outactors_2 (Actor|GetAllActorsOfClasswithTag "/Script/Engine.TargetPoint" "2nd"))
      (Transformation|Teleport _output_get (Transformation|GetActorLocation (Utilities|Array|Get(acopy) _outactors_2)) (Transformation|GetActorRotation (Utilities|Array|Get(acopy) _outactors_2))))))

(event EventPostLogin
  (params (NewPlayer :type Player%20Controller%20Object%20Reference))
  ;[0 0 0] Player Connect - Disconnect
  (Utilities|Array|Add (Variables|Default|GetAll%20Players) NewPlayer)
  (if (Variables|Default|GetisGameStarted?)
    (CallFunction|Spectator NewPlayer)
    (else
      (CallFunction|WaitingWidget NewPlayer)))
  (CallFunction|UpdateScoreboard))

(event EventOnSwapPlayerControllers
  (params (OldPC :type Player%20Controller%20Object%20Reference) (NewPC :type Player%20Controller%20Object%20Reference))
  ;[0 0 0] Player Connect - Disconnect
  (Utilities|Array|Add (Variables|Default|GetAll%20Players) NewPC))

(event EventBeginPlay
  (Utilities|FlowControl|Delay 1e+01)
  (CallFunction|RemoveWaitingWidget)
  (CallFunction|WinnerCamera)
  (CallFunction|GetAllScores)
  (CallFunction|FindWinnerPlayer)
  (CallFunction|Find2ndPlayer)
  (CallFunction|Find3rdPlayer)
  (CallFunction|GetWidget)
  (CallFunction|FinalScoreboard))

(event EventOnLogout
  (params (ExitingController :type Controller%20Object%20Reference))
  ;[0 0 0] Player Connect - Disconnect
  (bind _asbp_pc_party_game (Utilities|Casting|CastToBP_PC_PartyGame ExitingController))
  (Utilities|Array|RemoveItem (Variables|Default|GetAll%20Players) _asbp_pc_party_game)
  (CallFunction|UpdateScoreboard))

(fn ConstructionScript)