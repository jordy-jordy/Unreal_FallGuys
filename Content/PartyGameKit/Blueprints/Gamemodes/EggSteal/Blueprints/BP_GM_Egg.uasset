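; Game mode for the Egg Steal party minigame, running one timed team round from waiting period to map travel.
; After a countdown it starts the egg spawner, assigns teams by character index, enables the egg goals and pushes UI through every player controller.
; At time-up it compares goal scores, awards points to winning team members, handling ties, then server-travels to the next map.
; Players joining after the start become spectators.
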(event Custom|UpdateScore
  (for _array_element (Variables|DoNotEdit|GetAll%20Players)
    (Default|UpdateScore (.AsBP%20PC%20Party%20Game (Utilities|Casting|CastToBP_PC_PartyGame _array_element)))))

(event Custom|CountdownWidget
  (bind _outactors (Actor|GetAllActorsOfClass "/Game/PartyGameKit/Blueprints/BP_PC_PartyGame.BP_PC_PartyGame_C"))
  (for _array_element _outactors
    (Default|Countdown _array_element)))

(event Custom|GameFinish
  (bind _outactors (Actor|GetAllActorsOfClass "/Game/PartyGameKit/Blueprints/Gamemode_Content/BP_EggGoal.BP_EggGoal_C"))
  (for _array_element _outactors
    (Variables|/Game/PartyGameKit/Blueprints/Gamemode_Content/BP_EggGoal.BP_EggGoal_C|SetisGameStarted? _array_element false)))

(event Custom|GameStart
  (bind _outactors (Actor|GetAllActorsOfClass "/Game/PartyGameKit/Blueprints/Gamemode_Content/BP_EggGoal.BP_EggGoal_C"))
  (for _array_element _outactors
    (Variables|/Game/PartyGameKit/Blueprints/Gamemode_Content/BP_EggGoal.BP_EggGoal_C|SetisGameStarted? _array_element true)))

(event Custom|RedWinUI
  ;[0 0 0] Teams Win UI Events
  (bind _outactors (Actor|GetAllActorsOfClass "/Game/PartyGameKit/Blueprints/BP_PC_PartyGame.BP_PC_PartyGame_C"))
  (for _array_element _outactors
    (Default|RedTeamWins _array_element)))

(event Custom|Spectator
  (params (PC :type Player%20Controller%20Object%20Reference))
  (bind _asbp_pc_party_game (Utilities|Casting|CastToBP_PC_PartyGame PC))
  (Default|Spectator _asbp_pc_party_game))

(event Custom|BlueWinUI
  ;[0 0 0] Teams Win UI Events
  (bind _outactors (Actor|GetAllActorsOfClass "/Game/PartyGameKit/Blueprints/BP_PC_PartyGame.BP_PC_PartyGame_C"))
  (for _array_element _outactors
    (Default|BlueTeamWins _array_element)))

(event Custom|FindWinner
  (bind _winnerteams (Variables|DoNotEdit|GetWinnerTeams))
  (bind _output (Utilities|Array|Get(acopy) _winnerteams))
  ;[0 0 0] Get all BP_Egg_Goal instances in the map and save all scores to the 'All Scores' integer array
  (bind _outactors (Actor|GetAllActorsOfClass "/Game/PartyGameKit/Blueprints/Gamemode_Content/BP_EggGoal.BP_EggGoal_C"))
  (for _array_element _outactors
    (Utilities|Array|Add (Variables|DoNotEdit|GetAllScores) (Variables|/Game/PartyGameKit/Blueprints/Gamemode_Content/BP_EggGoal.BP_EggGoal_C|GetScore _array_element)))
  ;[0 0 0] After a 3-second delay, all widgets on the screen are removed. It takes the scores from all BP_Egg_Goal instances that are equal to the highest value in the All Scores array and saves them to the Winner Teams string array.
  (Utilities|FlowControl|Delay 3.0)
  (CallFunction|RemoveAllWidgets)
  (bind _outactors_2 (Actor|GetAllActorsOfClass "/Game/PartyGameKit/Blueprints/Gamemode_Content/BP_EggGoal.BP_EggGoal_C"))
  (for _array_element_2 _outactors_2
    (if (== (Variables|/Game/PartyGameKit/Blueprints/Gamemode_Content/BP_EggGoal.BP_EggGoal_C|GetScore _array_element_2) (.MaxValue (Math|Integer|MaxOfIntArray (Variables|DoNotEdit|GetAllScores))))
      (Utilities|Array|Add (Variables|DoNotEdit|GetWinnerTeams) (Variables|/Game/PartyGameKit/Blueprints/Gamemode_Content/BP_EggGoal.BP_EggGoal_C|GetTeam _array_element_2))))
  ;[0 0 0] If there are multiple teams in the Winner Teams array, all teams are sorted in the Winner Teams Single string. In the Player Controller, Multiple Team Wins is activated, and multiple winning teams are displayed on the screen. After the scores are distributed to the winning teams, the game transitions to the next map after a 5-second delay
  (if (>= (Utilities|Array|Length (Variables|DoNotEdit|GetWinnerTeams)) 2)
    (for _array_element_3 (Variables|DoNotEdit|GetWinnerTeams)
      (Variables|DoNotEdit|SetWinnerTeamsSingle (Utilities|String|Append " " (Variables|DoNotEdit|GetWinnerTeamsSingle) " " _array_element_3 " ")))
    (bind _outactors_3 (Actor|GetAllActorsOfClass "/Game/PartyGameKit/Blueprints/BP_PC_PartyGame.BP_PC_PartyGame_C"))
    (for _array_element_4 _outactors_3
      (Default|MultipleTeamWins _array_element_4 (Variables|DoNotEdit|GetWinnerTeamsSingle)))
    (for _array_element_5 (Variables|DoNotEdit|GetWinnerTeams)
      (CallFunction|SetScore _array_element_5))
    (CallFunction|UpdateScore)
    (Utilities|FlowControl|Delay 5.0)
    (CallFunction|NextMap)
    (else
      ;[0 0 0] If there is only one winning team, the winning UI specific to the team stored at the first index of the Winner Teams array is activated, and scores are given. Then, after a 5-second delay, the game transitions to the next map.
      (bind _outactors_4 (Actor|GetAllActorsOfClass "/Game/PartyGameKit/Blueprints/Gamemode_Content/BP_EggGoal.BP_EggGoal_C"))
      (for _array_element_6 _outactors_4
        (if (== (Variables|/Game/PartyGameKit/Blueprints/Gamemode_Content/BP_EggGoal.BP_EggGoal_C|GetScore _array_element_6) (.MaxValue (Math|Integer|MaxOfIntArray (Variables|DoNotEdit|GetAllScores))))
          (if (Utilities|String|Contains _output "Red")
            (CallFunction|RedWinUI)
            (elif (Utilities|String|Contains _output "Blue")
              (CallFunction|BlueWinUI)
              (elif (Utilities|String|Contains _output "Yellow")
                (CallFunction|YellowWinUI)
                (elif (Utilities|String|Contains _output "Green")
                  (CallFunction|GreenWinUI)))))))
      (CallFunction|SetScore _output)
      (CallFunction|UpdateScore)
      (Utilities|FlowControl|Delay 5.0)
      (CallFunction|NextMap))))

(event Custom|YellowWinUI
  ;[0 0 0] Teams Win UI Events
  (bind _outactors (Actor|GetAllActorsOfClass "/Game/PartyGameKit/Blueprints/BP_PC_PartyGame.BP_PC_PartyGame_C"))
  (for _array_element _outactors
    (Default|YellowTeamWins _array_element)))

(event Custom|RemoveWaitingWidget
  (bind _outactors (Actor|GetAllActorsOfClass "/Game/PartyGameKit/Blueprints/BP_PC_PartyGame.BP_PC_PartyGame_C"))
  (for _array_element _outactors
    (Default|RemoveWaiting _array_element)))

(event Custom|NextMap
  (bind _asgi_party_game (Utilities|Casting|CastToGI_PartyGame (Game|GetGameInstance)))
  (bind _result (Math|Integer|IncrementInt (Variables|/Game/PartyGameKit/Blueprints/GI_PartyGame.GI_PartyGame_C|GetMapIndex _asgi_party_game))
    (:%20%20
      (bind _output_get (Variables|/Game/PartyGameKit/Blueprints/GI_PartyGame.GI_PartyGame_C|SetMapIndex _asgi_party_game _result))
      (Development|ExecuteConsoleCommand (Utilities|String|Append "servertravel /game/PartyGameKit/Maps/" (Utilities|Array|Get(acopy) (Variables|/Game/PartyGameKit/Blueprints/GI_PartyGame.GI_PartyGame_C|GetMapList _asgi_party_game) _output_get)) (Game|GetPlayerController 0)))))

(event Custom|SetTeam
  (bind _outactors (Actor|GetAllActorsOfClass "/Game/PartyGameKit/Blueprints/Characters/BP_PGKThirdPersonCharacter.BP_PGKThirdPersonCharacter_C"))
  (for (_array_element _array_index) _outactors
    (Variables|/Game/PartyGameKit/Blueprints/Characters/BP_PGKThirdPersonCharacter.BP_PGKThirdPersonCharacter_C|SetTeam _array_element (Utilities|Array|Get(acopy) (Variables|DoNotEdit|GetTeams) _array_index))
    (Default|SetTeamColor _array_element)))

(event Custom|RemoveAllWidgets
  (bind _outactors (Actor|GetAllActorsOfClass "/Game/PartyGameKit/Blueprints/BP_PC_PartyGame.BP_PC_PartyGame_C"))
  (for _array_element _outactors
    (Default|RemoveAllWidget _array_element)))

(event Custom|TimerWidget
  (bind _outactors (Actor|GetAllActorsOfClass "/Game/PartyGameKit/Blueprints/BP_PC_PartyGame.BP_PC_PartyGame_C"))
  (for _array_element _outactors
    (Default|Timer _array_element (Variables|MainSettings|GetFinishGameDelay))))

(event Custom|EggScoreWidget
  (bind _outactors (Actor|GetAllActorsOfClass "/Game/PartyGameKit/Blueprints/BP_PC_PartyGame.BP_PC_PartyGame_C"))
  (for _array_element _outactors
    (Default|EEggCounter _array_element)))

(event Custom|GreenWinUI
  ;[0 0 0] Teams Win UI Events
  (bind _outactors (Actor|GetAllActorsOfClass "/Game/PartyGameKit/Blueprints/BP_PC_PartyGame.BP_PC_PartyGame_C"))
  (for _array_element _outactors
    (Default|GreenTeamWins _array_element)))

(event Custom|TimeOver
  (bind _outactors (Actor|GetAllActorsOfClass "/Game/PartyGameKit/Blueprints/BP_PC_PartyGame.BP_PC_PartyGame_C"))
  (for _array_element _outactors
    (Default|RemoveAllWidget _array_element)
    (Default|TimeOver _array_element)))

(event Custom|WaitingWidget
  (params (Controller :type Controller%20Object%20Reference))
  (bind _asbp_pc_party_game (Utilities|Casting|CastToBP_PC_PartyGame Controller))
  (Default|WaitingforPlayers _asbp_pc_party_game))

(event Custom|SetGameMode
  (bind _outactors (Actor|GetAllActorsOfClass "/Game/PartyGameKit/Blueprints/Characters/BP_PGKThirdPersonCharacter.BP_PGKThirdPersonCharacter_C"))
  (for _array_element _outactors
    (Variables|/Game/PartyGameKit/Blueprints/Characters/BP_PGKThirdPersonCharacter.BP_PGKThirdPersonCharacter_C|SetGamemodeEnum _array_element "NewEnumerator4")))

(event Custom|SetScore
  (params (Team :type String))
  (bind _outactors (Actor|GetAllActorsOfClass "/Game/PartyGameKit/Blueprints/Characters/BP_PGKThirdPersonCharacter.BP_PGKThirdPersonCharacter_C"))
  (for _array_element _outactors
    (if (Utilities|String|Contains (Variables|/Game/PartyGameKit/Blueprints/Characters/BP_PGKThirdPersonCharacter.BP_PGKThirdPersonCharacter_C|GetTeam _array_element) Team)
      (Default|SetScore _array_element (+ (Variables|/Game/PartyGameKit/Blueprints/Characters/BP_PGKThirdPersonCharacter.BP_PGKThirdPersonCharacter_C|GetCurrentScore _array_element) (Variables|MainSettings|GetE_Score))))))

(event Custom|FinishGame
  (Utilities|FlowControl|Delay (Variables|MainSettings|GetFinishGameDelay))
  (CallFunction|TimeOver)
  (CallFunction|GameFinish)
  (CallFunction|FindWinner)
  (Utilities|FlowControl|Delay 5.0)
  (CallFunction|NextMap))

(event EventOnSwapPlayerControllers
  (params (OldPC :type Player%20Controller%20Object%20Reference) (NewPC :type Player%20Controller%20Object%20Reference))
  ;[0 0 0] Player Connect - Disconnect
  (Utilities|Array|Add (Variables|DoNotEdit|GetAll%20Players) NewPC))

(event EventPostLogin
  (params (NewPlayer :type Player%20Controller%20Object%20Reference))
  ;[0 0 0] Player Connect - Disconnect
  (Utilities|Array|Add (Variables|DoNotEdit|GetAll%20Players) NewPlayer)
  (if (Variables|DoNotEdit|GetisGameStarted?)
    (CallFunction|Spectator NewPlayer)
    (else
      (CallFunction|WaitingWidget NewPlayer)))
  (CallFunction|UpdateScore))

(event EventBeginPlay
  (Utilities|FlowControl|Delay (Variables|MainSettings|GetWaitingForPlayersDelay))
  (CallFunction|RemoveWaitingWidget)
  (CallFunction|CountdownWidget)
  (Variables|DoNotEdit|SetisGameStarted? true)
  (Utilities|FlowControl|Delay 3.0)
  (CallFunction|SetGameMode)
  (bind _returnvalue (Actor|GetActorOfClass "/Game/PartyGameKit/Blueprints/Gamemode_Content/BP_EggSpawner.BP_EggSpawner_C"))
  (Default|SVRStartSpawner _returnvalue)
  (CallFunction|SetTeam)
  (CallFunction|EggScoreWidget)
  (CallFunction|TimerWidget)
  (CallFunction|GameStart)
  (CallFunction|FinishGame))

(event EventOnLogout
  (params (ExitingController :type Controller%20Object%20Reference))
  ;[0 0 0] Player Connect - Disconnect
  (bind _asbp_pc_party_game (Utilities|Casting|CastToBP_PC_PartyGame ExitingController))
  (Utilities|Array|RemoveItem (Variables|DoNotEdit|GetAll%20Players) _asbp_pc_party_game)
  (CallFunction|UpdateScore))

(fn ConstructionScript)