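; Game mode for the Escape the Missiles party minigame, where the last surviving character wins.
; After a waiting delay and countdown, a self-repeating event spawns missiles at tagged target points, aimed at random characters.
; Tick detects one remaining character, then clears missiles, awards score, shows the winner and server-travels to the game instance's next map.
; Late joiners spectate; the "NO ONE" branch is unreachable because it repeats the one-character check.
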(event Custom|UpdateScore
  (for _array_element (Variables|DoNotEdit|GetAll%20Players)
    (Default|UpdateScore (.AsBP%20PC%20Party%20Game (Utilities|Casting|CastToBP_PC_PartyGame _array_element)))))

(event Custom|Countdown
  (bind _outactors (Actor|GetAllActorsOfClass "/Game/PartyGameKit/Blueprints/BP_PC_PartyGame.BP_PC_PartyGame_C"))
  (for _array_element _outactors
    (Default|Countdown _array_element)))

(event Custom|Spectator
  (params (PC :type Player%20Controller%20Object%20Reference))
  (bind _asbp_pc_party_game (Utilities|Casting|CastToBP_PC_PartyGame PC))
  (Default|Spectator _asbp_pc_party_game))

(event Custom|RemoveWaitingWidget
  (bind _outactors (Actor|GetAllActorsOfClass "/Game/PartyGameKit/Blueprints/BP_PC_PartyGame.BP_PC_PartyGame_C"))
  (for _array_element _outactors
    (Default|RemoveWaiting _array_element)))

(event Custom|NextMap
  (bind _asgi_party_game (Utilities|Casting|CastToGI_PartyGame (Game|GetGameInstance)))
  (bind _result (Math|Integer|IncrementInt (Variables|/Game/PartyGameKit/Blueprints/GI_PartyGame.GI_PartyGame_C|GetMapIndex _asgi_party_game))
    (:%20%20
      (bind _output_get (Variables|/Game/PartyGameKit/Blueprints/GI_PartyGame.GI_PartyGame_C|SetMapIndex _asgi_party_game _result))
      (Development|ExecuteConsoleCommand (Utilities|String|Append "servertravel /game/PartyGameKit/Maps/" (Utilities|Array|Get(acopy) (Variables|/Game/PartyGameKit/Blueprints/GI_PartyGame.GI_PartyGame_C|GetMapList _asgi_party_game) _output_get)) (Game|GetPlayerController 0)))))

(event Custom|RPC_Missile
  (if (Variables|DoNotEdit|GetisGameStarted?)
    (bind _outactors (Actor|GetAllActorsOfClass "/Game/PartyGameKit/Blueprints/Characters/BP_PGKThirdPersonCharacter.BP_PGKThirdPersonCharacter_C"))
    (bind _outactors_2 (Actor|GetAllActorsOfClasswithTag "/Script/Engine.TargetPoint" "Missile"))
    (Game|SpawnActorfromClass "/Game/PartyGameKit/Blueprints/Gamemode_Content/BP_Missile.BP_Missile_C" (Math|Transform|MakeTransform (Transformation|GetActorLocation (.OutItem (Utilities|Array|Random _outactors_2))) "0, 0, 0" "1.000000,1.000000,1.000000") "Undefined" "MultiplyWithRoot" 0 (Variables|/Script/Engine.Character|GetCapsuleComponent (.OutItem (Utilities|Array|Random _outactors))) 0)
    (Utilities|FlowControl|Delay (Variables|MainSettings|GetTriggerDelay))
    (CallFunction|RPCMissile)))

(event Custom|Heart
  (bind _outactors (Actor|GetAllActorsOfClass "/Game/PartyGameKit/Blueprints/BP_PC_PartyGame.BP_PC_PartyGame_C"))
  (for _array_element _outactors
    (Default|ETMHeart _array_element)))

(event Custom|DestroyAllMissiles
  (bind _outactors (Actor|GetAllActorsOfClass "/Game/PartyGameKit/Blueprints/Gamemode_Content/BP_Missile.BP_Missile_C"))
  (for _array_element _outactors
    (Default|MCEffect _array_element)
    (Actor|DestroyActor _array_element)))

(event Custom|WaitingWidget
  (params (Controller :type Controller%20Object%20Reference))
  (bind _asbp_pc_party_game (Utilities|Casting|CastToBP_PC_PartyGame Controller))
  (Default|WaitingforPlayers _asbp_pc_party_game))

(event Custom|FinishGame
  (CallFunction|DestroyAllMissiles)
  (Variables|DoNotEdit|SetisGameStarted? false)
  (bind _returnvalue (Actor|GetActorOfClass "/Game/PartyGameKit/Blueprints/Characters/BP_PGKThirdPersonCharacter.BP_PGKThirdPersonCharacter_C"))
  (CallFunction|SetScore _returnvalue)
  (bind _outactors (Actor|GetAllActorsOfClass "/Game/PartyGameKit/Blueprints/BP_PC_PartyGame.BP_PC_PartyGame_C"))
  (for _array_element _outactors
    (Default|WinnerText _array_element (Variables|/Game/PartyGameKit/Blueprints/Characters/BP_PGKThirdPersonCharacter.BP_PGKThirdPersonCharacter_C|GetPlayerName _returnvalue)))
  (CallFunction|UpdateScore)
  (Utilities|FlowControl|Delay 5.0)
  (CallFunction|NextMap))

(event Custom|SetScore
  (params (Target :type BP%20PGK%20Third%20Person%20Character%20Object%20Reference))
  (Default|SetScore Target (+ (Variables|MainSettings|GetETM_Score) (Variables|/Game/PartyGameKit/Blueprints/Characters/BP_PGKThirdPersonCharacter.BP_PGKThirdPersonCharacter_C|GetCurrentScore Target))))

(event EventOnSwapPlayerControllers
  (params (OldPC :type Player%20Controller%20Object%20Reference) (NewPC :type Player%20Controller%20Object%20Reference))
  ;[0 0 0] Player Connect - Disconnect
  (Utilities|Array|Add (Variables|DoNotEdit|GetAll%20Players) NewPC))

(event EventPostLogin
  (params (NewPlayer :type Player%20Controller%20Object%20Reference))
  ;[0 0 0] Player Connect - Disconnect
  (Utilities|Array|Add (Variables|DoNotEdit|GetAll%20Players) NewPlayer)
  (if (Variables|DoNotEdit|GetisGameStarted?)
    (CallFunction|Spectator NewPlayer)
    (else
      (CallFunction|WaitingWidget NewPlayer)))
  (CallFunction|UpdateScore))

(event EventTick
  (params (DeltaSeconds :type Float%20%28single-precision%29))
  (if (Variables|DoNotEdit|GetisGameStarted?)
    (bind _outactors (Actor|GetAllActorsOfClass "/Game/PartyGameKit/Blueprints/Characters/BP_PGKThirdPersonCharacter.BP_PGKThirdPersonCharacter_C"))
    (if (== (Utilities|Array|Length _outactors) 1)
      (Utilities|FlowControl|DoOnce false
        (:Completed
          (CallFunction|FinishGame)))
      (elif (== (Utilities|Array|Length _outactors) 1)
        (bind _outactors_2 (Actor|GetAllActorsOfClass "/Game/PartyGameKit/Blueprints/BP_PC_PartyGame.BP_PC_PartyGame_C"))
        (for _array_element _outactors_2
          (Default|WinnerText _array_element "NO ONE"))
        (Utilities|FlowControl|Delay 5.0)
        (CallFunction|NextMap)))))

(event EventBeginPlay
  (Utilities|FlowControl|Delay (Variables|MainSettings|GetWaitingForPlayersDelay))
  (CallFunction|Countdown)
  (CallFunction|RemoveWaitingWidget)
  (Variables|DoNotEdit|SetisGameStarted? true)
  (Utilities|FlowControl|Delay 3.0)
  (CallFunction|RPCMissile)
  (CallFunction|Heart))

(event EventOnLogout
  (params (ExitingController :type Controller%20Object%20Reference))
  ;[0 0 0] Player Connect - Disconnect
  (bind _asbp_pc_party_game (Utilities|Casting|CastToBP_PC_PartyGame ExitingController))
  (Utilities|Array|RemoveItem (Variables|DoNotEdit|GetAll%20Players) _asbp_pc_party_game)
  (CallFunction|UpdateScore))

(fn ConstructionScript)