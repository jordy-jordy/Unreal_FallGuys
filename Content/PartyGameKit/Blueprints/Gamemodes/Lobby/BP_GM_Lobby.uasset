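; Lobby game mode for a multiplayer party game that tracks joined player controllers and starts the match.
; On login it puts the player into the waiting lobby, and each login or logout updates the controller array and triggers a delayed list refresh on the game state.
; Starting the game runs a servertravel console command to the game instance's selected map, while KickPlayer removes players by array index.
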(event Custom|Starting%20Game
  (bind _asgi_party_game (Utilities|Casting|CastToGI_PartyGame (Game|GetGameInstance)))
  (if (Utilities|Array|IsEmpty (Variables|/Game/PartyGameKit/Blueprints/GI_PartyGame.GI_PartyGame_C|GetMapList _asgi_party_game))
    (Development|PrintString "No map seems to be selected.")
    (else
      (Development|ExecuteConsoleCommand (Utilities|String|Append "servertravel /game/PartyGameKit/Maps/" (Utilities|Array|Get(acopy) (Variables|/Game/PartyGameKit/Blueprints/GI_PartyGame.GI_PartyGame_C|GetMapList _asgi_party_game) (Variables|/Game/PartyGameKit/Blueprints/GI_PartyGame.GI_PartyGame_C|GetMapIndex _asgi_party_game))) (Game|GetPlayerController 0)))))

(event Custom|UpdateList
  (Utilities|FlowControl|Delay 0.5)
  (bind _asbp_gs_party_game (Utilities|Casting|CastToBP_GS_PartyGame (Game|GetGameState)))
  (Default|UpdateList _asbp_gs_party_game))

(event EventPostLogin
  (params (NewPlayer :type Player%20Controller%20Object%20Reference))
  (bind _asbp_pc_party_game (Utilities|Casting|CastToBP_PC_PartyGame NewPlayer))
  (Default|WaitingLobby _asbp_pc_party_game)
  (Utilities|Array|Add (Variables|Default|GetPlayer%20Controllers) _asbp_pc_party_game)
  (CallFunction|UpdateList))

(event EventOnLogout
  (params (ExitingController :type Controller%20Object%20Reference))
  (bind _asbp_pc_party_game (Utilities|Casting|CastToBP_PC_PartyGame ExitingController))
  (Utilities|Array|RemoveItem (Variables|Default|GetPlayer%20Controllers) _asbp_pc_party_game)
  (CallFunction|UpdateList))

(fn ConstructionScript)

(fn KickPlayer
  (params (PlayerID :type Integer))
  (Default|KickPlayer (Utilities|Array|Get(acopy) (Variables|Default|GetPlayer%20Controllers) PlayerID)))