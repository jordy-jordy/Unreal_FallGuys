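; Game mode for the Catch Tail party minigame, where whoever holds the tail when time runs out wins points.
; BeginPlay runs the round: waiting period, countdown, random tail assignment, timer, then winner announcement, scoring and servertravel to the next map in GI_PartyGame's MapList.
; It tracks players through login and logout, making late joiners spectators.
; UI changes are pushed by looping over BP_PC_PartyGame controllers.
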(event Custom|UpdateScore
  (for _array_element (Variables|DoNotEdit|GetAll%20Players)
    (Default|UpdateScore (.AsBP%20PC%20Party%20Game (Utilities|Casting|CastToBP_PC_PartyGame _array_element)))))

(event Custom|SetTails
  (bind _outactors (Actor|GetAllActorsOfClass "/Game/PartyGameKit/Blueprints/Characters/BP_PGKThirdPersonCharacter.BP_PGKThirdPersonCharacter_C"))
  (bind _output_get (Variables|DoNotEdit|SetTailPlayer (.OutItem (Utilities|Array|Random _outactors))))
  (Default|SVRAddTail _output_get)
  (bind _asbp_pc_party_game (Utilities|Casting|CastToBP_PC_PartyGame (Pawn|GetController _output_get)))
  (Default|CTCatchTail _asbp_pc_party_game))

(event Custom|RemoveAllWidget
  (bind _outactors (Actor|GetAllActorsOfClass "/Game/PartyGameKit/Blueprints/BP_PC_PartyGame.BP_PC_PartyGame_C"))
  (for _array_element _outactors
    (Default|RemoveAllWidget _array_element)))

(event Custom|NextMap
  (bind _asgi_party_game (Utilities|Casting|CastToGI_PartyGame (Game|GetGameInstance)))
  (bind _result (Math|Integer|IncrementInt (Variables|/Game/PartyGameKit/Blueprints/GI_PartyGame.GI_PartyGame_C|GetMapIndex _asgi_party_game))
    (:%20%20
      (bind _output_get (Variables|/Game/PartyGameKit/Blueprints/GI_PartyGame.GI_PartyGame_C|SetMapIndex _asgi_party_game _result))
      (Development|ExecuteConsoleCommand (Utilities|String|Append "servertravel /game/PartyGameKit/Maps/" (Utilities|Array|Get(acopy) (Variables|/Game/PartyGameKit/Blueprints/GI_PartyGame.GI_PartyGame_C|GetMapList _asgi_party_game) _output_get)) (Game|GetPlayerController 0)))))

(event Custom|SetScore
  (bind _tailplayer (Variables|DoNotEdit|GetTailPlayer))
  (Default|SetScore _tailplayer (+ (Variables|/Game/PartyGameKit/Blueprints/Characters/BP_PGKThirdPersonCharacter.BP_PGKThirdPersonCharacter_C|GetCurrentScore _tailplayer) (Variables|MainSettings|GetT_Score))))

(event Custom|Spectator
  (params (PC :type Player%20Controller%20Object%20Reference))
  (bind _asbp_pc_party_game (Utilities|Casting|CastToBP_PC_PartyGame PC))
  (Default|Spectator _asbp_pc_party_game))

(event Custom|SetGamemode
  (bind _outactors (Actor|GetAllActorsOfClass "/Game/PartyGameKit/Blueprints/Characters/BP_PGKThirdPersonCharacter.BP_PGKThirdPersonCharacter_C"))
  (for _array_element _outactors
    (Variables|/Game/PartyGameKit/Blueprints/Characters/BP_PGKThirdPersonCharacter.BP_PGKThirdPersonCharacter_C|SetGamemodeEnum _array_element "NewEnumerator1")))

(event Custom|Finish%20Game
  (Utilities|FlowControl|Delay (Variables|MainSettings|GetFinishGameDelay))
  (CallFunction|TimeOver)
  (Utilities|FlowControl|Delay 3.0)
  (CallFunction|RemoveAllWidget)
  (CallFunction|FindTailPlayer)
  (bind _tailplayer (Variables|DoNotEdit|GetTailPlayer)
    (:then
      (CallFunction|Winner (Variables|/Game/PartyGameKit/Blueprints/Characters/BP_PGKThirdPersonCharacter.BP_PGKThirdPersonCharacter_C|GetPlayerName _tailplayer))
      (CallFunction|SetScore)
      (CallFunction|UpdateScore)
      (Utilities|FlowControl|Delay 5.0)
      (CallFunction|NextMap))
    (:else)))

(event Custom|Winner
  (params (PlayerName :type String))
  (bind _outactors (Actor|GetAllActorsOfClass "/Game/PartyGameKit/Blueprints/BP_PC_PartyGame.BP_PC_PartyGame_C"))
  (for _array_element _outactors
    (Default|WinnerText _array_element PlayerName)))

(event Custom|Countdown
  (bind _outactors (Actor|GetAllActorsOfClass "/Game/PartyGameKit/Blueprints/BP_PC_PartyGame.BP_PC_PartyGame_C"))
  (for _array_element _outactors
    (Default|Countdown _array_element)))

(event Custom|TimeOver
  (bind _outactors (Actor|GetAllActorsOfClass "/Game/PartyGameKit/Blueprints/BP_PC_PartyGame.BP_PC_PartyGame_C"))
  (for _array_element _outactors
    (Default|RemoveAllWidget _array_element)
    (Default|TimeOver _array_element)))

(event Custom|WaitingWidget
  (params (Controller :type Controller%20Object%20Reference))
  (bind _asbp_pc_party_game (Utilities|Casting|CastToBP_PC_PartyGame Controller))
  (Default|WaitingforPlayers _asbp_pc_party_game))

(event Custom|RemoveWaitingWidget
  (bind _outactors (Actor|GetAllActorsOfClass "/Game/PartyGameKit/Blueprints/BP_PC_PartyGame.BP_PC_PartyGame_C"))
  (for _array_element _outactors
    (Default|RemoveWaiting _array_element)))

(event Custom|Timer
  (bind _outactors (Actor|GetAllActorsOfClass "/Game/PartyGameKit/Blueprints/BP_PC_PartyGame.BP_PC_PartyGame_C"))
  (for _array_element _outactors
    (Default|Timer _array_element (Variables|MainSettings|GetFinishGameDelay))))

(event Custom|FindTailPlayer
  (bind _outactors (Actor|GetAllActorsOfClass "/Game/PartyGameKit/Blueprints/Characters/BP_PGKThirdPersonCharacter.BP_PGKThirdPersonCharacter_C"))
  (for _array_element _outactors
    (if (Variables|/Game/PartyGameKit/Blueprints/Characters/BP_PGKThirdPersonCharacter.BP_PGKThirdPersonCharacter_C|GetHaveTail? _array_element)
      (Variables|DoNotEdit|SetTailPlayer _array_element))))

(event EventOnSwapPlayerControllers
  (params (OldPC :type Player%20Controller%20Object%20Reference) (NewPC :type Player%20Controller%20Object%20Reference))
  ;[0 0 0] Player Connect - Disconnect
  (Utilities|Array|Add (Variables|DoNotEdit|GetAll%20Players) NewPC))

(event EventPostLogin
  (params (NewPlayer :type Player%20Controller%20Object%20Reference))
  ;[0 0 0] Player Connect - Disconnect
  (Utilities|Array|Add (Variables|DoNotEdit|GetAll%20Players) NewPlayer)
  (if (Variables|DoNotEdit|GetisGameStarted?)
    (CallFunction|Spectator NewPlayer)
    (else
      (CallFunction|WaitingWidget NewPlayer)))
  (CallFunction|UpdateScore))

(event EventBeginPlay
  (Utilities|FlowControl|Delay (Variables|MainSettings|GetWaitingForPlayersDelay))
  (Variables|DoNotEdit|SetisGameStarted? true)
  (CallFunction|RemoveWaitingWidget)
  (CallFunction|SetGamemode)
  (CallFunction|Countdown)
  (Utilities|FlowControl|Delay 3.0)
  (CallFunction|SetTails)
  (CallFunction|Timer)
  (CallFunction|FinishGame))

(event EventOnLogout
  (params (ExitingController :type Controller%20Object%20Reference))
  ;[0 0 0] Player Connect - Disconnect
  (bind _asbp_pc_party_game (Utilities|Casting|CastToBP_PC_PartyGame ExitingController))
  (Utilities|Array|RemoveItem (Variables|DoNotEdit|GetAll%20Players) _asbp_pc_party_game)
  (CallFunction|UpdateScore))

(fn ConstructionScript)