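; Game mode for the HopHop survival party minigame, where the last remaining character wins.
; After a waiting delay it runs a countdown and starts the HopHop stick; late joiners become spectators.
; While the game runs, Tick triggers a check on the character count, announcing the winner and adding score, or "NO ONE" if none remain.
; It then server-travels to the next map in the game instance's list.
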(event Custom|UpdateScore
  (for _array_element (Variables|DoNotEdit|GetAll%20Players)
    (Default|UpdateScore (.AsBP%20PC%20Party%20Game (Utilities|Casting|CastToBP_PC_PartyGame _array_element)))))

(event Custom|NextMap
  (bind _asgi_party_game (Utilities|Casting|CastToGI_PartyGame (Game|GetGameInstance)))
  (bind _result (Math|Integer|IncrementInt (Variables|/Game/PartyGameKit/Blueprints/GI_PartyGame.GI_PartyGame_C|GetMapIndex _asgi_party_game))
    (:%20%20
      (bind _output_get (Variables|/Game/PartyGameKit/Blueprints/GI_PartyGame.GI_PartyGame_C|SetMapIndex _asgi_party_game _result))
      (Development|ExecuteConsoleCommand (Utilities|String|Append "servertravel /game/PartyGameKit/Maps/" (Utilities|Array|Get(acopy) (Variables|/Game/PartyGameKit/Blueprints/GI_PartyGame.GI_PartyGame_C|GetMapList _asgi_party_game) _output_get)) (Game|GetPlayerController 0)))))

(event Custom|Spectator
  (params (PC :type Player%20Controller%20Object%20Reference))
  (bind _asbp_pc_party_game (Utilities|Casting|CastToBP_PC_PartyGame PC))
  (Default|Spectator _asbp_pc_party_game))

(event Custom|RemoveWaitingWidget
  (bind _outactors (Actor|GetAllActorsOfClass "/Game/PartyGameKit/Blueprints/BP_PC_PartyGame.BP_PC_PartyGame_C"))
  (for _array_element _outactors
    (Default|RemoveWaiting _array_element)))

(event Custom|SVR_GameEnd
  (bind _outactors (Actor|GetAllActorsOfClass "/Game/PartyGameKit/Blueprints/Characters/BP_PGKThirdPersonCharacter.BP_PGKThirdPersonCharacter_C"))
  (if (== (Utilities|Array|Length _outactors) 1)
    (Variables|DoNotEdit|SetisGameStarted? false)
    (bind _returnvalue (Actor|GetActorOfClass "/Game/PartyGameKit/Blueprints/Characters/BP_PGKThirdPersonCharacter.BP_PGKThirdPersonCharacter_C"))
    (Pawn|Components|CharacterMovement|DisableMovement (Variables|/Script/Engine.Character|GetCharacterMovement _returnvalue))
    (bind _outactors_2 (Actor|GetAllActorsOfClass "/Game/PartyGameKit/Blueprints/BP_PC_PartyGame.BP_PC_PartyGame_C"))
    (for _array_element _outactors_2
      (Default|WinnerText _array_element (Variables|/Game/PartyGameKit/Blueprints/Characters/BP_PGKThirdPersonCharacter.BP_PGKThirdPersonCharacter_C|GetPlayerName _returnvalue)))
    (Default|SetScore _returnvalue (+ (Variables|/Game/PartyGameKit/Blueprints/Characters/BP_PGKThirdPersonCharacter.BP_PGKThirdPersonCharacter_C|GetCurrentScore _returnvalue) (Variables|MainSettings|GetH_Score)))
    (CallFunction|UpdateScore)
    (Utilities|FlowControl|Delay 5.0)
    (CallFunction|NextMap)
    (elif (== (Utilities|Array|Length _outactors) 0)
      (Variables|DoNotEdit|SetisGameStarted? false)
      (bind _outactors_3 (Actor|GetAllActorsOfClass "/Game/PartyGameKit/Blueprints/BP_PC_PartyGame.BP_PC_PartyGame_C"))
      (for _array_element_2 _outactors_3
        (Default|WinnerText _array_element_2 "NO ONE "))
      (Utilities|FlowControl|Delay 5.0)
      (CallFunction|NextMap))))

(event Custom|WaitingWidget
  (params (Controller :type Controller%20Object%20Reference))
  (bind _asbp_pc_party_game (Utilities|Casting|CastToBP_PC_PartyGame Controller))
  (Default|WaitingforPlayers _asbp_pc_party_game))

(event EventOnSwapPlayerControllers
  (params (OldPC :type Player%20Controller%20Object%20Reference) (NewPC :type Player%20Controller%20Object%20Reference))
  ;[0 0 0] Player Connect - Disconnect
  (Utilities|Array|Add (Variables|DoNotEdit|GetAll%20Players) NewPC))

(event EventPostLogin
  (params (NewPlayer :type Player%20Controller%20Object%20Reference))
  ;[0 0 0] Player Connect - Disconnect
  (Utilities|Array|Add (Variables|DoNotEdit|GetAll%20Players) NewPlayer)
  (if (Variables|DoNotEdit|GetisGameStarted?)
    (CallFunction|Spectator NewPlayer)
    (else
      (CallFunction|WaitingWidget NewPlayer)))
  (CallFunction|UpdateScore))

(event EventBeginPlay
  (Utilities|FlowControl|Delay (Variables|MainSettings|GetWaitingForPlayersDelay))
  (CallFunction|RemoveWaitingWidget)
  (Variables|DoNotEdit|SetisGameStarted? true)
  (bind _outactors (Actor|GetAllActorsOfClass "/Game/PartyGameKit/Blueprints/BP_PC_PartyGame.BP_PC_PartyGame_C"))
  (for _array_element _outactors
    (Default|Countdown _array_element))
  (Utilities|FlowControl|Delay 3.0)
  (bind _returnvalue (Actor|GetActorOfClass "/Game/PartyGameKit/Blueprints/Obstacles/BP_HopHopStick.BP_HopHopStick_C"))
  (Default|Start _returnvalue))

(event EventTick
  (params (DeltaSeconds :type Float%20%28single-precision%29))
  (if (Variables|DoNotEdit|GetisGameStarted?)
    (CallFunction|SVRGameEnd)))

(event EventOnLogout
  (params (ExitingController :type Controller%20Object%20Reference))
  ;[0 0 0] Player Connect - Disconnect
  (bind _asbp_pc_party_game (Utilities|Casting|CastToBP_PC_PartyGame ExitingController))
  (Utilities|Array|RemoveItem (Variables|DoNotEdit|GetAll%20Players) _asbp_pc_party_game)
  (CallFunction|UpdateScore))

(fn ConstructionScript)