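; BP_Qualifed is a qualification trigger volume for the Parkour and Mountain Run party game modes.
; BeginPlay caches the game mode matching CurrentMap.
; On box overlap, an unqualified character is marked qualified, its controller is notified and the mode records its score.
; The player then possesses a spectator pawn spawned at the tagged SpectatorSpawn point, the character is destroyed, and the first qualifier alone triggers the mode's timer.
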(event OnComponentBeginOverlap(Box)
  (params (OverlappedComponent :type Primitive%20Component%20Object%20Reference) (OtherActor :type Actor%20Object%20Reference) (OtherComp :type Primitive%20Component%20Object%20Reference) (OtherBodyIndex :type Integer) (bFromSweep :type Boolean) (SweepResult :type Hit%20Result%20Structure%20%28by%20ref%29))
  (bind _asbp_pgkthird_person_character (Utilities|Casting|CastToBP_PGKThirdPersonCharacter OtherActor))
  (if (not (Variables|/Game/PartyGameKit/Blueprints/Characters/BP_PGKThirdPersonCharacter.BP_PGKThirdPersonCharacter_C|GetisQualified? _asbp_pgkthird_person_character))
    (Variables|/Game/PartyGameKit/Blueprints/Characters/BP_PGKThirdPersonCharacter.BP_PGKThirdPersonCharacter_C|SetisQualified? _asbp_pgkthird_person_character true)
    (bind _asbp_pc_party_game (Utilities|Casting|CastToBP_PC_PartyGame (Pawn|GetController _asbp_pgkthird_person_character)))
    (Default|Qualified _asbp_pc_party_game)
    (bind _outactors (Actor|GetAllActorsOfClasswithTag "/Script/Engine.TargetPoint" "SpectatorSpawn"))
    (Utilities|IsValid (Utilities|Array|Get(acopy) _outactors)
      (:Is%20Valid
        (Variables|Default|SetSpawn%20Transform%20Location (Transformation|GetActorLocation (Utilities|Array|Get(acopy) _outactors))))
      (:Is%20Not%20Valid
        (Variables|Default|SetSpawn%20Transform%20Location "0, 0, 0")))
    (switch Utilities|FlowControl|Switch|SwitchonE_Qualified (Variables|Default|GetCurrentMap)
      (:NewEnumerator3
        (Default|SetScoreWinner (Variables|Default|GetParkourModeVar) _asbp_pgkthird_person_character))
      (:NewEnumerator4
        (Default|SetScore (Variables|Default|GetMountainRunVar) _asbp_pgkthird_person_character)))
    (bind _returnvalue (Game|SpawnActorfromClass "/Game/PartyGameKit/Blueprints/BP_SP_PartyGame.BP_SP_PartyGame_C" (Math|Transform|MakeTransform (Variables|Default|GetSpawn%20Transform%20Location) "0, 0, 0" "1.000000,1.000000,1.000000") "Undefined" "MultiplyWithRoot" 0 0))
    (Default|Spectator _returnvalue _asbp_pc_party_game)
    (Pawn|Possess (Pawn|GetController _asbp_pgkthird_person_character) _returnvalue)
    (Actor|DestroyActor _asbp_pgkthird_person_character)
    (Utilities|FlowControl|DoOnce false
      (:Completed
        (switch Utilities|FlowControl|Switch|SwitchonE_Qualified (Variables|Default|GetCurrentMap)
          (:NewEnumerator3
            (Default|TriggerTimer (Variables|Default|GetParkourModeVar)))
          (:NewEnumerator4
            (Default|TriggerTimer (Variables|Default|GetMountainRunVar))))))))

(event EventBeginPlay
  (switch Utilities|FlowControl|Switch|SwitchonE_Qualified (Variables|Default|GetCurrentMap)
    (:NewEnumerator3
      (bind _asbp_gm_parkour (Utilities|Casting|CastToBP_GM_Parkour (Game|GetGameMode)))
      (Variables|Default|SetParkourModeVar _asbp_gm_parkour))
    (:NewEnumerator4
      (bind _asbp_gm_mountain_run (Utilities|Casting|CastToBP_GM_MountainRun (Game|GetGameMode)))
      (Variables|Default|SetMountainRunVar _asbp_gm_mountain_run))))

(fn ConstructionScript)