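; BP_EggGoal is a goal zone for an egg game mode that keeps a score of the eggs inside it.
; Once the game has started, the server counts BP_Egg actors entering and leaving its Box collision, raising or lowering Score.
; Each egg's Captured flag is set on entry and cleared on exit, guarding against counting the same egg twice.
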(event OnComponentBeginOverlap(Box)
  (params (OverlappedComponent :type Primitive%20Component%20Object%20Reference) (OtherActor :type Actor%20Object%20Reference) (OtherComp :type Primitive%20Component%20Object%20Reference) (OtherBodyIndex :type Integer) (bFromSweep :type Boolean) (SweepResult :type Hit%20Result%20Structure%20%28by%20ref%29))
  ;[0 0 0] When the Collision overlaps, points are added to the score. When the overlap ends, points are deducted from the score.
  (Networking|SwitchHasAuthority
    (:Authority
      (if (Variables|DoNotEdit|GetisGameStarted?)
        (bind _asbp_egg (Utilities|Casting|CastToBP_Egg OtherActor))
        (if (not (Variables|/Game/PartyGameKit/Blueprints/Gamemode_Content/BP_Egg.BP_Egg_C|GetCaptured? _asbp_egg))
          (Variables|/Game/PartyGameKit/Blueprints/Gamemode_Content/BP_Egg.BP_Egg_C|SetCaptured? _asbp_egg true)
          (Math|Integer|IncrementInt (Variables|DoNotEdit|GetScore)))))))

(event OnComponentEndOverlap(Box)
  (params (OverlappedComponent :type Primitive%20Component%20Object%20Reference) (OtherActor :type Actor%20Object%20Reference) (OtherComp :type Primitive%20Component%20Object%20Reference) (OtherBodyIndex :type Integer))
  ;[0 0 0] When the Collision overlaps, points are added to the score. When the overlap ends, points are deducted from the score.
  (Networking|SwitchHasAuthority
    (:Authority
      (if (Variables|DoNotEdit|GetisGameStarted?)
        (bind _asbp_egg (Utilities|Casting|CastToBP_Egg OtherActor))
        (if (Variables|/Game/PartyGameKit/Blueprints/Gamemode_Content/BP_Egg.BP_Egg_C|GetCaptured? _asbp_egg)
          (Variables|/Game/PartyGameKit/Blueprints/Gamemode_Content/BP_Egg.BP_Egg_C|SetCaptured? _asbp_egg false)
          (Math|Integer|DecrementInt (Variables|DoNotEdit|GetScore)))))))

(fn ConstructionScript)