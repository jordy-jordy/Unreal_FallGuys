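; Football goal for the party game's football mode that scores when a BP_Ball overlaps its box.
; On authority it increments the goal count, fires the ball's radial impulse and destroys it.
; The last hitter, matched by player name, gains points or loses them for an own goal, then the game mode updates the scoreboard.
; A multicast event spawns confetti, updates the opposing team's score widget and requests a new ball from the game mode.
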(event OnComponentBeginOverlap(Box)
  (params (OverlappedComponent :type Primitive%20Component%20Object%20Reference) (OtherActor :type Actor%20Object%20Reference) (OtherComp :type Primitive%20Component%20Object%20Reference) (OtherBodyIndex :type Integer) (bFromSweep :type Boolean) (SweepResult :type Hit%20Result%20Structure%20%28by%20ref%29))
  (bind _asbp_ball (Utilities|Casting|CastToBP_Ball OtherActor))
  (Networking|SwitchHasAuthority
    (:Authority
      (CallFunction|SVRSetScore _asbp_ball)
      (Class|RadialForceComponent|FireImpulse (Variables|/Game/PartyGameKit/Blueprints/Gamemode_Content/BP_Ball.BP_Ball_C|GetRadialForce _asbp_ball))
      (bind _outactors (Actor|GetAllActorsOfClass "/Game/PartyGameKit/Blueprints/Characters/BP_PGKThirdPersonCharacter.BP_PGKThirdPersonCharacter_C"))
      (for _array_element _outactors
        (if (Utilities|String|Contains (PlayerState|GetPlayerName (Variables|/Script/Engine.Pawn|GetPlayerState _array_element)) (Variables|/Game/PartyGameKit/Blueprints/Gamemode_Content/BP_Ball.BP_Ball_C|GetLast%20Hit _asbp_ball))
          (if (Utilities|String|Contains (Variables|Default|GetTeam) (Variables|/Game/PartyGameKit/Blueprints/Characters/BP_PGKThirdPersonCharacter.BP_PGKThirdPersonCharacter_C|GetTeam _array_element))
            (Default|SetScore _array_element (- (Variables|/Game/PartyGameKit/Blueprints/Characters/BP_PGKThirdPersonCharacter.BP_PGKThirdPersonCharacter_C|GetCurrentScore _array_element) 10))
            (else
              (Default|SetScore _array_element (+ (Variables|/Game/PartyGameKit/Blueprints/Characters/BP_PGKThirdPersonCharacter.BP_PGKThirdPersonCharacter_C|GetCurrentScore _array_element) 10))))
          (bind _asbp_gm_football (Utilities|Casting|CastToBP_GM_Football (Game|GetGameMode)))
          (Default|UpdateScoreboard _asbp_gm_football)))
      (Actor|DestroyActor _asbp_ball))))

(event Custom|MPC%20Spawn
  (bind _asbp_gm_football (Utilities|Casting|CastToBP_GM_Football (Game|GetGameMode)))
  (Default|SVRSpawnBall _asbp_gm_football))

(event Custom|MulticastSetScore
  (params (Score :type Float%20%28double-precision%29) (Ball :type BP%20Ball%20Object%20Reference))
  (Variables|Default|SetScore Score)
  (Utilities|IsValid Ball
    (:Is%20Valid
      (Variables|Default|SetLocation (Transformation|GetActorLocation Ball)))
    (:Is%20Not%20Valid
      (Variables|Default|SetLocation (Transformation|GetActorLocation))))
  (Niagara|SpawnSystematLocation "/Game/PartyGameKit/VFX/Confetti/NS_Confetti.NS_Confetti" (Variables|Default|GetLocation))
  (bind _outactors (Actor|GetAllActorsOfClass "/Game/PartyGameKit/Blueprints/BP_PC_PartyGame.BP_PC_PartyGame_C"))
  (for _array_element _outactors
    (Utilities|IsValid (Variables|/Game/PartyGameKit/Blueprints/BP_PC_PartyGame.BP_PC_PartyGame_C|GetF_ScoreVar _array_element)
      (:Is%20Valid
        (if (Utilities|String|Contains (Variables|Default|GetTeam) "Red")
          (Default|UpdateBlue (Variables|/Game/PartyGameKit/Blueprints/BP_PC_PartyGame.BP_PC_PartyGame_C|GetF_ScoreVar _array_element) (Variables|Default|GetScore))
          (else
            (Default|UpdateRed (Variables|/Game/PartyGameKit/Blueprints/BP_PC_PartyGame.BP_PC_PartyGame_C|GetF_ScoreVar _array_element) (Variables|Default|GetScore)))))))
  (CallFunction|MPCSpawn))

(event Custom|SVR%20SetScore
  (params (Ball :type BP%20Ball%20Object%20Reference))
  (bind _result (Math|Float|IncrementFloat (Variables|Default|GetScore))
    (:%20%20
      (CallFunction|MulticastSetScore _result Ball))))

(fn ConstructionScript)