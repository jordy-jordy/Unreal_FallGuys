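; BP_Block is a dissolving hex block that disappears after a player character touches it.
; The server detects the box overlap with BP_PGKThirdPersonCharacter and calls a dissolve event, apparently multicast.
; If CanDissolve is set, a brief delay precedes a Timeline that shrinks the Hex mesh to half width, keeping its height.
; When the Timeline finishes, the block spawns a poof effect and destroys itself.
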(event OnComponentBeginOverlap(Box)
  (params (OverlappedComponent :type Primitive%20Component%20Object%20Reference) (OtherActor :type Actor%20Object%20Reference) (OtherComp :type Primitive%20Component%20Object%20Reference) (OtherBodyIndex :type Integer) (bFromSweep :type Boolean) (SweepResult :type Hit%20Result%20Structure%20%28by%20ref%29))
  ;[0 0 0] BP_Block, when the character touches the block, its mesh shrinks to half its size over half a second using a Timeline and disappears with a "Poof" effect.
  (Networking|SwitchHasAuthority
    (:Authority
      (Utilities|Casting|CastToBP_PGKThirdPersonCharacter OtherActor)
      (CallFunction|MCDissolve))))

(event Custom|MC_Dissolve
  (bind _hex (Variables|Default|GetHex))
  (bind _returnvalue (Transformation|GetWorldTransform _hex))
  ;[0 0 0] BP_Block, when the character touches the block, its mesh shrinks to half its size over half a second using a Timeline and disappears with a "Poof" effect.
  (if (Variables|DoNotEdit|GetCanDissolve)
    (Utilities|FlowControl|Delay 0.2)
    (bind _newtrack_0 (Timeline|Block%20Timeline Play)
      (:Update
        (Transformation|SetWorldScale3D (Variables|Default|GetHex) (Math|Vector|Lerp(Vector) "1.000000,1.000000,1.000000" "0.500000,0.500000,1.000000" _newtrack_0)))
      (:Finished
        (Niagara|SpawnSystematLocation "/Game/PartyGameKit/VFX/Poof/NS_Poof.NS_Poof" (.location _returnvalue) (.rotation _returnvalue) (.scale _returnvalue))
        (Actor|DestroyActor)))))

(fn ConstructionScript)