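; BP_EggSpawner is a party game kit actor that spawns eggs in timed waves at its own transform.
; With authority, SVR_StartSpawner plays confetti through MC_Effects, then spawns a batch of BP_Egg actors sized by SpawnNum.
; After a retriggerable delay, it increments the wave counter, resets the spawn index and calls itself again until CurrentWave equals MaxWave.
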(event Custom|SVR_StartSpawner
  ;[0 0 0] Adjust Max Wave and SpawnNum as desired. SpawnNum determines the number of eggs to spawn per wave. After each wave completes, a delay occurs, and the Current Wave value increments by one. Spawning continues until Current Wave equals Max Wave.
  (Networking|SwitchHasAuthority
    (:Authority
      (if (not (== (Variables|DoNotEdit|GetCurrentWave) (Variables|MainSettings|GetMax%20Wave)))
        (CallFunction|MCEffects)
        (for _index (range (Variables|DoNotEdit|GetSpawnIndex) (Variables|MainSettings|GetSpawnNum))
          (Game|SpawnActorfromClass "/Game/PartyGameKit/Blueprints/Gamemode_Content/BP_Egg.BP_Egg_C" (Transformation|GetActorTransform) "AdjustIfPossibleButAlwaysSpawn" "MultiplyWithRoot" 0 0))
        (Utilities|FlowControl|RetriggerableDelay (Variables|MainSettings|GetSpawnDelay))
        (bind _result (Math|Integer|IncrementInt (Variables|DoNotEdit|GetCurrentWave))
          (:%20%20
            (Variables|DoNotEdit|SetCurrentWave _result)
            (Variables|DoNotEdit|SetSpawnIndex 1)
            (CallFunction|SVRStartSpawner)))))))

(event Custom|MC_Effects
  ;[0 0 0] Adjust Max Wave and SpawnNum as desired. SpawnNum determines the number of eggs to spawn per wave. After each wave completes, a delay occurs, and the Current Wave value increments by one. Spawning continues until Current Wave equals Max Wave.
  ;;[0 0 0] Effects
  (Niagara|SpawnSystematLocation "/Game/PartyGameKit/VFX/Confetti/NS_Confetti.NS_Confetti" (Transformation|GetActorLocation)))

(fn ConstructionScript)