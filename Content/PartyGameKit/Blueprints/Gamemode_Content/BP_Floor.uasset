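; Floor tile for a team-based party game mode that takes on the Red or Blue color of the character overlapping it.
; Box overlap is handled on authority only, passing the character through a server event to an RPC color event.
; When CanChange is set, that event reads the character's Team, tints the Cube's dynamic material and records CurrentColor.
; A separate DynamicMaterial event creates that material and resets the color to None.
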(event OnComponentBeginOverlap(Box)
  (params (OverlappedComponent :type Primitive%20Component%20Object%20Reference) (OtherActor :type Actor%20Object%20Reference) (OtherComp :type Primitive%20Component%20Object%20Reference) (OtherBodyIndex :type Integer) (bFromSweep :type Boolean) (SweepResult :type Hit%20Result%20Structure%20%28by%20ref%29))
  (bind _asbp_pgkthird_person_character (Utilities|Casting|CastToBP_PGKThirdPersonCharacter OtherActor))
  (Networking|SwitchHasAuthority
    (:Authority
      (CallFunction|SVRChangeColor _asbp_pgkthird_person_character))))

(event Custom|RPC_ChangeColor
  (params (Target :type BP%20PGK%20Third%20Person%20Character%20Object%20Reference))
  (bind _team (Variables|/Game/PartyGameKit/Blueprints/Characters/BP_PGKThirdPersonCharacter.BP_PGKThirdPersonCharacter_C|GetTeam Target))
  (if (Variables|Default|GetCanChange?)
    (if (Utilities|String|Contains _team "Red")
      (Rendering|Material|SetVectorParameterValue (Variables|Default|GetCubeColor) "Color" (Variables|Default|GetRed) :!class /Script/Engine.MaterialInstanceDynamic)
      (Variables|Default|SetCurrentColor "Red")
      (elif (Utilities|String|Contains _team "Blue")
        (bind _cubecolor (Variables|Default|GetCubeColor)
          (:then
            (Rendering|Material|SetVectorParameterValue _cubecolor "Color" (Variables|Default|GetBlue) :!class /Script/Engine.MaterialInstanceDynamic)
            (Variables|Default|SetCurrentColor "Blue"))
          (:else))))))

(event Custom|SVR_ChangeColor
  (params (Target :type BP%20PGK%20Third%20Person%20Character%20Object%20Reference))
  (CallFunction|RPCChangeColor Target))

(event Custom|DynamicMaterial
  (bind _returnvalue (Rendering|Material|CreateDynamicMaterialInstance (Variables|Default|GetCube) 0 0 "None" :!class /Script/Engine.PrimitiveComponent))
  (Variables|Default|SetCubeColor _returnvalue)
  (Variables|Default|SetCurrentColor "None"))

(fn ConstructionScript)