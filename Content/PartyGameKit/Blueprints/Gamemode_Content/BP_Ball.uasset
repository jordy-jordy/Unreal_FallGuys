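; Football actor for the party game's football mode that players knock around by running or dashing into it.
; On authority, sphere overlap records the player's name as last hit and pushes the ball away, with dashes using separate strength and fixed lift, briefly gated against repeats.
; Authority also checks speed on Tick, calling RPC events that show timed Niagara smoke on fast shots.
; On NightFootball maps, the ball switches to an emissive white material.
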(event OnComponentBeginOverlap(Sphere)
  (params (OverlappedComponent :type Primitive%20Component%20Object%20Reference) (OtherActor :type Actor%20Object%20Reference) (OtherComp :type Primitive%20Component%20Object%20Reference) (OtherBodyIndex :type Integer) (bFromSweep :type Boolean) (SweepResult :type Hit%20Result%20Structure%20%28by%20ref%29))
  (bind _ball (Variables|Default|GetBall))
  ;[0 0 0] If the player overlaps the collision of the ball, it is set to Last Hit. If the dash boolean is not active, the ball is impulsed with Normal Strength. If dash is true, Impulse is applied with Dash Shot Strength and Chip Shot Impulse values.
  (Networking|SwitchHasAuthority
    (:Authority
      (bind _asbp_pgkthird_person_character (Utilities|Casting|CastToBP_PGKThirdPersonCharacter OtherActor))
      (Variables|DoNotEdit|SetLast%20Hit (PlayerState|GetPlayerName (Variables|/Script/Engine.Pawn|GetPlayerState _asbp_pgkthird_person_character)))
      (if (not (Variables|/Game/PartyGameKit/Blueprints/Characters/BP_PGKThirdPersonCharacter.BP_PGKThirdPersonCharacter_C|GetisDashing? _asbp_pgkthird_person_character))
        (Physics|AddImpulse _ball (* (Math|Vector|GetUnitDirection(Vector) (Transformation|GetActorLocation _asbp_pgkthird_person_character) (Transformation|GetActorLocation)) (Variables|MainSettings|GetNormalStrength)) "None" true)
        (else
          (Utilities|FlowControl|DoOnce false :!label _label
            (:Completed
              (Physics|AddImpulse _ball (Math|Vector|MakeVector (.x (* (Math|Vector|GetUnitDirection(Vector) (Transformation|GetActorLocation _asbp_pgkthird_person_character) (Transformation|GetActorLocation)) (Variables|MainSettings|GetDashShotStrength))) (.y (* (Math|Vector|GetUnitDirection(Vector) (Transformation|GetActorLocation _asbp_pgkthird_person_character) (Transformation|GetActorLocation)) (Variables|MainSettings|GetDashShotStrength))) (Variables|MainSettings|GetChipShotImpulse)) "None" true)
              (Utilities|FlowControl|Delay 0.2)
              (goto _label Reset))))))))

(event Custom|RPC_Smoke
  (bind _niagara (Variables|Default|GetNiagara))
  ;[0 0 0] If the velocity of the ball exceeds 2000, the Smoke niagara  is activated. After 3 seconds it is deactivated again.
  (Components|Activation|SetActive _niagara true false)
  (Utilities|FlowControl|Delay 3.0)
  (Components|Activation|SetActive _niagara false false))

(event Custom|SVR_Smoke
  ;[0 0 0] If the velocity of the ball exceeds 2000, the Smoke niagara  is activated. After 3 seconds it is deactivated again.
  (CallFunction|RPCSmoke))

(event EventTick
  (params (DeltaSeconds :type Float%20%28single-precision%29))
  ;[0 0 0] If the velocity of the ball exceeds 2000, the Smoke niagara  is activated. After 3 seconds it is deactivated again.
  (Networking|SwitchHasAuthority
    (:Authority
      (if (>= (Math|Vector|VectorLength (Transformation|GetVelocity)) 2e+03)
        (CallFunction|SVRSmoke)))))

(event EventBeginPlay
  ;[0 0 0] If the map to be played is “NightFootball”, the material of the football ball changes to neon white.
  (bind _returnvalue (Game|GetCurrentLevelName true))
  (if (Utilities|String|Contains _returnvalue "NightFootball")
    (Rendering|Material|SetMaterial (Variables|Default|GetBall) 0 "/Game/PartyGameKit/Assets/Materials/M_WhiteEmission.M_WhiteEmission")))

(fn ConstructionScript)